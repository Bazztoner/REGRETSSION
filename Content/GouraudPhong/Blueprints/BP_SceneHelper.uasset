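; BP_SceneHelper is a scene utility actor for the Gouraud/Phong lighting setup driven by the MPC_GlobalLighting parameter collection.
; Construction-time reset toggles clear themselves after zeroing the collection's directional and ambient values or its eight indexed point/spot light slots.
; It also enables its PostProcess component from the DisableExposure flag.
; On construction and BeginPlay, it runs console command lists to disable or restore tonemapping.
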(event EventBeginPlay
  (CallFunction|UpdateTonemapper (Variables|Default|GetDisableTonemapping)))

(fn ConstructionScript
  (bind _linearcolor (Utilities|Struct|MakeLinearColor 0.0 0.0 0.0 0.0))
  (bind _linearcolor_2 (Utilities|Struct|MakeLinearColor 0.0 0.0 0.0 0.0))
  (Utilities|FlowControl|Sequence
    (:then_0
      ;[1 1 1] Reset Directional Light to 0
      (if (Variables|ResetLighting|GetResetDirectionalLighting)
        (Variables|ResetLighting|SetResetDirectionalLighting false)
        (Rendering|Material|SetVectorParameterValue "/Game/GouraudPhong/Materials/MPC_GlobalLighting.MPC_GlobalLighting" "DirectionalColour" _linearcolor_2 :!class /Script/Engine.KismetMaterialLibrary)
        (Rendering|Material|SetVectorParameterValue "/Game/GouraudPhong/Materials/MPC_GlobalLighting.MPC_GlobalLighting" "AmbientColour" _linearcolor_2 :!class /Script/Engine.KismetMaterialLibrary)
        (Rendering|Material|SetVectorParameterValue "/Game/GouraudPhong/Materials/MPC_GlobalLighting.MPC_GlobalLighting" "DirectionalSpecular" _linearcolor_2 :!class /Script/Engine.KismetMaterialLibrary)
        (Rendering|Material|SetVectorParameterValue "/Game/GouraudPhong/Materials/MPC_GlobalLighting.MPC_GlobalLighting" "DirectionalVector" _linearcolor_2 :!class /Script/Engine.KismetMaterialLibrary)))
    (:then_1
      ;[1 1 1] Reset Point Light to 0
      (if (Variables|ResetLighting|GetResetPointLighting)
        (Variables|ResetLighting|SetResetPointLighting false)
        (for _index (range 0 7)
          (Rendering|Material|SetVectorParameterValue "/Game/GouraudPhong/Materials/MPC_GlobalLighting.MPC_GlobalLighting" (Utilities|String|StringToName (Utilities|String|Append "PointLocation" (Utilities|String|ToString(Integer) _index))) _linearcolor :!class /Script/Engine.KismetMaterialLibrary)
          (Rendering|Material|SetScalarParameterValue "/Game/GouraudPhong/Materials/MPC_GlobalLighting.MPC_GlobalLighting" (Utilities|String|StringToName (Utilities|String|Append "PointRadius" (Utilities|String|ToString(Integer) _index))) 0.0 :!class /Script/Engine.KismetMaterialLibrary)
          (Rendering|Material|SetVectorParameterValue "/Game/GouraudPhong/Materials/MPC_GlobalLighting.MPC_GlobalLighting" (Utilities|String|StringToName (Utilities|String|Append "PointColour" (Utilities|String|ToString(Integer) _index))) _linearcolor :!class /Script/Engine.KismetMaterialLibrary)
          (Rendering|Material|SetVectorParameterValue "/Game/GouraudPhong/Materials/MPC_GlobalLighting.MPC_GlobalLighting" (Utilities|String|StringToName (Utilities|String|Append "PointSpecular" (Utilities|String|ToString(Integer) _index))) _linearcolor :!class /Script/Engine.KismetMaterialLibrary)
          (Rendering|Material|SetScalarParameterValue "/Game/GouraudPhong/Materials/MPC_GlobalLighting.MPC_GlobalLighting" (Utilities|String|StringToName (Utilities|String|Append "PointBrightness" (Utilities|String|ToString(Integer) _index))) 0.0 :!class /Script/Engine.KismetMaterialLibrary)
          (Rendering|Material|SetScalarParameterValue "/Game/GouraudPhong/Materials/MPC_GlobalLighting.MPC_GlobalLighting" (Utilities|String|StringToName (Utilities|String|Append "SpotAngle" (Utilities|String|ToString(Integer) _index))) 0.0 :!class /Script/Engine.KismetMaterialLibrary)
          (Rendering|Material|SetVectorParameterValue "/Game/GouraudPhong/Materials/MPC_GlobalLighting.MPC_GlobalLighting" (Utilities|String|StringToName (Utilities|String|Append "SpotDirection" (Utilities|String|ToString(Integer) _index))) _linearcolor :!class /Script/Engine.KismetMaterialLibrary)
          (Rendering|Material|SetScalarParameterValue "/Game/GouraudPhong/Materials/MPC_GlobalLighting.MPC_GlobalLighting" (Utilities|String|StringToName (Utilities|String|Append "SpotSoftness" (Utilities|String|ToString(Integer) _index))) 0.0 :!class /Script/Engine.KismetMaterialLibrary))))
    (:then_2
      (Variables|/Script/Engine.PostProcessComponent|SetbEnabled (Variables|Default|GetPostProcess) (Variables|Default|GetDisableExposure)))
    (:then_3
      (CallFunction|UpdateTonemapper (Variables|Default|GetDisableTonemapping)))))

(fn UpdateTonemapper
  (params (Enabled :type Boolean))
  (if Enabled
    (for _array_element (LocalVariables|GetDisableTonemapperCommands)
      (Development|ExecuteConsoleCommand _array_element 0))
    (else
      (for _array_element_2 (LocalVariables|GetEnableTonemapperCommands)
        (Development|ExecuteConsoleCommand _array_element_2 0)))))