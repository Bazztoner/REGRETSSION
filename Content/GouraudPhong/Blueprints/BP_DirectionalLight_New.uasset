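; Directional light Blueprint that feeds global lighting values to materials through the MPC_GlobalLighting parameter collection, apparently for Gouraud/Phong shading.
; UpdateLight writes the directional, ambient and specular colours, plus the negated forward vector of the light scaled by Brightness.
; It runs on BeginPlay and in the construction script, where a self-resetting UpdateLight boolean acts as an editor refresh toggle.
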(event EventBeginPlay
  (CallFunction|UpdateLight))

(fn ConstructionScript
  (CallFunction|UpdateLight)
  (if (Variables|Default|GetUpdate%20Light)
    (Variables|Default|SetUpdate%20Light false)))

(fn UpdateLight
  ;[1 1 1] Directional Light
  (Rendering|Material|SetVectorParameterValue "/Game/GouraudPhong/Materials/MPC_GlobalLighting.MPC_GlobalLighting" "DirectionalColour" (Variables|DirectionalLight|GetLightColour) :!class /Script/Engine.KismetMaterialLibrary)
  (Rendering|Material|SetVectorParameterValue "/Game/GouraudPhong/Materials/MPC_GlobalLighting.MPC_GlobalLighting" "AmbientColour" (Variables|DirectionalLight|GetAmbientColour) :!class /Script/Engine.KismetMaterialLibrary)
  (Rendering|Material|SetVectorParameterValue "/Game/GouraudPhong/Materials/MPC_GlobalLighting.MPC_GlobalLighting" "DirectionalSpecular" (Variables|DirectionalLight|GetSpecularColour) :!class /Script/Engine.KismetMaterialLibrary)
  (Rendering|Material|SetVectorParameterValue "/Game/GouraudPhong/Materials/MPC_GlobalLighting.MPC_GlobalLighting" "DirectionalVector" (Math|Conversions|ToLinearColor(Vector) (* (* (Math|Vector|GetForwardVector (Variables|Default|GetDirectionalLight)) -1.0) (Variables|DirectionalLight|GetBrightness))) :!class /Script/Engine.KismetMaterialLibrary))