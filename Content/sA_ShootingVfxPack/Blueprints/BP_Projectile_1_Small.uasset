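; Small projectile Blueprint from a shooting VFX pack that produces impact effects when it hits something.
; BeginPlay assigns the HitEffect asset to the Hiteffects component.
; When Sphere1 hits anything other than the first FPSReg actor found, it activates and moves that effect to the hit location and disables sphere collision.
; It then spawns ImpactActor there with default rotation, ignoring the surface normal, and immediately destroys itself.
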(event OnComponentHit(Sphere1)
  (params (HitComponent :type Primitive%20Component%20Object%20Reference) (OtherActor :type Actor%20Object%20Reference) (OtherComp :type Primitive%20Component%20Object%20Reference) (NormalImpulse :type Vector :default "0, 0, 0") (Hit :type Hit%20Result%20Structure%20%28by%20ref%29))
  (bind _location (Collision|BreakHitResult Hit))
  (bind _hiteffects (Variables|Default|GetHiteffects))
  (bind _returnvalue (Actor|GetActorOfClass "/Game/REGRETSSION-Assets/Blueprints/Player/FPSReg.FPSReg_C"))
  (if (!= OtherActor _returnvalue)
    (Components|Activation|SetActive _hiteffects true false)
    (Transformation|SetWorldLocation _hiteffects _location false false)
    (Collision|SetCollisionEnabled (Variables|Default|GetSphere1) "NoCollision")
    (Game|SpawnActorfromClass (Variables|Default|GetImpactActor) (Math|Transform|MakeTransform _location) "Undefined" 0 0)
    (Actor|DestroyActor)))

(event EventBeginPlay
  (Class|NiagaraComponent|SetAsset (Variables|Default|GetHiteffects) (Variables|Default|GetHitEffect)))

(fn ConstructionScript)