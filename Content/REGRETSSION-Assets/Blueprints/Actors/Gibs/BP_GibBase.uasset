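; BP_GibBase is a base gib actor that launches a random chunk mesh and leaves decals where it hits.
; BeginPlay picks a mesh from GibMeshes and applies a randomized, mostly upward velocity-change impulse.
; Hit spawns a random long-lived decal at the actor's location, gated by a timer cooldown and a MaxDecals check.
; CurrentDecals is compared against that cap but never incremented here.
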(event Custom|SetSpawnAvailable
  (Variables|Default|SetCanSpawnDecal true))

(event EventBeginPlay
  (Components|StaticMesh|SetStaticMesh (Variables|Default|GetStaticMesh) (.OutItem (Utilities|Array|Random (Variables|Default|GetGibMeshes))))
  (CallFunction|AddForce))

(event Collision|EventHit
  (params (MyComp :type Primitive%20Component%20Object%20Reference) (Other :type Actor%20Object%20Reference) (OtherComp :type Primitive%20Component%20Object%20Reference) (bSelfMoved :type Boolean) (HitLocation :type Vector :default "0, 0, 0") (HitNormal :type Vector :default "0, 0, 0") (NormalImpulse :type Vector :default "0, 0, 0") (Hit :type Hit%20Result%20Structure%20%28by%20ref%29))
  (bind _returnvalue (CallFunction|CheckSpawnableDecal))
  (if _returnvalue
    (Rendering|Decal|SpawnDecalatLocation (.OutItem (Utilities|Array|Random (Variables|Default|GetSpawnableDecalsMat))) "75.000000,75.000000,75.000000" (Transformation|GetActorLocation) "-90.000000,0.000000,0.000000" 1.5e+02)
    (Variables|Default|SetCanSpawnDecal false)
    (Utilities|Time|SetTimerbyEvent (delegate Custom|SetSpawnAvailable) (Variables|Default|GetDecalCooldown))))

(fn ConstructionScript)

(fn CheckSpawnableDecal
  (return (and (Variables|Default|GetCanSpawnDecal) (< (Variables|Default|Get_currentDecals) (Variables|Default|GetMaxDecals)))))

(fn AddForce
  (Physics|AddImpulse (Variables|Default|GetStaticMesh) (+ (* (Transformation|GetActorForwardVector) (Math|Random|RandomFloatinRange 0.0 3e+02)) (* (Transformation|GetActorUpVector) (Math|Random|RandomFloatinRange 3e+02 8e+02)) (* (Transformation|GetActorRightVector) (Math|Random|RandomFloatinRange -2e+02 2e+02))) "None" true))