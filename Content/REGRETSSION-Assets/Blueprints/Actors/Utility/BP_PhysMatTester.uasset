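; BP_PhysMatTester is a utility actor that labels SuperGrid_Wall test walls with the name of their physical material.
; It finds every SuperGrid_Wall in the level and writes the display name of each wall's override physical material into that wall's text render component, if one exists.
; The pass runs in both the construction script and BeginPlay, so labels update in the editor and at play start.
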(event EventBeginPlay
  (CallFunction|SetPhysMatText))

(event Collision|EventActorBeginOverlap
  (params (OtherActor :type Actor%20Object%20Reference)))

(event EventTick
  (params (DeltaSeconds :type Float%20%28single-precision%29)))

(fn ConstructionScript
  (CallFunction|SetPhysMatText))

(fn SetPhysMatText
  (bind _outactors (Actor|GetAllActorsOfClass "/Game/SuperGrid/StarterPack/Blueprints/SuperGrid_Wall.SuperGrid_Wall_C"))
  (for _array_element _outactors
    (Utilities|IsValid (Actor|GetComponentbyClass _array_element "/Script/Engine.TextRenderComponent")
      (:Is%20Valid
        (Rendering|Components|TextRender|SetText (Actor|GetComponentbyClass _array_element "/Script/Engine.TextRenderComponent") (Utilities|Text|ToText(String) (Utilities|GetDisplayName (Variables|/Game/SuperGrid/StarterPack/Blueprints/SuperGrid_Wall.SuperGrid_Wall_C|GetOverridePhysicalMaterial _array_element))))))))