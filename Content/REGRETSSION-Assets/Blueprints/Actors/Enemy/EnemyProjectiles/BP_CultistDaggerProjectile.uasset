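; Dagger projectile for the cultist enemy that flies straight ahead and damages the first Character it overlaps other than its instigator.
; Each Tick offsets it along its forward vector without sweep, and a spawn sound plays attached to its mesh.
; InitializeProjectile sets damage and ammo type.
; Overlaps apply damage credited to the instigator and destroy the projectile, while non-Character actors are ignored.
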(event EventTick
  (params (DeltaSeconds :type Float%20%28single-precision%29))
  (CallFunction|HandleMovement DeltaSeconds))

(event Collision|EventActorBeginOverlap
  (params (OtherActor :type Actor%20Object%20Reference))
  (CallFunction|CheckCollision OtherActor))

(event EventBeginPlay
  (Audio|SpawnSoundAttached (Variables|Default|GetSpawnSound) (Variables|Default|GetStaticMesh) "None" "0, 0, 0" "0, 0, 0" "KeepRelativeOffset" false 1.0 1.0 0.0 0 0))

(fn ConstructionScript
  (|CallParentFunction))

(fn HandleMovement
  (params (Delta%20Time :type Float%20%28double-precision%29))
  (Transformation|AddActorWorldOffset self (* (Transformation|GetActorForwardVector self) (* (Variables|Default|GetMovementSpeed) Delta%20Time))))

(fn InitializeProjectile
  (params (Damage :type Float%20%28double-precision%29) (AmmoType :type ENUM_AmmoTypes%20Enum :default "NewEnumerator6"))
  (Variables|Default|SetDamage Damage)
  (Variables|Default|SetAmmoType AmmoType))

(fn CheckCollision
  (params (Actor :type Actor%20Object%20Reference))
  (bind _instigator (Variables|Default|GetInstigator))
  (bind _aspawn (Utilities|Casting|CastToPawn Actor))
  (if (== _aspawn (Variables|Default|GetInstigator))
    (return)
    (else
      (bind _ascharacter (Utilities|Casting|CastToCharacter Actor))
      (Game|Damage|ApplyDamage _ascharacter (Variables|Default|GetDamage) (Game|GetInstigatorController _instigator) _instigator)
      (Actor|DestroyActor))))