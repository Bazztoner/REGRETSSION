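; Enemy hitscan bullet actor that resolves a shot instantly with a line trace while showing a travelling tracer.
; SpawnHitscan traces on the Camera channel, spawns a tracer toward the impact or max range, and plays a Niagara muzzle flash.
; Hits apply and report damage, add surface-based particles and decals, then start delayed self-destruction; misses never start it.
; CheckActorHit can notify BP_IHittable targets but is not called within this Blueprint.
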(event Custom|DelayedDestruction
  (Utilities|FlowControl|Delay (Variables|Default|GetLifeTIme))
  (Actor|DestroyActor))

(event EventBeginPlay)

(event Collision|EventActorBeginOverlap
  (params (OtherActor :type Actor%20Object%20Reference)))

(event EventTick
  (params (DeltaSeconds :type Float%20%28single-precision%29)))

(fn ConstructionScript)

(fn SpawnHitscan
  (params (MaxDistance :type Float%20%28double-precision%29) (Damage :type Float%20%28double-precision%29) (Type :type ENUM_AmmoTypes%20Enum :default "NewEnumerator6") (Position :type Vector) (Rotation :type Vector))
  (bind _returnvalue (Transformation|GetActorTransform))
  (bind _instigator (Variables|Default|GetInstigator))
  (Utilities|FlowControl|Sequence
    (:then_0
      (Variables|Default|SetDamage Damage)
      (Variables|Default|SetMaxRange MaxDistance)
      (Variables|Default|SetAmmoType Type))
    (:then_1
      (bind (_outhit _returnvalue_2) (Collision|LineTraceByChannel Position (+ Position (* Rotation (Variables|Default|GetMaxRange))) "TraceTypeQuery2" true 0 "None" true "(R=1.000000,G=0.485008,B=0.000000,A=1.000000)" "(R=0.000000,G=1.000000,B=0.085811,A=1.000000)" 2.0))
      (if _returnvalue_2
        (CallFunction|SpawnTracer (.ImpactPoint (Collision|BreakHitResult _outhit)))
        (bind _returnvalue_3 (Game|Damage|ApplyDamage (.HitActor (Collision|BreakHitResult _outhit)) (Variables|Default|GetDamage) (Game|GetInstigatorController) _instigator))
        (Class|AISenseDamage|ReportDamageEvent (.HitActor (Collision|BreakHitResult _outhit)) _instigator _returnvalue_3 (.Location (Collision|BreakHitResult _outhit)) "0, 0, 0" "None")
        (CallFunction|CheckSpawnHitParticle (Variables|/Script/PhysicsCore.PhysicalMaterial|GetSurfaceType (.PhysMat (Collision|BreakHitResult _outhit))) (.ImpactPoint (Collision|BreakHitResult _outhit)) (.ImpactNormal (Collision|BreakHitResult _outhit)))
        (CallFunction|CheckSpawnHitDecal false (Variables|/Script/PhysicsCore.PhysicalMaterial|GetSurfaceType (.PhysMat (Collision|BreakHitResult _outhit))) "1.500000,4.000000,4.000000" 0 (.ImpactPoint (Collision|BreakHitResult _outhit)) (Math|Conversions|RotationFromXVector (.ImpactNormal (Collision|BreakHitResult _outhit))) 3e+02)
        (CallFunction|DelayedDestruction)
        (else
          (CallFunction|SpawnTracer (+ Position (* Rotation (Variables|Default|GetMaxRange)))))))
    (:then_2
      (Niagara|SpawnSystematLocation "/Game/sA_ShootingVfxPack/FX/NiagaraSystems/NS_AR_Muzzleflash_1_ONCE.NS_AR_Muzzleflash_1_ONCE" (.location _returnvalue) (.rotation _returnvalue) "1.000000,1.000000,1.000000" true true "AutoRelease"))))

(fn SpawnTracer
  (params (ImpactPoint :type Vector))
  (bind _returnvalue (Transformation|GetActorLocation))
  (bind _instigator (Variables|Default|GetInstigator))
  (Game|SpawnActorfromClass (Variables|Default|GetTracer) (Math|Transform|MakeTransform _returnvalue (Math|Rotator|FindLookatRotation _returnvalue ImpactPoint) "1.000000,1.000000,1.000000") "Undefined" "SelectDefaultAtRuntime" _instigator 1.0 ImpactPoint 8.5e+03 _instigator))

(fn CheckActorHit
  (params (HittedActor :type Actor%20Object%20Reference) (ImpactPoint :type Vector) (ImpactNormal :type Vector))
  (bind _asbp_ihittable (Utilities|Casting|CastToBP_IHittable HittedActor))
  (Default|OnDamagingImpact _asbp_ihittable ImpactPoint ImpactNormal "NewEnumerator0" "NewEnumerator9"))