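; Base enemy Blueprint handling health, sounds, hit effects and gore-based deaths.
; Damage and ammo types select a particle component class, added temporarily to pick a random Niagara or Cascade effect.
; On death, damage thresholds and impact height choose torso gibbing, then headshot, hiding bones and spawning blood, plus gibs for torso hits.
; The resulting death type places the blood pool when death ends, before the blood spray is removed.
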(event Custom|OnEndDeath
  (CallFunction|SpawnBloodPool)
  (Utilities|FlowControl|Delay 1.0)
  (bind _gibbedbloodparticle (Variables|Default|GetGibbedBloodParticle)
    (:then
      (Effects|Components|ParticleSystem|ReleasetoPool _gibbedbloodparticle)
      (Class|NiagaraComponent|SetRenderingEnabled _gibbedbloodparticle false)
      (Components|DestroyComponent _gibbedbloodparticle))
    (:else)))

(event EventOnDamagingImpact
  (params (ImpactPoint :type Vector :default "0, 0, 0") (ImpactNormal :type Vector :default "0, 0, 0") (DamageType :type ENUM_DamageTypes%20Enum :default "NewEnumerator0") (AmmoType :type ENUM_AmmoTypes%20Enum :default "NewEnumerator6"))
  (CallFunction|SpawnDamageParticle ImpactPoint ImpactNormal DamageType AmmoType))

(fn ConstructionScript)

(fn OnTargetFound)

(fn StartDeath
  (params (ImpactPoint :type Vector) (KillingDamage :type Float%20%28double-precision%29))
  (bind _gibbed (CallFunction|CheckTorsoGibbing ImpactPoint KillingDamage))
  (if (not _gibbed)
    (bind _gibbed_2 (CallFunction|CheckHeadshotGibbing ImpactPoint KillingDamage))
    (if (not _gibbed_2)
      (Variables|Default|SetDeathType "NewEnumerator0"))))

(fn InitializeEnemy
  (bind _capsulecomponent (Variables|Collision|GetCapsuleComponent))
  (Variables|Default|Set_currentHP (Math|Conversions|ToFloat(Integer) (Variables|Default|GetMaxHP)))
  (Variables|Default|SetSpawnedPosition (Transformation|GetWorldLocation _capsulecomponent))
  (Variables|Default|SetSpawnedRotation (Transformation|GetWorldRotation _capsulecomponent))
  (bind _returnvalue (Actor|GetActorOfClass "/Game/REGRETSSION-Assets/Blueprints/Player/BP_Player.BP_Player_C"))
  (Variables|Default|SetPlayer _returnvalue))

(fn PlaySound
  (params (Sound :type Sound%20Base%20Object%20Reference) (CancelPreviousSound :type Boolean) (Cancellable :type Boolean))
  (Utilities|FlowControl|Sequence
    (:then_0
      (if CancelPreviousSound
        (bind _currentsound (Variables|Default|GetCurrentSound)
          (:then
            (Audio|Components|Audio|Stop _currentsound))
          (:else))))
    (:then_1
      (bind _returnvalue (Audio|SpawnSoundAttached Sound (Variables|Character|GetMesh) "None" "0, 0, 0" "0, 0, 0" "KeepRelativeOffset" true 1.0 1.0 0.0 0 0))
      (if Cancellable
        (Variables|Default|SetCurrentSound _returnvalue)))))

(fn TakeDamageGeneric
  (params (Dmg :type Float%20%28double-precision%29))
  (Variables|Default|Set_currentHP (- (Variables|Default|Get_currentHP) Dmg))
  (Effects|SpawnEmitteratLocation (Variables|Default|GetHitParticleSystem) (Transformation|GetActorLocation) "0, 0, 0" "1.000000,1.000000,1.000000" true "AutoRelease"))

(fn TakeDamagePoint
  (params (Dmg :type Float%20%28double-precision%29) (HitLoc :type Vector) (HitNormal :type Vector) (HitBone :type Name))
  (Variables|Default|Set_currentHP (- (Variables|Default|Get_currentHP) Dmg)))

(fn SpawnDamageParticle
  (params (ImpactPoint :type Vector) (ImpactNormal :type Vector) (DamageType :type ENUM_DamageTypes%20Enum :default "NewEnumerator0") (AmmoType :type ENUM_AmmoTypes%20Enum :default "NewEnumerator6"))
  (bind _bp_enemydamageparticles (Variables|Default|GetBP_EnemyDamageParticles))
  (Utilities|FlowControl|Sequence
    (:then_0
      (switch Utilities|FlowControl|Switch|SwitchonENUM_DamageTypes DamageType
        (:NewEnumerator0
          (LocalVariables|SetParticleComponent (.Value (Utilities|Map|Find (Variables|/Game/REGRETSSION-Assets/Blueprints/Actors/Enemy/EnemyBP/BP_EnemyDamageParticles.BP_EnemyDamageParticles_C|GetAmmoDamageParticles _bp_enemydamageparticles) AmmoType))))
        (:NewEnumerator1
          (LocalVariables|SetParticleComponent (.Value (Utilities|Map|Find (Variables|/Game/REGRETSSION-Assets/Blueprints/Actors/Enemy/EnemyBP/BP_EnemyDamageParticles.BP_EnemyDamageParticles_C|GetNonWeaponDamageParticles _bp_enemydamageparticles) DamageType)) :!label _label))
        (:NewEnumerator2
          (goto _label))
        (:NewEnumerator3
          (LocalVariables|SetParticleComponent (.Value (Utilities|Map|Find (Variables|/Game/REGRETSSION-Assets/Blueprints/Actors/Enemy/EnemyBP/BP_EnemyDamageParticles.BP_EnemyDamageParticles_C|GetGibParticles (Variables|Default|GetBP_EnemyDamageParticles)) "NewEnumerator0"))))))
    (:then_1
      (bind _returnvalue (Game|AddComponentbyClass (LocalVariables|GetParticleComponent)))
      (if (Variables|/Game/REGRETSSION-Assets/Blueprints/Components/BP_ParticleArrayComponent.BP_ParticleArrayComponent_C|GetUseNiagara _returnvalue)
        (bind _particle (Default|GetRandomNiagara _returnvalue))
        (Niagara|SpawnSystemAttached _particle (Variables|Character|GetMesh) "None" ImpactPoint "0, 0, 0" "KeepWorldPosition" true true "AutoRelease")
        (else
          (bind _particle_2 (Default|GetRandomCascade _returnvalue))
          (Effects|SpawnEmitterAttached _particle_2 (Variables|Character|GetMesh) "None" ImpactPoint "0, 0, 0" "1.000000,1.000000,1.000000" "KeepWorldPosition" true "AutoRelease"))))
    (:then_2
      (Components|DestroyComponent _returnvalue))))

(fn CheckHeadshotGibbing
  (params (ImpactPoint :type Vector) (KillingDamage :type Float%20%28double-precision%29))
  (bind _headbonename (Variables|Default|GetHeadBoneName))
  (bind _mesh (Variables|Character|GetMesh))
  (bind _returnvalue (Transformation|GetSocketLocation _mesh _headbonename))
  (if (>= KillingDamage (Variables|Default|GetHeadshotDamageThreshold))
    (if (>= (.Z (Math|Vector|BreakVector ImpactPoint)) (.Z (Math|Vector|BreakVector _returnvalue)))
      (Components|SkinnedMesh|HideBonebyName (Variables|Character|GetMesh) (Variables|Default|GetHeadBoneName) "PBO_None")
      (CallFunction|SpawnDamageParticle _returnvalue "0, 0, 0" "NewEnumerator3" "NewEnumerator6")
      (Variables|Default|SetDeathType "NewEnumerator1")
      (CallFunction|SpawnGibBloodParticle (Variables|Default|GetHeadSocket))
      (return true)
      (else
        (return false)))
    (else
      (return false))))

(fn CheckTorsoGibbing
  (params (ImpactPoint :type Vector) (KillingDamage :type Float%20%28double-precision%29))
  (bind _mesh (Variables|Character|GetMesh))
  (if (>= KillingDamage (Variables|Default|GetGibbingDamageThreshold))
    (if (or (>= (.Z (Math|Vector|BreakVector ImpactPoint)) (.z (Transformation|GetSocketLocation (Variables|Character|GetMesh) (Variables|Default|GetGibBoneName)))) (>= KillingDamage (Variables|Default|GetLiquifiyingGibsThreshold)))
      (for _array_element (Variables|Default|GetGibbingBones)
        (Components|SkinnedMesh|HideBonebyName _mesh _array_element "PBO_None")
        (CallFunction|SpawnDamageParticle (Transformation|GetSocketLocation _mesh _array_element) "0, 0, 0" "NewEnumerator3" "NewEnumerator6"))
      (CallFunction|SpawnGibs 6)
      (CallFunction|SpawnGibBloodParticle (Variables|Default|GetTorsoSocket))
      (return true)
      (else
        (return false)))
    (else
      (return false))))

(fn SpawnBloodPool
  (Utilities|FlowControl|Sequence
    (:then_0
      (switch Utilities|FlowControl|Switch|SwitchonENUM_EnemyDeathStates (Variables|Default|GetDeathType)
        (:NewEnumerator0
          (return))
        (:NewEnumerator1
          (LocalVariables|SetBloodPoolLocation (Transformation|GetSocketLocation (Variables|Character|GetMesh) (Variables|Default|GetHeadSocket))))
        (:NewEnumerator2
          (LocalVariables|SetBloodPoolLocation (Transformation|GetSocketLocation (Variables|Character|GetMesh) (Variables|Default|GetTorsoSocket))))))
    (:then_1
      (bind _bloodpoolclass (Variables|Default|GetBloodPoolClass)
        (:then
          (Game|SpawnActorfromClass _bloodpoolclass (Math|Transform|MakeTransform (LocalVariables|GetBloodPoolLocation) "0, 0, 0" "1.000000,1.000000,1.000000") "AlwaysSpawn" "SelectDefaultAtRuntime" 0 0))
        (:else)))))

(fn SpawnGibs
  (params (GibAmount :type Integer))
  (for _index (range 1 GibAmount)
    (Game|SpawnActorfromClass "/Game/REGRETSSION-Assets/Blueprints/Actors/Gibs/BP_GibBase.BP_GibBase_C" (Math|Transform|MakeTransform (Transformation|GetSocketLocation (Variables|Character|GetMesh) (Variables|Default|GetGibBoneName)) "0, 0, 0" "1.000000,1.000000,1.000000") "AdjustIfPossibleButAlwaysSpawn" "OverrideRootScale" 0 "0.000000,0.000000,0.000000" 0))
  (Variables|Default|SetDeathType "NewEnumerator2"))

(fn SpawnGibBloodParticle
  (params (Socket :type Name))
  (Utilities|FlowControl|Sequence
    (:then_0
      (LocalVariables|SetParticleToSpawn (.OutItem (Utilities|Array|Random (Variables|/Game/REGRETSSION-Assets/Blueprints/Actors/Enemy/EnemyBP/BP_EnemyDamageParticles.BP_EnemyDamageParticles_C|GetBloodParticles (Variables|Default|GetBP_EnemyDamageParticles))))))
    (:then_1
      (bind _returnvalue (Niagara|SpawnSystemAttached (LocalVariables|GetParticleToSpawn) (Variables|Character|GetMesh) Socket "0, 0, 0" "270.000000, 0, 0" "SnapToTarget" false true "AutoRelease"))
      (Variables|Default|SetGibbedBloodParticle _returnvalue))))