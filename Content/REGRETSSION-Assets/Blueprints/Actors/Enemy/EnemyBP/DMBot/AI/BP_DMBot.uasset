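; BP_DMBot is an enemy bot Blueprint whose only logic is a hitscan gunshot.
; Shoot requires a valid AI controller focus actor, then spawns a BP_EnemyHitscanBullet at the Muzzle.
; The bullet's SpawnHitscan receives the normalized direction toward that focus actor, and a Garand shot sound plays at the Weapon.
; The event graph and construction script are empty, so nothing in this file triggers Shoot.
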(event EventBeginPlay)

(event Collision|EventActorBeginOverlap
  (params (OtherActor :type Actor%20Object%20Reference)))

(event EventTick
  (params (DeltaSeconds :type Float%20%28single-precision%29)))

(fn ConstructionScript)

(fn Shoot
  (bind _self self)
  (bind _muzzle (Variables|Default|GetMuzzle))
  (bind _returnvalue (AI|GetAIController _self))
  (bind _returnvalue_2 (Transformation|GetSocketLocation _muzzle "None"))
  (bind _returnvalue_3 (Class|AIController|GetFocusActor _returnvalue))
  (Utilities|IsValid _returnvalue_3
    (:Is%20Valid
      (bind _returnvalue_4 (Game|SpawnActorfromClass "/Game/REGRETSSION-Assets/Blueprints/Actors/Enemy/EnemyProjectiles/BP_EnemyHitscanBullet.BP_EnemyHitscanBullet_C" (Transformation|GetSocketTransform _muzzle "None" "RTS_World") "Undefined" 0 0))
      (Default|SpawnHitscan _returnvalue_4 3e+03 1.0 "NewEnumerator0" _returnvalue_2 (Math|Vector|Normalize (- (Transformation|GetActorLocation _returnvalue_3) _returnvalue_2)))
      (Audio|PlaySoundatLocation "/Game/REGRETSSION-Assets/Art/Weapons/M1Garand/Sounds/garand_shoot.garand_shoot" (Transformation|GetWorldLocation (Variables|Default|GetWeapon)) "0, 0, 0" 1.0 1.0 0.0 0 0 0))))