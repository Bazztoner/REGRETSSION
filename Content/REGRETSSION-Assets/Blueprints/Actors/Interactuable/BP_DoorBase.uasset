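; BP_DoorBase is a base interactable door that is pushed open or knocked by physics impulses.
; CheckInteract forwards to DoorInteracted, which applies a velocity-change impulse from the interactor's forward vector and InteractForce.
; AnyDamage pushes it likewise, scaled by damage along the causer's forward vector; both impulses use only the X component.
; Damaging impacts spawn a pooled hit particle at the impact point.
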(event Custom|DoorInteracted
  (params (Interactor :type Actor%20Object%20Reference))
  (Physics|AddImpulse (Variables|Default|GetDoor) (Math|Vector|MakeVector (* (.X (Math|Vector|BreakVector (Transformation|GetActorForwardVector Interactor))) (Variables|Default|GetInteractForce)) 0.0 0.0) "None" true))

(event Game|Damage|EventAnyDamage
  (params (Damage :type Float%20%28single-precision%29) (DamageType :type Damage%20Type%20Object%20Reference) (InstigatedBy :type Controller%20Object%20Reference) (DamageCauser :type Actor%20Object%20Reference))
  ;[1 1 1] Fix later or add chaos
  (if (Utilities|IsValid DamageCauser)
    (Physics|AddImpulse (Variables|Default|GetDoor) (Math|Vector|MakeVector (* Damage (.X (Math|Vector|BreakVector (Transformation|GetActorForwardVector DamageCauser))) 1.0) 0.0 0.0) "None" true)))

(event EventOnDamagingImpact
  (params (ImpactPoint :type Vector :default "0, 0, 0") (ImpactNormal :type Vector :default "0, 0, 0") (DamageType :type ENUM_DamageTypes%20Enum :default "NewEnumerator0") (AmmoType :type ENUM_AmmoTypes%20Enum :default "NewEnumerator6"))
  (Effects|SpawnEmitteratLocation (Variables|Default|GetHitParticle) ImpactPoint "0, 0, 0" "1.000000,1.000000,1.000000" true "AutoRelease"))

(fn ConstructionScript)

(fn CheckInteract
  (params (Interactor :type Actor%20Object%20Reference))
  (CallFunction|DoorInteracted Interactor))