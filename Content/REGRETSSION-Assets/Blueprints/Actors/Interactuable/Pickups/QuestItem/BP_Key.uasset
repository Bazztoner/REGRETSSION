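; BP_Key is a key pickup that spins and moves vertically while waiting to be collected.
; On BeginPlay it stores the Key component's world location and plays a timeline that drives the Scene component's yaw and height offset.
; When BP_Player overlaps it, it passes itself to the player's CheckPickupKey, then plays a 2D pickup sound and destroys itself unconditionally.
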(event EventBeginPlay
  (Variables|Default|SetInitialPosition (Transformation|GetWorldLocation (Variables|Default|GetKey)))
  (bind (_direction _rotation _position) (Timeline|MeshAnimation PlayFromStart)
    (:Update
      (CallFunction|RotateMesh _rotation)
      (CallFunction|MoveMesh _position))))

(event Collision|EventActorBeginOverlap
  (params (OtherActor :type Actor%20Object%20Reference))
  (bind _asbp_player (Utilities|Casting|CastToBP_Player OtherActor))
  (Default|CheckPickupKey _asbp_player self)
  (Audio|PlaySound2D (Variables|Default|GetPickupSound) 1.0 1.0 0.0 0 0)
  (Actor|DestroyActor))

(fn ConstructionScript)

(fn RotateMesh
  (params (RotationInput :type Float%20%28double-precision%29))
  (bind _scene (Variables|Default|GetScene))
  (bind _relativerotation (Variables|/Script/Engine.SceneComponent|GetRelativeRotation _scene))
  (bind (_roll _pitch) (Math|Rotator|BreakRotator _relativerotation))
  (LocalVariables|SetAnimRot RotationInput)
  (Utilities|IsValid _scene
    (:Is%20Valid
      (Transformation|SetRelativeRotation _scene (Math|Rotator|MakeRotator _roll _pitch (LocalVariables|GetAnimRot)) false false))))

(fn MoveMesh
  (params (PositionInput :type Float%20%28double-precision%29))
  (bind _scene (Variables|Default|GetScene))
  (bind _initialposition (Variables|Default|GetInitialPosition))
  (bind (_x _y _z) (Math|Vector|BreakVector _initialposition))
  (LocalVariables|SetZPos PositionInput)
  (Utilities|IsValid _scene
    (:Is%20Valid
      (Transformation|SetWorldLocation _scene (Math|Vector|MakeVector _x _y (+ _z (LocalVariables|GetZPos))) false false))))