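; Base ammo pickup actor that gives ammo to the player character when touched.
; On overlap it casts the other actor to FPSReg and asks whether it can take this ammo type.
; If so, it passes the type and amount to the character, has it play the pickup sound, then destroys itself.
; Otherwise it stays in the world.
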(event EventBeginPlay
  (|CallParentFunction) ; This node is disabled and will not be called.\nDrag off pins to build functionality.
)

(event Collision|EventActorBeginOverlap
  (params (OtherActor :type Actor%20Object%20Reference))
  (bind _asfpsreg (Utilities|Casting|CastToFPSReg OtherActor))
  (bind _canpickup (Default|CanPickupAmmo _asfpsreg (Variables|Default|GetAmmoType)))
  (if _canpickup
    (Default|PickupAmmo _asfpsreg (Variables|Default|GetAmmoType) (Variables|Default|GetAmount))
    (Default|PlaySound _asfpsreg (Variables|Default|GetPickupSound))
    (Actor|DestroyActor)))

(event EventTick
  (params (DeltaSeconds :type Float%20%28single-precision%29))
  (|CallParentFunction DeltaSeconds) ; This node is disabled and will not be called.\nDrag off pins to build functionality.
)

(fn ConstructionScript
  (|CallParentFunction))