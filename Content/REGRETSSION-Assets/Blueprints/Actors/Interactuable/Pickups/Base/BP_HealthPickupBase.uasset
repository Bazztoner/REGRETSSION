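; BP_HealthPickupBase is a base pickup actor that restores the player's health on touch.
; On actor overlap it casts the other actor to BP_Player and asks whether it can pick up health.
; If so, it heals the player by HealthAmount, plays PickupSound in 2D and destroys itself; otherwise it stays in the world.
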(event EventBeginPlay
  (|CallParentFunction) ; This node is disabled and will not be called.\nDrag off pins to build functionality.
)

(event Collision|EventActorBeginOverlap
  (params (OtherActor :type Actor%20Object%20Reference))
  (bind _asfpsreg (Utilities|Casting|CastToBP_Player OtherActor))
  (bind _canpickup (Default|CanPickupHealth _asfpsreg))
  (if _canpickup
    (Default|TakeHeal _asfpsreg (Variables|Default|GetHealthAmount))
    (Audio|PlaySound2D (Variables|Default|GetPickupSound) 1.0 1.0 0.0 0 0)
    (Actor|DestroyActor)))

(event EventTick
  (params (DeltaSeconds :type Float%20%28single-precision%29))
  (|CallParentFunction DeltaSeconds) ; This node is disabled and will not be called.\nDrag off pins to build functionality.
)

(fn ConstructionScript
  (|CallParentFunction))