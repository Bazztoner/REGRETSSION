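; Base ammo pickup actor that gives a set amount of an ammo type to an overlapping BP_Player, if the player can take it.
; On a successful pickup it plays the sound through the player and destroys itself.
; A text component shows the ammo type, set at construction, with visibility toggled on BeginPlay.
; An optional timeline yaws the mesh pivot; MoveMesh supports vertical offset but AnimateMesh never calls it.
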(event EventBeginPlay
  (Utilities|FlowControl|Sequence
    (:then_0
      (Rendering|SetVisibility (Variables|Default|GetAmmoTypeText) (Variables|Default|GetAmmoTextVisible) false))
    (:then_1
      (if (Variables|Default|GetAnimationEnabled)
        (bind (_direction _rotation _position) (Timeline|MeshAnim PlayFromStart)
          (:Update
            (Utilities|AnimateMesh _rotation _position)))))))

(event Collision|EventActorBeginOverlap
  (params (OtherActor :type Actor%20Object%20Reference))
  (bind _asbp_player (Utilities|Casting|CastToBP_Player OtherActor))
  (bind _canpickup (Default|CanPickupAmmo _asbp_player (Variables|Default|GetAmmoType)))
  (if _canpickup
    (Default|PickupAmmo _asbp_player (Variables|Default|GetAmmoType) (Variables|Default|GetAmount))
    (Default|PlaySound _asbp_player (Variables|Default|GetPickupSound))
    (Actor|DestroyActor)))

(event EventTick
  (params (DeltaSeconds :type Float%20%28single-precision%29))
  (|CallParentFunction DeltaSeconds) ; This node is disabled and will not be called.\nDrag off pins to build functionality.
)

(fn ConstructionScript
  (|CallParentFunction)
  (Rendering|Components|TextRender|SetText (Variables|Default|GetAmmoTypeText) (Utilities|Text|ToText(String) (Utilities|String|EnumtoString (Variables|Default|GetAmmoType)))))

(fn MoveMesh
  (params (PositionInput :type Float%20%28double-precision%29))
  (bind _initialposition (Variables|Default|GetInitialPosition))
  (bind _meshpivot (Variables|Default|GetMeshPivot))
  (bind (_x _y _z) (Math|Vector|BreakVector _initialposition))
  (LocalVariables|SetPosInput PositionInput)
  (Utilities|IsValid _meshpivot
    (:Is%20Valid
      (Transformation|SetWorldLocation _meshpivot (Math|Vector|MakeVector _x _y (+ _z (LocalVariables|GetPosInput))) false false))))

(fn RotateMesh
  (params (RotationInput :type Float%20%28double-precision%29))
  (bind _meshpivot (Variables|Default|GetMeshPivot))
  (bind _relativerotation (Variables|/Script/Engine.SceneComponent|GetRelativeRotation _meshpivot))
  (bind (_roll _pitch) (Math|Rotator|BreakRotator _relativerotation))
  (LocalVariables|SetRot RotationInput)
  (Utilities|IsValid _meshpivot
    (:Is%20Valid
      (Transformation|SetRelativeRotation _meshpivot (Math|Rotator|MakeRotator _roll _pitch (LocalVariables|GetRot)) false false))))