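; BP_PickupBase is a base pickup actor that gives a chosen mesh an idle spin and vertical bob animation.
; SetAnimatingMesh stores the mesh and its starting world location when AnimationEnabled is set.
; On BeginPlay, if enabled, the MeshAnimation timeline feeds AnimateMesh, which sets the mesh's relative yaw and offsets its world Z from that stored position.
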(event EventBeginPlay
  (if (Variables|Default|GetAnimationEnabled)
    (bind (_direction _rotation _position) (Timeline|MeshAnimation PlayFromStart)
      (:Update
        (Utilities|AnimateMesh _rotation _position)))))

(event Collision|EventActorBeginOverlap
  (params (OtherActor :type Actor%20Object%20Reference)))

(event EventTick
  (params (DeltaSeconds :type Float%20%28single-precision%29)))

(fn ConstructionScript)

(fn RotateMesh
  (params (RotationInput :type Float%20%28single-precision%29))
  (bind _mesh (Variables|Default|GetMesh))
  (bind _relativerotation (Variables|/Script/Engine.SceneComponent|GetRelativeRotation _mesh))
  (bind (_roll _pitch) (Math|Rotator|BreakRotator _relativerotation))
  (LocalVariables|SetZRot RotationInput)
  (Utilities|IsValid _mesh
    (:Is%20Valid
      (Transformation|SetRelativeRotation _mesh (Math|Rotator|MakeRotator _roll _pitch (LocalVariables|GetZRot)) false false))))

(fn MoveMesh
  (params (PositionInput :type Float%20%28single-precision%29))
  (bind _mesh (Variables|Default|GetMesh))
  (bind _initialposition (Variables|Default|GetInitialPosition))
  (bind (_x _y _z) (Math|Vector|BreakVector _initialposition))
  (LocalVariables|SetZPos PositionInput)
  (Utilities|IsValid _mesh
    (:Is%20Valid
      (Transformation|SetWorldLocation _mesh (Math|Vector|MakeVector _x _y (+ _z (LocalVariables|GetZPos))) false false))))

(fn SetAnimatingMesh
  (params (ToAnim :type Mesh%20Component%20Object%20Reference))
  (if (Variables|Default|GetAnimationEnabled)
    (bind _output_get (Variables|Default|SetMesh ToAnim))
    (Variables|Default|SetInitialPosition (Transformation|GetWorldLocation _output_get))))