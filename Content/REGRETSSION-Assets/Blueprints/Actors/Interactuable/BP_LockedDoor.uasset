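; BP_LockedDoor is an interactable door that opens only for a player holding the matching colored key.
; CheckInteract casts the interactor to BP_Player and calls CheckHasKey, which maps the door's KeyColor (blue, red or yellow) to the player's corresponding key flag.
; When the key is present the door simply destroys itself, with no animation or key consumption.
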(event EventBeginPlay)

(event Collision|EventActorBeginOverlap
  (params (OtherActor :type Actor%20Object%20Reference)))

(event EventTick
  (params (DeltaSeconds :type Float%20%28single-precision%29)))

(fn ConstructionScript)

(fn CheckHasKey
  (params (Player :type Actor%20Object%20Reference))
  (bind _asfpsreg (Utilities|Casting|CastToBP_Player Player))
  (switch Utilities|FlowControl|Switch|SwitchonENUM_KeyColors (Variables|Default|GetKeyColor)
    (:NewEnumerator0
      (return (Variables|/Game/REGRETSSION-Assets/Blueprints/Player/BP_Player.BP_Player_C|GetHasBlueKey _asfpsreg)))
    (:NewEnumerator1
      (return (Variables|/Game/REGRETSSION-Assets/Blueprints/Player/BP_Player.BP_Player_C|GetHasRedKey _asfpsreg)))
    (:NewEnumerator2
      (return (Variables|/Game/REGRETSSION-Assets/Blueprints/Player/BP_Player.BP_Player_C|GetHasYellowKey _asfpsreg)))))

(fn CheckInteract
  (params (Interactor :type Actor%20Object%20Reference))
  (bind _asfpsreg (Utilities|Casting|CastToBP_Player Interactor))
  (bind _correctkey (CallFunction|CheckHasKey _asfpsreg))
  (if _correctkey
    (Actor|DestroyActor)))