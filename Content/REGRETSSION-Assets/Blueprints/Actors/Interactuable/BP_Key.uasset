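; BP_Key is a key pickup actor that the player collects by overlapping it.
; On overlap with an FPSReg, it passes itself to that actor's CheckPickupKey, then destroys itself.
; A timeline started on BeginPlay bobs the Key component vertically around its initial world position through MoveMesh.
; A RotateMesh function for rolling the key exists, but its call is not connected to execution.
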(event EventBeginPlay
  (Variables|Default|SetInitialPosition (Transformation|GetWorldLocation (Variables|Default|GetKey)))
  (bind (_direction _rotation _position) (Timeline|MeshAnimation PlayFromStart)
    (:Update
      (CallFunction|MoveMesh _position))))

(event Collision|EventActorBeginOverlap
  (params (OtherActor :type Actor%20Object%20Reference))
  (bind _asfpsreg (Utilities|Casting|CastToFPSReg OtherActor))
  (Default|CheckPickupKey _asfpsreg self)
  (Actor|DestroyActor))

(fn ConstructionScript)

(fn RotateMesh
  (params (RotationInput :type Float%20%28single-precision%29))
  (bind _key (Variables|Default|GetKey))
  (bind _relativerotation (Variables|/Script/Engine.SceneComponent|GetRelativeRotation _key))
  (bind (_roll _pitch _yaw) (Math|Rotator|BreakRotator _relativerotation))
  (LocalVariables|SetXRot RotationInput)
  (Utilities|IsValid _key
    (:Is%20Valid
      (Transformation|SetRelativeRotation _key (Math|Rotator|MakeRotator (LocalVariables|GetXRot) _pitch _yaw) false false))))

(fn MoveMesh
  (params (PositionInput :type Float%20%28single-precision%29))
  (bind _initialposition (Variables|Default|GetInitialPosition))
  (bind _key (Variables|Default|GetKey))
  (bind (_x _y _z) (Math|Vector|BreakVector _initialposition))
  (LocalVariables|SetZPos PositionInput)
  (Utilities|IsValid _key
    (:Is%20Valid
      (Transformation|SetWorldLocation _key (Math|Vector|MakeVector _x _y (+ _z (LocalVariables|GetZPos))) false false))))