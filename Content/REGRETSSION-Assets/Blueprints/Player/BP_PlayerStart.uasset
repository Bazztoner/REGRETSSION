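; Player start Blueprint that gives BP_Player its starting ammo and weapons when the level begins.
; After a short BeginPlay delay, it finds the player and initializes its ammo pool from a map, if that map has entries.
; It then adds the starting weapon list to a set, dropping duplicates, and passes that set to the player.
; A FilterWeaponList helper is defined but not called in this Blueprint.
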(event EventBeginPlay
  (Utilities|FlowControl|Delay 0.2)
  (CallFunction|SetPlayerStartingWeapons))

(event EventTick
  (params (DeltaSeconds :type Float%20%28single-precision%29)))

(fn ConstructionScript)

(fn SetPlayerStartingWeapons
  (bind _startingammo (Variables|Default|GetStartingAmmo))
  (bind _returnvalue (Actor|GetActorOfClass "/Game/REGRETSSION-Assets/Blueprints/Player/BP_Player.BP_Player_C"))
  (Utilities|IsValid _returnvalue
    (:Is%20Valid
      (Utilities|FlowControl|Sequence
        (:then_0
          (if (Utilities|Map|IsNotEmpty _startingammo)
            (Default|InitializeAmmoPool _returnvalue _startingammo)))
        (:then_1
          (Utilities|Set|AddItems (LocalVariables|GetStartWeapons) (Variables|Default|GetStartingWeapons))
          (Default|InitializeStartingWeapons _returnvalue (LocalVariables|GetStartWeapons)))))))

(fn FilterWeaponList
  (for _array_element (Variables|Default|GetStartingWeapons)
    (if (Utilities|IsValidClass (LocalVariables|GetCurrentWeapon))
      (if (not (== _array_element (LocalVariables|GetCurrentWeapon)))
        (bind _output_get (LocalVariables|SetCurrentWeapon (LocalVariables|GetCurrentWeapon) :!label _label))
        (Utilities|Array|AddUnique (LocalVariables|GetFilteredWeapons) _output_get))
      (else
        (goto _label))))
  (return (LocalVariables|GetFilteredWeapons)))