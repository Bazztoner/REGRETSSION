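; Hitscan shot actor for player weapons that resolves a multi-pellet shot through line traces from the player camera.
; SpawnHitscan splits damage across pellets, randomizes each direction within horizontal and vertical spread, and spawns muzzle tracers plus surface-based particles and decals.
; ManageHits totals damage per actor, so each victim receives one ApplyPointDamage call, followed by AI damage and noise reports.
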(event Custom|DelayedDestruction
  (Utilities|FlowControl|Delay (Variables|Default|GetLifeTIme))
  (Actor|DestroyActor))

(event EventBeginPlay
  (|CallParentFunction) ; This node is disabled and will not be called.\nDrag off pins to build functionality.
)

(event Collision|EventActorBeginOverlap
  (params (OtherActor :type Actor%20Object%20Reference))
  (|CallParentFunction OtherActor) ; This node is disabled and will not be called.\nDrag off pins to build functionality.
)

(event EventTick
  (params (DeltaSeconds :type Float%20%28single-precision%29))
  (|CallParentFunction DeltaSeconds) ; This node is disabled and will not be called.\nDrag off pins to build functionality.
)

(fn ConstructionScript
  (|CallParentFunction))

(fn SpawnHitscan
  (params (Owner :type BP%20Weapon%20Base%20Object%20Reference) (MaxDistance :type Float%20%28double-precision%29) (Damage :type Float%20%28double-precision%29) (Type :type ENUM_AmmoTypes%20Enum :default "NewEnumerator6") (Pellets :type Integer) (YSpread :type Float%20%28double-precision%29) (ZSpread :type Float%20%28double-precision%29))
  (bind _defaultsceneroot (Variables|Default|GetDefaultSceneRoot))
  (bind _instigator (Variables|Default|GetInstigator))
  (bind _returnvalue (Transformation|GetWorldLocation _defaultsceneroot))
  (Utilities|FlowControl|Sequence
    (:then_0
      (Variables|Default|SetFromWeapon Owner)
      (Variables|Default|SetDamage (/ Damage (Math|Conversions|ToFloat(Integer) Pellets)))
      (Variables|Default|SetMaxRange MaxDistance)
      (Variables|Default|SetAmmoType Type)
      (Variables|Default|SetPellets Pellets)
      (Variables|Default|SetHorizontalSpread ZSpread)
      (Variables|Default|SetVerticalSpread YSpread))
    (:then_1
      (bind _asfpsreg (Utilities|Casting|CastToBP_Player (Game|GetInstigator)))
      (bind (_location _forwardvector) (Default|GetCameraInfo _asfpsreg))
      (Utilities|FlowControl|Sequence
        (:then_0
          (LocalVariables|SetStartPos _location)
          (LocalVariables|SetDirection _forwardvector))
        (:then_1
          (for _index (range 1 (Variables|Default|GetPellets))
            (bind _rotatedvector (CallFunction|GetRandomizedDirection (LocalVariables|GetDirection) (* -1 (Variables|Default|GetHorizontalSpread)) (Variables|Default|GetHorizontalSpread) (Math|Vector|GetUpVector (Variables|Default|GetDefaultSceneRoot))))
            (bind _rotatedvector_2 (CallFunction|GetRandomizedDirection _rotatedvector (* -1 (Variables|Default|GetVerticalSpread)) (Variables|Default|GetVerticalSpread) (Math|Vector|GetRightVector (Variables|Default|GetDefaultSceneRoot))))
            (bind (_outhit _returnvalue_2) (Collision|LineTraceByChannel (LocalVariables|GetStartPos) (+ (LocalVariables|GetStartPos) (* _rotatedvector_2 (Variables|Default|GetMaxRange))) "TraceTypeQuery1" false 0 "None" true "(R=0.859016,G=0.000000,B=1.000000,A=1.000000)" "(R=0.000000,G=1.000000,B=0.980904,A=1.000000)" 2.0))
            (if _returnvalue_2
              (CallFunction|SpawnTracer (.ImpactPoint (Collision|BreakHitResult _outhit)))
              (if (Utilities|IsValid (.HitActor (Collision|BreakHitResult _outhit)))
                (CallFunction|CheckSpawnHitParticle (Variables|/Script/PhysicsCore.PhysicalMaterial|GetSurfaceType (.PhysMat (Collision|BreakHitResult _outhit))) (.ImpactPoint (Collision|BreakHitResult _outhit)) (.ImpactNormal (Collision|BreakHitResult _outhit)))
                (CallFunction|CheckSpawnHitDecal false (Variables|/Script/PhysicsCore.PhysicalMaterial|GetSurfaceType (.PhysMat (Collision|BreakHitResult _outhit))) "1.500000,4.000000,4.000000" 0 (.ImpactPoint (Collision|BreakHitResult _outhit)) (Math|Conversions|RotationFromXVector (.ImpactNormal (Collision|BreakHitResult _outhit))) 3e+02)
                (bind _modifiedmap (CallFunction|ManageHits (LocalVariables|GetDamageToEnemies) (.HitActor (Collision|BreakHitResult _outhit)) (Variables|Default|GetDamage)))
                (LocalVariables|SetDamageToEnemies _modifiedmap))
              (else
                (CallFunction|SpawnTracer (+ (LocalVariables|GetStartPos) (* _rotatedvector_2 (Variables|Default|GetMaxRange)))))))
          (bind _keys (Utilities|Map|Keys (LocalVariables|GetDamageToEnemies)))
          (for _array_element _keys
            (Game|Damage|ApplyPointDamage _array_element (.Value (Utilities|Map|Find (LocalVariables|GetDamageToEnemies) _array_element)) (Math|Vector|Normalize (- (Transformation|GetActorLocation _array_element) (Transformation|GetWorldLocation (Variables|Default|GetDefaultSceneRoot)))) (Collision|MakeHitResult false false 0.0 0.0 "0, 0, 0" "0, 0, 0" "0,0,1" "0,0,1" 0 0) (Game|GetInstigatorController) _instigator)
            (Class|AISenseDamage|ReportDamageEvent _array_element _instigator (.Value (Utilities|Map|Find (LocalVariables|GetDamageToEnemies) _array_element)) _returnvalue "0, 0, 0" "None")
            (Class|AISenseHearing|ReportNoiseEvent _returnvalue 1.0 (Variables|/Game/REGRETSSION-Assets/Blueprints/Player/Weapons/BP_WeaponBase.BP_WeaponBase_C|GetPlayerOwner (Variables|Default|GetFromWeapon)) 0.0 "None")))))))

(fn ManageHits
  (params (Hits :type Map%20of%20Actor%20Object%20References%20to%20Reals) (Actor :type Actor%20Object%20Reference) (Damage :type Float%20%28double-precision%29))
  (bind (_value _returnvalue) (Utilities|Map|Find Hits Actor))
  (Utilities|FlowControl|Sequence
    (:then_0
      (if _returnvalue
        (LocalVariables|SetDamageForActor (+ _value Damage))
        (else
          (LocalVariables|SetDamageForActor Damage))))
    (:then_1
      (Utilities|Map|Add Hits Actor (LocalVariables|GetDamageForActor))
      (return Hits))))

(fn SpawnTracer
  (params (ImpactPoint :type Vector))
  (bind _fromweapon (Variables|Default|GetFromWeapon))
  (bind _muzzle (Variables|/Game/REGRETSSION-Assets/Blueprints/Player/Weapons/BP_WeaponBase.BP_WeaponBase_C|GetMuzzle _fromweapon))
  (bind _returnvalue (Transformation|GetSocketLocation _muzzle "None"))
  (if (>= (Math|Vector|DotProduct (Math|Vector|GetForwardVector _muzzle) (Math|Vector|Normalize (- ImpactPoint _returnvalue))) 0.0)
    (Game|SpawnActorfromClass (Variables|Default|GetTracer) (Math|Transform|MakeTransform _returnvalue (Math|Rotator|FindLookatRotation _returnvalue ImpactPoint) "1.000000,1.000000,1.000000") "Undefined" "SelectDefaultAtRuntime" (Variables|Default|GetFromWeapon) 1.0 ImpactPoint (Variables|Default|GetInstigator))))

(fn CheckActorHit
  (params (HittedActor :type Actor%20Object%20Reference) (ImpactPoint :type Vector) (ImpactNormal :type Vector))
  (bind _asbp_ihittable (Utilities|Casting|CastToBP_IHittable HittedActor))
  (Default|OnDamagingImpact _asbp_ihittable ImpactPoint ImpactNormal "NewEnumerator0" (Variables|/Game/REGRETSSION-Assets/Blueprints/Player/Weapons/BP_WeaponBase.BP_WeaponBase_C|GetAmmoType (Variables|Default|GetFromWeapon))))