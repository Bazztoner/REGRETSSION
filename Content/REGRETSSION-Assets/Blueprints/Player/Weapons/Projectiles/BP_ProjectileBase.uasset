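; BP_ProjectileBase is the base weapon projectile Blueprint, providing shared helpers for surface-dependent hit effects.
; CheckSpawnHitParticle asks the REG_GameInstance particle manager for the surface's particle and, if found, spawns it oriented along the impact normal.
; CheckSpawnHitDecal uses the decal manager to spawn a physical-surface decal, either attached or at a location.
; The event graph and construction script are empty, and neither helper is called here.
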(event EventBeginPlay)

(event Collision|EventActorBeginOverlap
  (params (OtherActor :type Actor%20Object%20Reference)))

(event EventTick
  (params (DeltaSeconds :type Float%20%28single-precision%29)))

(fn ConstructionScript)

(fn CheckSpawnHitParticle
  (params (Surface :type EPhysicalSurface%20Enum :default "SurfaceType_Default") (ImpactPoint :type Vector) (ImpactNormal :type Vector))
  (bind _asreg_game_instance (Utilities|Casting|CastToREG_GameInstance (Game|GetGameInstance)))
  (bind _particlemanagerinstance (Default|GetParticleManager _asreg_game_instance))
  (bind (_particle _foundany) (Default|GetHitParticle _particlemanagerinstance Surface))
  (if _foundany
    (Default|SpawnHitParticle _particlemanagerinstance _particle (Math|Transform|MakeTransform ImpactPoint (Math|Rotator|MakeRotfromX ImpactNormal)))))

(fn CheckSpawnHitDecal
  (params (Attached :type Boolean) (PhysicalSurface :type EPhysicalSurface%20Enum :default "SurfaceType_Default") (DecalSIze :type Vector) (AttachTo :type Scene%20Component%20Object%20Reference) (Location :type Vector) (Rotation :type Rotator) (LifeSpan :type Float%20%28double-precision%29))
  (bind _asreg_game_instance (Utilities|Casting|CastToREG_GameInstance (Game|GetGameInstance)))
  (bind _decalmanagerinstance (Default|GetDecalManager _asreg_game_instance))
  (if Attached
    (Default|SpawnDecalAttached _decalmanagerinstance PhysicalSurface DecalSIze AttachTo Location Rotation LifeSpan)
    (else
      (Default|SpawnDecalatLocation _decalmanagerinstance PhysicalSurface DecalSIze Location Rotation LifeSpan))))