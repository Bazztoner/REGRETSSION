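; BP_DummyExplosion is an explosion actor that deals environmental damage around its location, with sound, and destroys itself after LifeTime once ManageDestuction fires.
; Explode sphere-traces on Visibility, then applies radial damage and spawns particles for every hit.
; ExplodeGeneric is a variant using direct per-hit damage, debug drawing and no particles.
; Both report damage events for each hit; neither is called within this Blueprint.
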(event Custom|ManageDestuction
  (Utilities|FlowControl|Delay (Variables|Default|GetLifeTime))
  (CallFunction|DelayedDestruction))

(fn ConstructionScript)

(fn Explode
  (bind _returnvalue (Transformation|GetActorLocation))
  (Audio|Components|Audio|Play (Variables|Default|GetExplosionSound) 0.0)
  (bind _outhits (Collision|MultiSphereTraceByChannel _returnvalue _returnvalue (Variables|Default|GetExplosionRadius) "TraceTypeQuery1" false 0 "None" true "(R=1.000000,G=0.000000,B=0.000000,A=1.000000)" "(R=0.000000,G=1.000000,B=0.000000,A=1.000000)" 2.0))
  (for _array_element _outhits
    (Game|Damage|ApplyRadialDamage (Variables|Default|GetDamage) (.Location (Collision|BreakHitResult _array_element)) (Variables|Default|GetExplosionRadius) "/Engine/EngineDamageTypes/DmgTypeBP_Environmental.DmgTypeBP_Environmental_C" 0 (.HitActor (Collision|BreakHitResult _array_element)) (Game|GetInstigatorController) true "ECC_Visibility")
    (Class|AISenseDamage|ReportDamageEvent (.HitActor (Collision|BreakHitResult _array_element)) 0 0.0 (.Location (Collision|BreakHitResult _array_element)) (.ImpactPoint (Collision|BreakHitResult _array_element)) "None")
    (CallFunction|SpawnExplosionParticles)))

(fn DelayedDestruction
  (Actor|DestroyActor))

(fn ExplodeGeneric
  (bind _returnvalue (Transformation|GetActorLocation))
  (bind _instigator (Variables|Actor|GetInstigator))
  (Audio|Components|Audio|Play (Variables|Default|GetExplosionSound) 0.0)
  (bind _outhits (Collision|MultiSphereTraceByChannel _returnvalue _returnvalue (Variables|Default|GetExplosionRadius) "TraceTypeQuery1" false 0 "ForDuration" true "(R=1.000000,G=0.000000,B=0.000000,A=1.000000)" "(R=0.000000,G=1.000000,B=0.000000,A=1.000000)" 2.0))
  (for _array_element _outhits
    (bind _returnvalue_2 (Game|Damage|ApplyDamage (.HitActor (Collision|BreakHitResult _array_element)) (Variables|Default|GetDamage) (Game|GetInstigatorController) _instigator "/Engine/EngineDamageTypes/DmgTypeBP_Environmental.DmgTypeBP_Environmental_C"))
    (Class|AISenseDamage|ReportDamageEvent (.HitActor (Collision|BreakHitResult _array_element)) _instigator _returnvalue_2 (.Location (Collision|BreakHitResult _array_element)) "0, 0, 0" "None")))

(fn SpawnExplosionParticles
  (Effects|SpawnEmitteratLocation (Variables|Default|GetExplosionParticle) (Transformation|GetWorldLocation (Variables|Default|GetDefaultSceneRoot)) "0, 0, 0" "1.000000,1.000000,1.000000" true "AutoRelease"))