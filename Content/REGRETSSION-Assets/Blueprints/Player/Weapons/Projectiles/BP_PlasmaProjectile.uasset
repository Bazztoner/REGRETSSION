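; Plasma weapon projectile that flies straight forward and explodes on overlapping actors.
; Initialize stores weapon, damage, ammo and particle data, enables overlap collision and starts a lifetime delay; Tick moves it without sweeping.
; Explode ignores the instigator and trigger-tagged actors, then places an ammo-based decal, spawns an ExplosionDummy to handle the blast and destroys the projectile.
; Lifetime expiry passes no actor to Explode, so its validity check blocks detonation.
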(event Custom|InitializeTimedLife
  (Utilities|FlowControl|Delay (Variables|Default|GetLifeTIme))
  (CallFunction|Explode))

(event EventTick
  (params (DeltaSeconds :type Float%20%28single-precision%29))
  (CallFunction|HandleMovement DeltaSeconds))

(event Collision|EventActorBeginOverlap
  (params (OtherActor :type Actor%20Object%20Reference))
  (if (Variables|Default|GetbInitialized)
    (CallFunction|Explode OtherActor)))

(fn ConstructionScript
  (|CallParentFunction))

(fn HandleMovement
  (params (DeltaTime :type Float%20%28double-precision%29))
  (Transformation|AddActorWorldOffset self (* (Transformation|GetActorForwardVector self) (* (Variables|Default|GetMovementSpeed) DeltaTime))))

(fn Initialize
  (params (From :type BP%20Weapon%20Base%20Object%20Reference) (Damage :type Float%20%28double-precision%29) (AmmoType :type ENUM_AmmoTypes%20Enum :default "NewEnumerator6") (LifeTime :type Float%20%28double-precision%29) (Radius :type Float%20%28double-precision%29) (ExplosionParticle :type Particle%20System%20Object%20Reference))
  (Variables|Default|SetFromWeapon From)
  (Variables|Default|SetDamage Damage)
  (Variables|Default|SetAmmoType AmmoType)
  (Variables|Default|SetExplosionParticle ExplosionParticle)
  (Variables|Default|SetbInitialized true)
  (CallFunction|InitializeTimedLife)
  (Collision|SetCollisionProfileName (Variables|Default|GetStaticMesh) "OverlapAll" true :!class /Script/Engine.PrimitiveComponent))

(fn Explode
  (params (OverlappedActor :type Actor%20Object%20Reference))
  (Utilities|IsValid OverlappedActor
    (:Is%20Valid
      ;[1 0.7619 1] If the overlapped actor is not the player nor a Weapon pickup
      (if (not (Actor|ActorHasTag OverlappedActor (GameplayTags|GetTagName (GameplayTags|MakeLiteralGameplayTag "(TagName=\"Entities.Trigger\")"))))
        (if (!= OverlappedActor (Variables|Default|GetInstigator))
          (Utilities|FlowControl|Sequence
            (:then_0
              (bind _asreg_game_instance (Utilities|Casting|CastToREG_GameInstance (Game|GetGameInstance)))
              (bind _decalmanagerinstance (Default|GetDecalManager _asreg_game_instance))
              (Default|SpawnDecalbyAmmoatLocation _decalmanagerinstance "15.000000,15.000000,15.000000" (Transformation|GetActorLocation) (Math|Conversions|RotationFromXVector (* (Transformation|GetActorForwardVector) "-1.000000,1.000000,1.000000")) 3e+02 (Variables|Default|GetAmmoType)))
            (:then_1
              (CallFunction|SpawnExplosion)
              (Actor|DestroyActor))))))))

(fn SpawnExplosion
  (bind _returnvalue (Game|SpawnActorfromClass (Variables|Default|GetExplosionDummy) (Transformation|GetActorTransform) "AlwaysSpawn" "SelectDefaultAtRuntime" 0 (Variables|Default|GetExplosionRadius) (Variables|Default|GetDamage) (Variables|/Game/REGRETSSION-Assets/Blueprints/Player/Weapons/BP_WeaponBase.BP_WeaponBase_C|GetPlayerOwner (Variables|Default|GetFromWeapon)) (Variables|Default|GetFromWeapon) self (Variables|Default|GetExplosionParticle) (Variables|Default|GetInstigator)))
  (Default|Explode _returnvalue))