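; BP_HitscanBullet is a hitscan shot actor that a weapon initializes through SpawnHitscan with range, damage, ammo type and spread.
; It line-traces from the player camera, randomizing spread by rotating the world-space end point in roll and yaw.
; Hits apply point damage, report damage and noise to AI, and trigger surface-based particles and decals.
; Tracers fly from the muzzle toward the hit or end point, skipped when it lies behind the muzzle.
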(event Custom|DelayedDestruction
  (Utilities|FlowControl|Delay (Variables|Default|GetLifeTIme))
  (Actor|DestroyActor))

(event EventBeginPlay)

(event Collision|EventActorBeginOverlap
  (params (OtherActor :type Actor%20Object%20Reference)))

(event EventTick
  (params (DeltaSeconds :type Float%20%28single-precision%29)))

(fn ConstructionScript)

(fn SpawnHitscan
  (params (Owner :type BP%20Weapon%20Base%20Object%20Reference) (MaxDistance :type Float%20%28double-precision%29) (Damage :type Float%20%28double-precision%29) (Type :type ENUM_AmmoTypes%20Enum :default "NewEnumerator6") (XSpread :type Float%20%28double-precision%29) (YSpread :type Float%20%28double-precision%29))
  (bind _instigator (Variables|Default|GetInstigator))
  (Utilities|FlowControl|Sequence
    (:then_0
      (Variables|Default|SetFromWeapon Owner)
      (Variables|Default|SetDamage Damage)
      (Variables|Default|SetMaxRange MaxDistance)
      (Variables|Default|SetAmmoType Type))
    (:then_1
      (bind _asfpsreg (Utilities|Casting|CastToBP_Player (Game|GetInstigator)))
      ;[1 1 1] Shoot From Camera
      (bind (_location _forwardvector) (Default|GetCameraInfo _asfpsreg))
      (bind _output_get (LocalVariables|SetRaycastEndPoint (Math|Vector|RotateVector (+ _location (* _forwardvector (Variables|Default|GetMaxRange))) (Math|Rotator|MakeRotator (Math|Random|RandomFloatinRange (* -1 XSpread) XSpread) 0.0 (Math|Random|RandomFloatinRange (* -1 YSpread) YSpread)))))
      (bind (_outhit _returnvalue) (Collision|LineTraceByChannel _location _output_get "TraceTypeQuery1" false 0 "None" true "(R=0.859016,G=0.000000,B=1.000000,A=1.000000)" "(R=0.000000,G=1.000000,B=0.980904,A=1.000000)" 2.0))
      (if _returnvalue
        (CallFunction|SpawnTracer (.ImpactPoint (Collision|BreakHitResult _outhit)))
        (Game|Damage|ApplyPointDamage (.HitActor (Collision|BreakHitResult _outhit)) (Variables|Default|GetDamage) (.ImpactNormal (Collision|BreakHitResult _outhit)) _outhit (Game|GetInstigatorController) _instigator)
        (Class|AISenseDamage|ReportDamageEvent (.HitActor (Collision|BreakHitResult _outhit)) _instigator (Variables|Default|GetDamage) (.Location (Collision|BreakHitResult _outhit)) (.ImpactPoint (Collision|BreakHitResult _outhit)) "None")
        (Class|AISenseHearing|ReportNoiseEvent (Transformation|GetWorldLocation (Variables|Default|GetDefaultSceneRoot)) 1.0 (Variables|/Game/REGRETSSION-Assets/Blueprints/Player/Weapons/BP_WeaponBase.BP_WeaponBase_C|GetPlayerOwner (Variables|Default|GetFromWeapon)) 0.0 "None")
        (CallFunction|CheckSpawnHitParticle (Variables|/Script/PhysicsCore.PhysicalMaterial|GetSurfaceType (.PhysMat (Collision|BreakHitResult _outhit))) (.ImpactPoint (Collision|BreakHitResult _outhit)) (.ImpactNormal (Collision|BreakHitResult _outhit)))
        (CallFunction|CheckSpawnHitDecal false (Variables|/Script/PhysicsCore.PhysicalMaterial|GetSurfaceType (.PhysMat (Collision|BreakHitResult _outhit))) "1.500000,4.000000,4.000000" 0 (.ImpactPoint (Collision|BreakHitResult _outhit)) (Math|Conversions|RotationFromXVector (.ImpactNormal (Collision|BreakHitResult _outhit))) 3e+02)
        (return (.ImpactPoint (Collision|BreakHitResult _outhit)) (.ImpactNormal (Collision|BreakHitResult _outhit)))
        (else
          (CallFunction|SpawnTracer (LocalVariables|GetRaycastEndPoint)))))))

(fn SpawnTracer
  (params (Impact%20Point :type Vector))
  (bind _fromweapon (Variables|Default|GetFromWeapon))
  (bind _muzzle (Variables|/Game/REGRETSSION-Assets/Blueprints/Player/Weapons/BP_WeaponBase.BP_WeaponBase_C|GetMuzzle _fromweapon))
  (bind _returnvalue (Transformation|GetSocketLocation _muzzle "None"))
  (if (>= (Math|Vector|DotProduct (Math|Vector|GetForwardVector _muzzle) (Math|Vector|Normalize (- Impact%20Point _returnvalue))) 0.0)
    (Game|SpawnActorfromClass (Variables|Default|GetTracer) (Math|Transform|MakeTransform _returnvalue (Math|Rotator|FindLookatRotation _returnvalue Impact%20Point) "1.000000,1.000000,1.000000") "Undefined" "SelectDefaultAtRuntime" (Variables|Default|GetFromWeapon) 1.0 Impact%20Point (Variables|Default|GetInstigator))))

(fn CheckActorHit
  (params (HittedActor :type Actor%20Object%20Reference) (ImpactPoint :type Vector) (ImpactNormal :type Vector)))