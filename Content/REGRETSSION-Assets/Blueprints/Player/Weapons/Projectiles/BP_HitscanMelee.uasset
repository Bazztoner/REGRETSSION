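; BP_HitscanMelee is a melee weapon hitscan actor that resolves a player's strike as an instant line trace.
; SpawnHitscan stores weapon, range, damage and ammo type, then traces on Visibility from the instigating BP_Player's camera.
; Hits apply point damage, report a damage event for AI hearing or sight, and spawn surface-based particles.
; Tracer and BP_IHittable helpers exist but SpawnHitscan skips them; DelayedDestruction removes the actor after its lifetime.
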(event Custom|DelayedDestruction
  (Utilities|FlowControl|Delay (Variables|Default|GetLifeTIme))
  (Actor|DestroyActor))

(event EventBeginPlay)

(event Collision|EventActorBeginOverlap
  (params (OtherActor :type Actor%20Object%20Reference)))

(event EventTick
  (params (DeltaSeconds :type Float%20%28single-precision%29)))

(fn ConstructionScript)

(fn SpawnHitscan
  (params (Owner :type BP%20Weapon%20Base%20Object%20Reference) (MaxDistance :type Float%20%28double-precision%29) (Damage :type Float%20%28double-precision%29) (Type :type ENUM_AmmoTypes%20Enum :default "NewEnumerator6"))
  (bind _instigator (Variables|Default|GetInstigator))
  (Utilities|FlowControl|Sequence
    (:then_0
      (Variables|Default|SetFromWeapon Owner)
      (Variables|Default|SetDamage Damage)
      (Variables|Default|SetMaxRange MaxDistance)
      (Variables|Default|SetAmmoType Type))
    (:then_1
      (bind _asfpsreg (Utilities|Casting|CastToBP_Player (Game|GetInstigator)))
      ;[1 1 1] Shoot From Camera
      (bind (_location _forwardvector) (Default|GetCameraInfo _asfpsreg))
      (bind (_outhit _returnvalue) (Collision|LineTraceByChannel _location (+ _location (* _forwardvector (Variables|Default|GetMaxRange))) "TraceTypeQuery1" false 0 "None" true "(R=0.859016,G=0.000000,B=1.000000,A=1.000000)" "(R=0.000000,G=1.000000,B=0.980904,A=1.000000)" 2.0))
      (if _returnvalue
        (Game|Damage|ApplyPointDamage (.HitActor (Collision|BreakHitResult _outhit)) (Variables|Default|GetDamage) (.ImpactNormal (Collision|BreakHitResult _outhit)) _outhit (Game|GetInstigatorController) _instigator)
        (Class|AISenseDamage|ReportDamageEvent (.HitActor (Collision|BreakHitResult _outhit)) _instigator (Variables|Default|GetDamage) (.Location (Collision|BreakHitResult _outhit)) (.ImpactPoint (Collision|BreakHitResult _outhit)) "None")
        (CallFunction|CheckSpawnHitParticle (Variables|/Script/PhysicsCore.PhysicalMaterial|GetSurfaceType (.PhysMat (Collision|BreakHitResult _outhit))) (.ImpactPoint (Collision|BreakHitResult _outhit)) (.ImpactNormal (Collision|BreakHitResult _outhit)))
        (return (.ImpactPoint (Collision|BreakHitResult _outhit)) (.ImpactNormal (Collision|BreakHitResult _outhit)))))))

(fn SpawnTracer
  (params (Impact%20Point :type Vector))
  (Game|SpawnActorfromClass (Variables|Default|GetTracer) (Math|Transform|MakeTransform (Transformation|GetWorldLocation (Variables|/Game/REGRETSSION-Assets/Blueprints/Player/Weapons/BP_WeaponBase.BP_WeaponBase_C|GetMuzzle (Variables|Default|GetFromWeapon))) "0, 0, 0" "1.000000,1.000000,1.000000") "Undefined" "SelectDefaultAtRuntime" (Variables|Default|GetFromWeapon) 0.25 Impact%20Point (Variables|Default|GetInstigator)))

(fn CheckActorHit
  (params (HittedActor :type Actor%20Object%20Reference) (ImpactPoint :type Vector) (ImpactNormal :type Vector))
  (bind _asbp_ihittable (Utilities|Casting|CastToBP_IHittable HittedActor))
  (Default|OnDamagingImpact _asbp_ihittable ImpactPoint ImpactNormal "NewEnumerator0" (Variables|/Game/REGRETSSION-Assets/Blueprints/Player/Weapons/BP_WeaponBase.BP_WeaponBase_C|GetAmmoType (Variables|Default|GetFromWeapon))))