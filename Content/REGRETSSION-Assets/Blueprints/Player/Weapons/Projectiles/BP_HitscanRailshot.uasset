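; Hitscan railshot projectile for player weapons that pierces multiple actors along the camera's aim, up to a hit limit.
; SpawnHitscan chains line traces from each impact point, ignoring actors already hit, applying and reporting damage and notifying BP_IHittable actors.
; Tracers spawn for each hit or miss, oriented from the weapon muzzle, while the game instance's decal manager marks the final impact.
; It also reports a noise event at the actor's location.
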(event Custom|DelayedDestruction
  (Utilities|FlowControl|Delay (Variables|Default|GetLifeTIme))
  (Actor|DestroyActor))

(event EventBeginPlay)

(event Collision|EventActorBeginOverlap
  (params (OtherActor :type Actor%20Object%20Reference)))

(event EventTick
  (params (DeltaSeconds :type Float%20%28single-precision%29)))

(fn ConstructionScript)

(fn SpawnHitscan
  (params (Owner :type BP%20Weapon%20Base%20Object%20Reference) (MaxDistance :type Float%20%28double-precision%29) (Damage :type Float%20%28double-precision%29) (Type :type ENUM_AmmoTypes%20Enum :default "NewEnumerator6") (MaximumHits :type Integer))
  (bind _instigator (Variables|Default|GetInstigator))
  (bind _instigator_2 (Variables|Default|GetInstigator))
  (Utilities|FlowControl|Sequence
    (:then_0
      ;[1 1 1] Variables Set
      (Variables|Default|SetFromWeapon Owner)
      (Variables|Default|SetDamage Damage)
      (Variables|Default|SetMaxRange MaxDistance)
      (Variables|Default|SetAmmoType Type)
      (Variables|Default|SetMaxHits MaximumHits))
    (:then_1
      (bind _asfpsreg (Utilities|Casting|CastToBP_Player (Game|GetInstigator)))
      ;[1 1 1] Shoot From Camera
      (bind (_location _forwardvector) (Default|GetCameraInfo _asfpsreg))
      (bind (_outhit _returnvalue) (Collision|LineTraceByChannel _location (+ _location (* _forwardvector (Variables|Default|GetMaxRange))) "TraceTypeQuery1" false 0 "None" true "(R=0.859016,G=0.000000,B=1.000000,A=1.000000)" "(R=0.000000,G=1.000000,B=0.980904,A=1.000000)" 2.0))
      (if _returnvalue
        ;[1 1 1] Set next raycast from impact point, then ignore hit actor to avoid re-hitting it
        (bind _output_get (LocalVariables|SetNextRaycastStart (.ImpactPoint (Collision|BreakHitResult _outhit))))
        (bind _output_get_2 (LocalVariables|SetFinalImpactPoint _output_get))
        (CallFunction|SpawnTracer _output_get_2)
        (bind _output_get_3 (LocalVariables|SetFinalImpactNormal (.ImpactNormal (Collision|BreakHitResult _outhit))))
        (CallFunction|CheckActorHit (.HitActor (Collision|BreakHitResult _outhit)) _output_get_2 _output_get_3)
        (Utilities|Array|AddUnique (LocalVariables|GetActorsToIgnore) (.HitActor (Collision|BreakHitResult _outhit)))
        (Game|Damage|ApplyPointDamage (.HitActor (Collision|BreakHitResult _outhit)) (Variables|Default|GetDamage) _output_get_3 _outhit (Game|GetInstigatorController) _instigator_2)
        (Class|AISenseDamage|ReportDamageEvent (.HitActor (Collision|BreakHitResult _outhit)) _instigator_2 (Variables|Default|GetDamage) (.Location (Collision|BreakHitResult _outhit)) (.ImpactPoint (Collision|BreakHitResult _outhit)) "None")
        ;[1 1 1] First index is 2 because we already shot a raycast
        (Utilities|FlowControl|ForLoopwithBreak 2 (Variables|Default|GetMaxHits) :!label _label
          (:LoopBody
            (bind (_outhit_2 _returnvalue_2) (Collision|LineTraceByChannel (LocalVariables|GetNextRaycastStart) (+ _location (* _forwardvector (Variables|Default|GetMaxRange))) "TraceTypeQuery1" false (LocalVariables|GetActorsToIgnore) "None" true "(R=0.859016,G=0.000000,B=1.000000,A=1.000000)" "(R=0.000000,G=1.000000,B=0.980904,A=1.000000)" 2.0))
            ;[1 1 1] If we don't hit anything, break the loop
            (if _returnvalue_2
              (Utilities|Array|AddUnique (LocalVariables|GetActorsToIgnore) (.HitActor (Collision|BreakHitResult _outhit_2)))
              (bind _output_get_4 (LocalVariables|SetFinalImpactNormal (.ImpactNormal (Collision|BreakHitResult _outhit_2))))
              (Game|Damage|ApplyPointDamage (.HitActor (Collision|BreakHitResult _outhit_2)) (Variables|Default|GetDamage) _output_get_4 _outhit_2 (Game|GetInstigatorController) _instigator)
              (Class|AISenseDamage|ReportDamageEvent (.HitActor (Collision|BreakHitResult _outhit_2)) _instigator (Variables|Default|GetDamage) (.Location (Collision|BreakHitResult _outhit_2)) (.ImpactPoint (Collision|BreakHitResult _outhit_2)) "None")
              (bind _output_get_5 (LocalVariables|SetNextRaycastStart (.ImpactPoint (Collision|BreakHitResult _outhit_2))))
              (bind _output_get_6 (LocalVariables|SetFinalImpactPoint _output_get_5))
              (CallFunction|SpawnTracer _output_get_6)
              (CallFunction|CheckActorHit (.HitActor (Collision|BreakHitResult _outhit_2)) _output_get_6 _output_get_4)
              (else
                (CallFunction|SpawnTracer (+ _location (* _forwardvector (Variables|Default|GetMaxRange))))
                (goto _label Break))))
          (:Completed
            (bind _asreg_game_instance (Utilities|Casting|CastToREG_GameInstance (Game|GetGameInstance)))
            (bind _decalmanagerinstance (Default|GetDecalManager _asreg_game_instance))
            (Default|SpawnDecalbyAmmoatLocation _decalmanagerinstance "15.000000,15.000000,15.000000" (LocalVariables|GetFinalImpactPoint) (Math|Conversions|RotationFromXVector (LocalVariables|GetFinalImpactNormal)) 3e+02 (Variables|Default|GetAmmoType))))
        (else
          (CallFunction|SpawnTracer (+ _location (* _forwardvector (Variables|Default|GetMaxRange)))))))
    (:then_2
      (Class|AISenseHearing|ReportNoiseEvent (Transformation|GetActorLocation) 1.0 (Variables|/Game/REGRETSSION-Assets/Blueprints/Player/Weapons/BP_WeaponBase.BP_WeaponBase_C|GetPlayerOwner (Variables|Default|GetFromWeapon)) 0.0 "None"))))

(fn SpawnTracer
  (params (ImpactPoint :type Vector))
  (Game|SpawnActorfromClass (Variables|Default|GetTracer) (Math|Transform|MakeTransform ImpactPoint (Math|Rotator|FindLookatRotation (Transformation|GetWorldLocation (Variables|/Game/REGRETSSION-Assets/Blueprints/Player/Weapons/BP_WeaponBase.BP_WeaponBase_C|GetMuzzle (Variables|Default|GetFromWeapon))) ImpactPoint) "1.000000,1.000000,1.000000") "Undefined" "SelectDefaultAtRuntime" (Variables|Default|GetFromWeapon) 1.0 ImpactPoint (Variables|Default|GetInstigator)))

(fn CheckActorHit
  (params (HittedActor :type Actor%20Object%20Reference) (ImpactPoint :type Vector) (ImpactNormal :type Vector))
  (bind _asbp_ihittable (Utilities|Casting|CastToBP_IHittable HittedActor))
  (Default|OnDamagingImpact _asbp_ihittable ImpactPoint ImpactNormal "NewEnumerator0" (Variables|/Game/REGRETSSION-Assets/Blueprints/Player/Weapons/BP_WeaponBase.BP_WeaponBase_C|GetAmmoType (Variables|Default|GetFromWeapon))))