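; Rocket projectile fired by a weapon, moving forward each Tick without sweep and exploding on overlap or timeout.
; Overlaps with trigger-tagged actors and the instigator are ignored.
; Exploding spawns an explosion dummy carrying damage and weapon ownership, places an ammo-type decal through the game instance's decal manager, then removes the trail and actor.
; InitializeRocket arms it but ignores its LifeTime and Radius inputs, hardcoding the lifetime.
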(event Custom|InitializeTimedLife
  (Utilities|FlowControl|Delay (Variables|Default|GetLifeTIme))
  (CallFunction|Explode))

(event EventBeginPlay)

(event EventTick
  (params (DeltaSeconds :type Float%20%28single-precision%29))
  (CallFunction|HandleMovement DeltaSeconds))

(event Collision|EventActorBeginOverlap
  (params (OtherActor :type Actor%20Object%20Reference))
  (if (Variables|Default|GetbInitialized)
    (CallFunction|Explode OtherActor)))

(fn ConstructionScript
  (|CallParentFunction))

(fn HandleMovement
  (params (DeltaTime :type Float%20%28double-precision%29))
  (Transformation|AddActorWorldOffset self (* (Transformation|GetActorForwardVector self) (* (Variables|Default|GetMovementSpeed) DeltaTime))))

(fn InitializeRocket
  (params (From :type BP%20Weapon%20Base%20Object%20Reference) (Damage :type Float%20%28double-precision%29) (Type :type ENUM_AmmoTypes%20Enum :default "NewEnumerator6") (LifeTime :type Float%20%28double-precision%29) (Radius :type Float%20%28double-precision%29) (ExplosionParticle :type Particle%20System%20Object%20Reference))
  (Variables|Default|SetFromWeapon From)
  (Variables|Default|SetDamage Damage)
  (Variables|Default|SetAmmoType Type)
  (Variables|Default|SetLifeTIme 15.0)
  (Variables|Default|SetExplosionParticle ExplosionParticle)
  (Variables|Default|SetbInitialized true)
  (CallFunction|InitializeTimedLife))

(fn Explode
  (params (OverlappedActor :type Actor%20Object%20Reference))
  ;[1 0.7619 1] If the overlapped actor is not the player nor a Weapon pickup
  (if (not (Actor|ActorHasTag OverlappedActor (GameplayTags|GetTagName (GameplayTags|MakeLiteralGameplayTag "(TagName=\"Entities.Trigger\")"))))
    (if (!= OverlappedActor (Variables|Default|GetInstigator))
      (CallFunction|SpawnExplosion)
      (Utilities|FlowControl|Sequence
        (:then_0
          (bind _asreg_game_instance (Utilities|Casting|CastToREG_GameInstance (Game|GetGameInstance)))
          (bind _decalmanagerinstance (Default|GetDecalManager _asreg_game_instance))
          (Default|SpawnDecalbyAmmoatLocation _decalmanagerinstance "50.000000,50.000000,50.000000" (Transformation|GetActorLocation) (Math|Conversions|RotationFromXVector (* (Transformation|GetActorForwardVector) "-1.000000,1.000000,1.000000")) 3e+02 (Variables|Default|GetAmmoType)))
        (:then_1
          (bind __livetrail (Variables|Default|Get_liveTrail)
            (:then
              (Components|Activation|SetActive __livetrail false false)
              (Class|NiagaraComponent|SetRenderingEnabled __livetrail false)
              (Components|DestroyComponent __livetrail))
            (:else)))
        (:then_2
          (Actor|DestroyActor))))))

(fn SpawnExplosion
  (bind _fromweapon (Variables|Default|GetFromWeapon))
  (bind _playerowner (Variables|/Game/REGRETSSION-Assets/Blueprints/Player/Weapons/BP_WeaponBase.BP_WeaponBase_C|GetPlayerOwner _fromweapon))
  (bind _returnvalue (Game|SpawnActorfromClass (Variables|Default|GetExplosionDummy) (Transformation|GetActorTransform) "AlwaysSpawn" "SelectDefaultAtRuntime" 0 (Variables|Default|GetExplosionRadius) (Variables|Default|GetDamage) _playerowner (Variables|Default|GetFromWeapon) self (Variables|Default|GetExplosionParticle) _playerowner))
  (Default|Explode _returnvalue))

(fn SpawnTrail
  (bind _returnvalue (Niagara|SpawnSystemAttached (Variables|Default|GetTrailParticle) (Variables|Default|GetCollision) "None" "0, 0, 0" "0, 0, 0" "KeepRelativeOffset" true true "AutoRelease"))
  (Variables|Default|Set_liveTrail _returnvalue))