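; Displacer player weapon: a charge-up gun that spins up on Shoot and fires when shooting stops or charge time maxes out.
; A delayed self-calling tick accumulates charge time, damage and ammo cost, gated by an ammo pool check.
; Release plays the shoot montage section, consumes ammo, starts cooldown and notifies the owning player.
; Reload is stubbed out; the magazine refills straight from the player's ammo pool on draw-initialization and after each shot.
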(event Custom|ChargeHandler
  (bind _tickduration (Variables|Default|GetTickDuration))
  (if (and (Variables|Default|Get_isCharging) (< (Variables|Default|GetCurrentChargeTime) (Variables|Default|GetmaxChargeTime)))
    (CallFunction|AddCharge _tickduration)
    (Utilities|FlowControl|Delay _tickduration)
    (CallFunction|ChargeHandlerFunc)
    (else
      (CallFunction|StopShooting))))

(event Custom|Ev_ReloadEnd)

(event Custom|Ev_ShootCooldownHandler
  (Utilities|ShootCooldownHandler))

(fn ConstructionScript
  (|CallParentFunction))

(fn StopShooting
  (Variables|Default|Set_isShooting false)
  (if (Math|Boolean|ORBoolean (Variables|Default|Get_isDrawing) (Variables|Default|Get_isHolstering) (not (Variables|Default|Get_isCharging)))
    (CallFunction|ResetCharge)
    (Variables|Default|Set_isCharging false)
    (else
      (CallFunction|SetAnimation (Utilities|Struct|BreakSTRUCT_DisplacerAnims (Variables|Default|GetDisplacerAnims)))
      (CallFunction|ConsumeAmmo)
      (CallFunction|ResetCharge)
      (CallFunction|EvShootCooldownHandler)
      (Default|EvCurrentWeaponShot (Variables|Default|GetPlayerOwner))
      (Variables|Default|Set_isCharging false))))

(fn Shoot
  (|CallParentFunction)
  (bind _isabletoshoot (CallFunction|CanShoot))
  (if _isabletoshoot
    (if (not (Variables|Default|Get_isShooting))
      (CallFunction|SetAnimation (Utilities|Struct|BreakSTRUCT_DisplacerAnims (Variables|Default|GetDisplacerAnims)))
      (bind _output_get (Variables|Default|Set_isShooting true))
      (Variables|Default|Set_isCharging _output_get)
      (CallFunction|SetInitialCharge))))

(fn CanShoot
  (bind _isabletoshoot (|CallParentFunction))
  (Utilities|FlowControl|Sequence
    (:then_0
      (if (not _isabletoshoot)
        (Variables|Default|Set_isShooting false)))
    (:then_1
      (return _isabletoshoot))))

(fn Reload
  (params (CurrentAmmoPool :type Integer)))

(fn SetAnimator
  (params (Anim :type ABP%20Displacer%20Object%20Reference))
  (Variables|Default|SetAnimator Anim))

(fn SetAnimation
  (params (AnimName :type Name))
  (bind _animator (Variables|Default|GetAnimator))
  (bind _animation_montage (Variables|Default|GetAnimation%20Montage))
  (Animation|Montage|MontagePlay _animator _animation_montage 1.0 "MontageLength" 0.0 true)
  (Ability|Animation|MontageJumptoSection _animator AnimName _animation_montage))

(fn InitializeWeapon
  (params (CurrentAmmo :type Integer) (PlayerOwner :type BP%20Player%20Object%20Reference) (DrawWeapon :type Boolean))
  (|CallParentFunction CurrentAmmo PlayerOwner DrawWeapon)
  (Variables|Default|SetDisplacerAnims (Utilities|Struct|MakeSTRUCT_DisplacerAnims "Draw" "Idle"))
  (if DrawWeapon
    (CallFunction|DrawWeapon)
    (bind _ammo (Default|GetAmmoPool (Variables|Default|GetPlayerOwner) (Variables|Default|GetAmmoType)))
    (bind _ammotakenfrompool (CallFunction|GetAmmotoReload _ammo))
    (CallFunction|SetAmmoinMag _ammotakenfrompool)
    (Default|OnWeaponFinishedReloading (Variables|Default|GetPlayerOwner) _ammotakenfrompool (Variables|Default|GetAmmoType))))

(fn SetDraw
  (params (State :type Boolean))
  (|CallParentFunction State)
  (if State
    (CallFunction|SetAnimation (Utilities|Struct|BreakSTRUCT_DisplacerAnims (Variables|Default|GetDisplacerAnims)))))

(fn SetHolster
  (params (State :type Boolean))
  (if (not (Variables|Default|Get_isHolstering))
    (|CallParentFunction State)
    (if State
      (CallFunction|SetAnimation (Utilities|Struct|BreakSTRUCT_DisplacerAnims (Variables|Default|GetDisplacerAnims))))))

(fn OnReloadEnd)

(fn OnHolsterEnd
  (|CallParentFunction)
  (Variables|Default|Set_isHolstering false)
  (Default|OnHolsteredCurrentWeapon (Variables|Default|GetPlayerOwner)))

(fn DrawWeapon
  (|CallParentFunction)
  (CallFunction|SetDraw true)
  (Variables|Default|Set_isShooting false))

(fn CheckAutomaticFire
  (if (and (not (Variables|Default|Get_shootInCooldown)) (Variables|Default|Get_isShooting))
    (CallFunction|Shoot)))

(fn ConsumeAmmo
  (bind _output_get (Variables|Default|Set_currentAmmoInMag (- (Variables|Default|Get_currentAmmoInMag) (Math|Float|Truncate (Variables|Default|GetCurrentAmmoToConsume)))))
  (Utilities|FlowControl|Sequence
    (:then_0
      (if (<= _output_get 0)
        (Variables|Default|Set_currentAmmoInMag 0)))
    (:then_1
      (bind _ammo (Default|GetAmmoPool (Variables|Default|GetPlayerOwner) (Variables|Default|GetAmmoType)))
      (bind _ammotakenfrompool (CallFunction|GetAmmotoReload _ammo))
      (CallFunction|SetAmmoinMag _ammotakenfrompool)
      (Default|OnWeaponFinishedReloading (Variables|Default|GetPlayerOwner) _ammotakenfrompool (Variables|Default|GetAmmoType)))))

(fn AddCharge
  (params (Tick :type Float%20%28double-precision%29))
  (bind _ammo (CallFunction|GetAmmoPool (Variables|Default|GetAmmoType)))
  (if (>= (Variables|Default|GetCurrentAmmoToConsume) (Math|Conversions|ToFloat(Integer) _ammo))
    (Variables|Default|SetCurrentChargeTime (Math|Float|Min(Float) (+ (Variables|Default|GetCurrentChargeTime) Tick) (Variables|Default|GetmaxChargeTime)))
    (Variables|Default|SetCurrentAmmoToConsume (Math|Float|Min(Float) (+ (Variables|Default|GetCurrentAmmoToConsume) (Variables|Default|GetAmmoConsumedPerTick)) (Math|Conversions|ToFloat(Integer) (Variables|Default|GetMagSize))))
    (Variables|Default|SetCurrentDamageCharged (Math|Float|Min(Float) (+ (Variables|Default|GetCurrentDamageCharged) (Variables|Default|GetDamagePerTick)) (Math|Conversions|ToFloat(Integer) (Variables|Default|GetMaxDamage))))
    (else
      (return))))

(fn ResetCharge
  (bind _output_get (Variables|Default|SetCurrentChargeTime 0.0))
  (bind _output_get_2 (Variables|Default|SetCurrentAmmoToConsume _output_get))
  (Variables|Default|SetCurrentDamageCharged _output_get_2)
  (CallFunction|SetInitialCharge))

(fn SetInitialCharge
  (Variables|Default|SetCurrentAmmoToConsume (Variables|Default|GetAmmoConsumedPerTick))
  (Variables|Default|SetCurrentDamageCharged (Variables|Default|GetDamagePerShot)))

(fn ChargeHandlerFunc
  (CallFunction|ChargeHandler))