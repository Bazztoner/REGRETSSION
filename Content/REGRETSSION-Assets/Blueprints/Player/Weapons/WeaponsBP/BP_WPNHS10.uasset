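; Player weapon Blueprint for the HS10, a pellet-firing shotgun that extends a parent weapon class.
; Shooting spends ammo, starts a delay-based cooldown and spawns a BP_HitscanShell actor that receives damage, range, pellet and spread settings.
; Reload inserts one shell at a time until the magazine is full or the pool is empty, and a shot attempt can end it early.
; Animator flags and montage section jumps drive its animations.
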(event Custom|Ev_ReloadEnd
  (CallFunction|OnReloadEnd))

(event Custom|Ev_ShootCooldownHandler
  (Utilities|ShootCooldownHandler))

(event EventBeginPlay
  (|CallParentFunction) ; This node is disabled and will not be called.\nDrag off pins to build functionality.
)

(event Collision|EventActorBeginOverlap
  (params (OtherActor :type Actor%20Object%20Reference))
  (|CallParentFunction OtherActor) ; This node is disabled and will not be called.\nDrag off pins to build functionality.
)

(event EventTick
  (params (DeltaSeconds :type Float%20%28single-precision%29))
  (|CallParentFunction DeltaSeconds) ; This node is disabled and will not be called.\nDrag off pins to build functionality.
)

(fn ConstructionScript
  (|CallParentFunction))

(fn Shoot
  (|CallParentFunction)
  (bind _isabletoshoot (CallFunction|CanShoot))
  (if _isabletoshoot
    (if (Variables|Default|Get_isReloading)
      (if (not (Variables|Default|Get_isFinishingReload))
        (CallFunction|EndReloadLoop))
      (else
        (Utilities|FlowControl|Sequence
          (:then_0
            (CallFunction|SetAnimation (Utilities|Struct|BreakSTRUCT_HS10Anims (Variables|Default|GetHS10Anims)))
            (Default|SetShoot (Variables|Default|GetAnimator) true))
          (:then_1
            (Variables|Default|Set_currentAmmoInMag (- (Variables|Default|Get_currentAmmoInMag) (Variables|Default|GetAmmoConsumption)))
            (CallFunction|EvShootCooldownHandler))
          (:then_2
            (Default|EvCurrentWeaponShot (Variables|Default|GetPlayerOwner))
            (CallFunction|SpawnProjectile)
            (CallFunction|SpawnMuzzleFlash)
            (Audio|SpawnSoundAttached "/Game/REGRETSSION-Assets/Art/Weapons/HS10/Sounds/HS10_Shoot.HS10_Shoot" (Variables|Default|GetMuzzle) "None" "0, 0, 0" "0, 0, 0" "KeepRelativeOffset" false 1.0 1.0 0.0 0 0)))))
    (else
      (bind _ammo (CallFunction|GetAmmoPool (Variables|Default|GetAmmoType)))
      (bind _forcereload (CallFunction|HastoForceReload _ammo))
      (if _forcereload
        (CallFunction|Reload _ammo)))))

(fn Reload
  (params (CurrentAmmoPool :type Integer))
  (bind _reloadavailable (CallFunction|CanReload CurrentAmmoPool))
  (if _reloadavailable
    (Variables|Default|Set_isReloading true)
    (CallFunction|SetAnimation (Utilities|Struct|BreakSTRUCT_HS10Anims (Variables|Default|GetHS10Anims)))
    (Default|SetReload (Variables|Default|GetAnimator) true)))

(fn SetAnimator
  (params (Anim :type ABP%20HS10%20Object%20Reference))
  (Variables|Default|SetAnimator Anim))

(fn SetAnimation
  (params (AnimName :type Name))
  (bind _animator (Variables|Default|GetAnimator))
  (bind _animation_montage (Variables|Default|GetAnimation%20Montage))
  (Animation|Montage|MontagePlay _animator _animation_montage 1.0 "MontageLength" 0.0 true)
  (Ability|Animation|MontageJumptoSection _animator AnimName _animation_montage))

(fn InitializeWeapon
  (params (CurrentAmmo :type Integer) (PlayerOwner :type BP%20Player%20Object%20Reference) (DrawWeapon :type Boolean))
  (|CallParentFunction CurrentAmmo PlayerOwner DrawWeapon)
  (Variables|Default|SetHS10Anims (Utilities|Struct|MakeSTRUCT_HS10Anims "Draw" "Idle"))
  (if DrawWeapon
    (CallFunction|DrawWeapon)))

(fn SetDraw
  (params (State :type Boolean))
  (|CallParentFunction State)
  (Default|SetDraw (Variables|Default|GetAnimator) State)
  (CallFunction|SetAnimation (Utilities|Struct|BreakSTRUCT_HS10Anims (Variables|Default|GetHS10Anims)))
  (Variables|Default|Set_isFinishingReload false))

(fn SetHolster
  (params (State :type Boolean))
  (if (not (Variables|Default|Get_isHolstering))
    (|CallParentFunction State)
    (Default|SetHolster (Variables|Default|GetAnimator) State)
    (CallFunction|SetAnimation (Utilities|Struct|BreakSTRUCT_HS10Anims (Variables|Default|GetHS10Anims)))))

(fn OnReloadEnd
  (bind _output_get (Variables|Default|Set_isReloading false))
  (Variables|Default|Set_isFinishingReload _output_get)
  (Default|SetReload (Variables|Default|GetAnimator) false))

(fn OnHolsterEnd
  (|CallParentFunction)
  (Variables|Default|Set_isHolstering false)
  (Default|OnHolsteredCurrentWeapon (Variables|Default|GetPlayerOwner))
  (Default|SetDisabled (Variables|Default|GetAnimator) true))

(fn DrawWeapon
  (|CallParentFunction)
  (CallFunction|SetDraw true)
  (Default|SetDisabled (Variables|Default|GetAnimator) false))

(fn OnShellInserted
  (bind _ammo (Default|GetAmmoPool (Variables|Default|GetPlayerOwner) (Variables|Default|GetAmmoType)))
  (bind _ammotakenfrompool (CallFunction|GetAmmotoReload _ammo))
  (CallFunction|SetAmmoinMag _ammotakenfrompool)
  (Default|OnWeaponFinishedReloading (Variables|Default|GetPlayerOwner) _ammotakenfrompool (Variables|Default|GetAmmoType))
  (bind _ammo_2 (Default|GetAmmoPool (Variables|Default|GetPlayerOwner) (Variables|Default|GetAmmoType)))
  (if (or (>= (Variables|Default|Get_currentAmmoInMag) (Variables|Default|GetMagSize)) (< _ammo_2 1))
    (CallFunction|EndReloadLoop)))

(fn EndReloadLoop
  (CallFunction|SetAnimation (Utilities|Struct|BreakSTRUCT_HS10Anims (Variables|Default|GetHS10Anims)))
  (Variables|Default|Set_isFinishingReload true))

(fn GetAmmotoReload
  (params (AmmoPool :type Integer))
  (if (>= AmmoPool 1)
    (return 1)
    (else
      (return 0))))

(fn CanShoot
  (bind __currentammoinmag (Variables|Default|Get_currentAmmoInMag))
  (bind _ammoconsumption (Variables|Default|GetAmmoConsumption))
  (bind _returnvalue (>= __currentammoinmag _ammoconsumption))
  (if _returnvalue
    (return (Math|Boolean|ANDBoolean _returnvalue (not (Variables|Default|Get_shootInCooldown)) (not (Variables|Default|Get_isHolstering)) (not (Variables|Default|Get_isDrawing))))
    (else
      (return false))))

(fn SpawnProjectile
  (|CallParentFunction)
  (bind _returnvalue (Game|SpawnActorfromClass (Variables|Default|GetProjectileClass) (Transformation|GetWorldTransform (Variables|Default|GetMuzzle)) "AlwaysSpawn" "SelectDefaultAtRuntime" self (Variables|Default|GetPlayerOwner)))
  (bind _asbp_hitscan_shell (Utilities|Casting|CastToBP_HitscanShell _returnvalue))
  (Default|SpawnHitscan _asbp_hitscan_shell self (Variables|Default|GetMaxDistance) (Variables|Default|GetDamagePerShot) (Variables|Default|GetAmmoType) (Variables|Default|GetPellets) (Variables|Default|GetVerticalSpread) (Variables|Default|GetHorizontalSpread)))

(fn ForcedHolstering
  (|CallParentFunction)
  (Default|SetDisabled (Variables|Default|GetAnimator) true)
  (CallFunction|SetAnimation (Utilities|Struct|BreakSTRUCT_HS10Anims (Variables|Default|GetHS10Anims))))

(fn StopShooting
  (|CallParentFunction)
  (Default|SetShoot (Variables|Default|GetAnimator) false))