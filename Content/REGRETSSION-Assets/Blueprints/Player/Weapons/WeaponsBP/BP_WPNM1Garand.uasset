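; M1 Garand player weapon, extending a parent weapon class with Garand-specific firing, reloading, draw and holster behaviour.
; Shots spawn a hitscan bullet actor using component-driven spread, then notify the owner; reloading requires an empty magazine and draws on the owner's ammo pool.
; An animator receives state flags and jumps between montage sections, with last-shot and empty variants.
; Five levels swap damage, recoil, fire rate and camera shake.
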(event Custom|Ev_ReloadStart
  ;[1 1 1] Delays the Animation Montage to avoid an animation bug
  (Utilities|FlowControl|Delay 0.2)
  (CallFunction|SetAnimation (Utilities|Struct|BreakSTRUCT_M1GarandAnims (Variables|Default|GetGarandAnims))))

(event Custom|Ev_ReloadEnd
  (CallFunction|OnReloadEnd))

(event Custom|Ev_ShootCooldownHandler
  (Utilities|ShootCooldownHandler))

(fn ConstructionScript
  (|CallParentFunction))

(fn Shoot
  (bind _garandanims (Variables|Default|GetGarandAnims))
  (bind (_shoot _shoot_last) (Utilities|Struct|BreakSTRUCT_M1GarandAnims _garandanims))
  (|CallParentFunction)
  (bind _isabletoshoot (CallFunction|CanShoot))
  (if _isabletoshoot
    (Utilities|FlowControl|Sequence
      (:then_0
        (if (> (Variables|Default|Get_currentAmmoInMag) 1)
          (LocalVariables|Setanim _shoot)
          (Default|SetEmptyWeapon (Variables|Default|GetAnimator) false)
          (else
            (LocalVariables|Setanim _shoot_last)
            (Default|SetEmptyWeapon (Variables|Default|GetAnimator) true))))
      (:then_1
        (CallFunction|SetAnimation (LocalVariables|Getanim))
        (Default|SetShoot (Variables|Default|GetAnimator) true))
      (:then_2
        (Variables|Default|Set_currentAmmoInMag (- (Variables|Default|Get_currentAmmoInMag) (Variables|Default|GetAmmoConsumption)))
        (CallFunction|EvShootCooldownHandler))
      (:then_3
        (Default|EvCurrentWeaponShot (Variables|Default|GetPlayerOwner))
        (CallFunction|SpawnProjectile)
        (CallFunction|SpawnMuzzleFlash)
        (Default|OnShoot (Variables|Default|GetWeaponSpreadComponent))))
    (else
      (bind _ammo (CallFunction|GetAmmoPool (Variables|Default|GetAmmoType)))
      (bind _forcereload (CallFunction|HastoForceReload _ammo))
      (if _forcereload
        (CallFunction|Reload _ammo)))))

(fn Reload
  (params (CurrentAmmoPool :type Integer))
  (bind _reloadavailable (CallFunction|CanReload CurrentAmmoPool))
  (if _reloadavailable
    (bind _output_get (Variables|Default|Set_isReloading true))
    (Default|SetReload (Variables|Default|GetAnimator) _output_get)
    (CallFunction|EvReloadStart)))

(fn SetAnimator
  (params (Anim :type ABP%20M1%20Garand%20Object%20Reference))
  (Variables|Default|SetAnimator Anim))

(fn SetAnimation
  (params (AnimName :type Name))
  (bind _animator (Variables|Default|GetAnimator))
  (bind _animation_montage (Variables|Default|GetAnimation%20Montage))
  (Animation|Montage|MontagePlay _animator _animation_montage 1.0 "MontageLength" 0.0 true)
  (Ability|Animation|MontageJumptoSection _animator AnimName _animation_montage))

(fn InitializeWeapon
  (params (CurrentAmmo :type Integer) (PlayerOwner :type BP%20Player%20Object%20Reference) (DrawWeapon :type Boolean))
  (|CallParentFunction CurrentAmmo PlayerOwner DrawWeapon)
  (CallFunction|SetInitialLevel 1)
  (Variables|Default|SetGarandAnims (Utilities|Struct|MakeSTRUCT_M1GarandAnims "Draw" "Idle"))
  (if DrawWeapon
    (CallFunction|DrawWeapon)))

(fn SetDraw
  (params (State :type Boolean))
  (bind _garandanims (Variables|Default|GetGarandAnims))
  (bind (_draw _idle _draw_empty _empty_idle) (Utilities|Struct|BreakSTRUCT_M1GarandAnims _garandanims))
  (Utilities|FlowControl|Sequence
    (:then_0
      (|CallParentFunction State))
    (:then_1
      (Default|SetDraw (Variables|Default|GetAnimator) State)
      (bind _empty (CallFunction|GetEmptyMag))
      (Default|SetEmptyWeapon (Variables|Default|GetAnimator) _empty)
      (if _empty
        (LocalVariables|SetAnim _empty_idle)
        (else
          (LocalVariables|SetAnim _idle))))
    (:then_2
      (CallFunction|SetAnimation (LocalVariables|GetAnim)))))

(fn SetHolster
  (params (State :type Boolean))
  (bind _animator (Variables|Default|GetAnimator))
  (if (not (Variables|Default|Get_isHolstering))
    (|CallParentFunction State)
    (Default|SetHolster _animator State)
    (bind _empty (CallFunction|GetEmptyMag))
    (Default|SetEmptyWeapon _animator _empty)))

(fn OnReloadEnd
  (bind _output_get (Variables|Default|Set_isReloading false))
  (Default|SetReload (Variables|Default|GetAnimator) _output_get)
  (bind _ammo (Default|GetAmmoPool (Variables|Default|GetPlayerOwner) (Variables|Default|GetAmmoType)))
  (bind _ammotakenfrompool (CallFunction|GetAmmotoReload _ammo))
  (CallFunction|SetAmmoinMag _ammotakenfrompool)
  (Default|OnWeaponFinishedReloading (Variables|Default|GetPlayerOwner) _ammotakenfrompool (Variables|Default|GetAmmoType))
  (Default|SetEmptyWeapon (Variables|Default|GetAnimator) false))

(fn OnHolsterEnd
  (bind _animator (Variables|Default|GetAnimator))
  (|CallParentFunction)
  (Variables|Default|Set_isHolstering false)
  (Default|OnHolsteredCurrentWeapon (Variables|Default|GetPlayerOwner))
  (Default|SetHolster _animator false)
  (Default|SetDisabled _animator true))

(fn DrawWeapon
  (|CallParentFunction)
  (CallFunction|SetDraw true)
  (Default|SetDisabled (Variables|Default|GetAnimator) false))

(fn CanReload
  (params (AmmoPool :type Integer))
  (return (Math|Boolean|ANDBoolean (>= AmmoPool (Variables|Default|GetAmmoConsumption)) (< (Variables|Default|Get_currentAmmoInMag) 1) (not (Variables|Default|Get_isReloading)) (not (Variables|Default|Get_isHolstering)) (not (Variables|Default|Get_isDrawing)) (not (Variables|Default|Get_isShooting)))))

(fn SpawnProjectile
  (|CallParentFunction)
  (bind _returnvalue (Game|SpawnActorfromClass (Variables|Default|GetProjectileClass) (Transformation|GetWorldTransform (Variables|Default|GetMuzzle)) "AlwaysSpawn" "SelectDefaultAtRuntime" self (Variables|Default|GetPlayerOwner)))
  ;[1 1 1] Hardcoded?
  (bind _asbp_hitscan_bullet (Utilities|Casting|CastToBP_HitscanBullet _returnvalue))
  (bind (_xspread _yspread) (Default|GetSpread (Variables|Default|GetWeaponSpreadComponent)))
  (Default|SpawnHitscan _asbp_hitscan_bullet self (Variables|Default|GetMaxDistance) (Variables|Default|GetDamagePerShot) (Variables|Default|GetAmmoType) _xspread _yspread))

(fn ChangeLevel
  (params (NewLevel :type Byte))
  (bind _struct_m1garanddata_lv5 (Utilities|Struct|MakeSTRUCT_M1GarandData_LV5 105.0 -0.86 0.2 2.4e+02 "/Game/REGRETSSION-Assets/Art/Weapons/1_BaseData/BP_RecoilLight.BP_RecoilLight_C"))
  (bind _struct_m1garanddata_lv4 (Utilities|Struct|MakeSTRUCT_M1GarandData_LV4 95.0 -1.6 0.5 2e+02 "/Game/REGRETSSION-Assets/Art/Weapons/1_BaseData/BP_RecoilLight.BP_RecoilLight_C"))
  (bind _struct_m1garanddata_lv3 (Utilities|Struct|MakeSTRUCT_M1GarandData_LV3 85.0 -2.6 0.85 1.6e+02 "/Game/REGRETSSION-Assets/Art/Weapons/1_BaseData/BP_RecoilLight.BP_RecoilLight_C"))
  (bind _struct_m1garanddata_lv2 (Utilities|Struct|MakeSTRUCT_M1GarandData_LV2 8e+01 -4.6 1.35 1.2e+02 "/Game/REGRETSSION-Assets/Art/Weapons/1_BaseData/BP_RecoilHeavy.BP_RecoilHeavy_C"))
  (bind _struct_m1garanddata_lv1 (Utilities|Struct|MakeSTRUCT_M1GarandData_LV1 75.0 -6.6 2.0 8e+01 "/Game/REGRETSSION-Assets/Art/Weapons/1_BaseData/BP_RecoilHeavy.BP_RecoilHeavy_C"))
  (bind (_damagepershot _verticalrecoil _horizontalrecoil _rpm _camshake) (Utilities|Struct|BreakSTRUCT_M1GarandData_LV1 _struct_m1garanddata_lv1))
  (bind (_damagepershot_2 _verticalrecoil_2 _horizontalrecoil_2 _rpm_2 _camshake_2) (Utilities|Struct|BreakSTRUCT_M1GarandData_LV2 _struct_m1garanddata_lv2))
  (bind (_damagepershot_3 _verticalrecoil_3 _horizontalrecoil_3 _rpm_3 _camshake_3) (Utilities|Struct|BreakSTRUCT_M1GarandData_LV3 _struct_m1garanddata_lv3))
  (bind (_damagepershot_4 _verticalrecoil_4 _horizontalrecoil_4 _rpm_4 _camshake_4) (Utilities|Struct|BreakSTRUCT_M1GarandData_LV4 _struct_m1garanddata_lv4))
  (bind (_damagepershot_5 _verticalrecoil_5 _horizontalrecoil_5 _rpm_5 _camshake_5) (Utilities|Struct|BreakSTRUCT_M1GarandData_LV5 _struct_m1garanddata_lv5))
  (bind _output_get (Variables|Default|SetCurrentLevel NewLevel))
  (Development|PrintString (Utilities|String|ToString(Byte) _output_get) true true "(R=0.880564,G=0.800990,B=1.000000,A=1.000000)")
  (switch string (Utilities|String|ToString(Byte) _output_get)
    (:1
      (CallFunction|SetWeaponData _damagepershot _verticalrecoil _horizontalrecoil _rpm _camshake))
    (:2
      (CallFunction|SetWeaponData _damagepershot_2 _verticalrecoil_2 _horizontalrecoil_2 _rpm_2 _camshake_2))
    (:3
      (CallFunction|SetWeaponData _damagepershot_3 _verticalrecoil_3 _horizontalrecoil_3 _rpm_3 _camshake_3))
    (:4
      (CallFunction|SetWeaponData _damagepershot_4 _verticalrecoil_4 _horizontalrecoil_4 _rpm_4 _camshake_4))
    (:5
      (CallFunction|SetWeaponData _damagepershot_5 _verticalrecoil_5 _horizontalrecoil_5 _rpm_5 _camshake_5))))

(fn SetInitialLevel
  (params (InitialLevel :type Byte))
  (CallFunction|ChangeLevel InitialLevel))

(fn SetWeaponData
  (params (Damage :type Float%20%28double-precision%29) (VerticalRecoil :type Float%20%28double-precision%29) (HorizontalRecoul :type Float%20%28double-precision%29) (RPM :type Float%20%28double-precision%29) (CamShake :type Legacy%20Camera%20Shake%20Class%20Reference))
  (Variables|Default|SetDamagePerShot Damage)
  (Variables|Default|SetVerticalRecoil VerticalRecoil)
  (Variables|Default|SetHorizontalRecoil HorizontalRecoul)
  (Variables|Default|SetRPM RPM)
  (CallFunction|InitializeRPM)
  (Variables|Default|SetCamShakeData CamShake))

(fn ForcedHolstering
  (|CallParentFunction)
  (Default|SetDisabled (Variables|Default|GetAnimator) true))

(fn StopShooting
  (|CallParentFunction)
  (Default|SetShoot (Variables|Default|GetAnimator) false)
  (Default|OnShootEnd (Variables|Default|GetWeaponSpreadComponent)))