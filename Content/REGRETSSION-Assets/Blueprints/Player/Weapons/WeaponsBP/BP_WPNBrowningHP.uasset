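; Browning HP pistol weapon that overrides its parent's shoot, reload, draw and holster behavior, driving an animator through state flags and montage section jumps.
; Shooting consumes ammo, starts a cooldown, notifies the owning player, spawns muzzle effects and a spread-adjusted BP_HitscanBullet, with a separate last-shot animation.
; A failed shot can force a reload.
; Reload completion refills the magazine from the player's ammo pool and reports the amount back.
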(event Custom|Ev_ReloadEnd
  (CallFunction|OnReloadEnd))

(event Custom|Ev_ShootCooldownHandler
  (Utilities|ShootCooldownHandler))

(event EventBeginPlay
  (|CallParentFunction) ; This node is disabled and will not be called.\nDrag off pins to build functionality.
)

(event Collision|EventActorBeginOverlap
  (params (OtherActor :type Actor%20Object%20Reference))
  (|CallParentFunction OtherActor) ; This node is disabled and will not be called.\nDrag off pins to build functionality.
)

(event EventTick
  (params (DeltaSeconds :type Float%20%28single-precision%29))
  (|CallParentFunction DeltaSeconds) ; This node is disabled and will not be called.\nDrag off pins to build functionality.
)

(fn ConstructionScript
  (|CallParentFunction))

(fn Shoot
  (bind _browninghpanims (Variables|Default|GetBrowningHPAnims))
  (bind _animator (Variables|Default|GetAnimator))
  (bind (_shoot _shoot_last) (Utilities|Struct|BreakSTRUCT_BrowningHPAnims _browninghpanims))
  (|CallParentFunction)
  (bind _isabletoshoot (CallFunction|CanShoot))
  (if _isabletoshoot
    (Utilities|FlowControl|Sequence
      (:then_0
        (if (> (Variables|Default|Get_currentAmmoInMag) 1)
          (LocalVariables|Setanim _shoot)
          (Default|SetShooting _animator true false)
          (else
            (LocalVariables|Setanim _shoot_last)
            (Default|SetShooting _animator true true)
            (Default|SetWeaponEmpty _animator true))))
      (:then_1
        (CallFunction|SetAnimation (LocalVariables|Getanim)))
      (:then_2
        (Variables|Default|Set_currentAmmoInMag (- (Variables|Default|Get_currentAmmoInMag) (Variables|Default|GetAmmoConsumption)))
        (CallFunction|EvShootCooldownHandler))
      (:then_3
        (Default|EvCurrentWeaponShot (Variables|Default|GetPlayerOwner))
        (CallFunction|SpawnProjectile)
        (CallFunction|SpawnMuzzleFlash)
        (Audio|SpawnSoundAttached "/Game/REGRETSSION-Assets/Art/Weapons/BrowningHP/Sounds/browninghp_shoot_Cue.browninghp_shoot_Cue" (Variables|Default|GetMuzzle) "None" "0, 0, 0" "0, 0, 0" "KeepRelativeOffset" false 1.0 1.0 0.0 0 0)))
    (else
      (bind _ammo (CallFunction|GetAmmoPool (Variables|Default|GetAmmoType)))
      (bind _forcereload (CallFunction|HastoForceReload _ammo))
      (if _forcereload
        (CallFunction|Reload _ammo)))))

(fn Reload
  (params (CurrentAmmoPool :type Integer))
  (bind _reloadavailable (CallFunction|CanReload CurrentAmmoPool))
  (if _reloadavailable
    (bind _output_get (Variables|Default|Set_isReloading true))
    (Default|SetReloading (Variables|Default|GetAnimator) _output_get)
    (CallFunction|SetAnimation (Utilities|Struct|BreakSTRUCT_BrowningHPAnims (Variables|Default|GetBrowningHPAnims)))))

(fn SetAnimator
  (params (Anim :type ABP%20Browning%20HP%20Object%20Reference))
  (Variables|Default|SetAnimator Anim))

(fn SetAnimation
  (params (AnimName :type Name))
  (bind _animator (Variables|Default|GetAnimator))
  (bind _animation_montage (Variables|Default|GetAnimation%20Montage))
  (Animation|Montage|MontagePlay _animator _animation_montage 1.0 "MontageLength" 0.0 true)
  (Ability|Animation|MontageJumptoSection _animator AnimName _animation_montage))

(fn InitializeWeapon
  (params (CurrentAmmo :type Integer) (PlayerOwner :type BP%20Player%20Object%20Reference) (DrawWeapon :type Boolean))
  (|CallParentFunction CurrentAmmo PlayerOwner DrawWeapon)
  (Variables|Default|SetBrowningHPAnims (Utilities|Struct|MakeSTRUCT_BrowningHPAnims "Draw" "Idle"))
  (if DrawWeapon
    (CallFunction|DrawWeapon)))

(fn SetDraw
  (params (State :type Boolean))
  (bind _animator (Variables|Default|GetAnimator))
  (bind _browninghpanims (Variables|Default|GetBrowningHPAnims))
  (bind (_idle _idle_empty) (Utilities|Struct|BreakSTRUCT_BrowningHPAnims _browninghpanims))
  (|CallParentFunction State)
  (Default|SetDrawing _animator State)
  (bind _empty (CallFunction|GetEmptyMag))
  (Default|SetWeaponEmpty _animator _empty)
  (if _empty
    (CallFunction|SetAnimation _idle_empty)
    (else
      (CallFunction|SetAnimation _idle))))

(fn SetHolster
  (params (State :type Boolean))
  (if (not (Variables|Default|Get_isHolstering))
    (|CallParentFunction State)
    (Default|SetHolstering (Variables|Default|GetAnimator) State)))

(fn OnReloadEnd
  (Variables|Default|Set_isReloading false)
  (Utilities|FlowControl|Sequence
    (:then_0
      (bind _ammo (Default|GetAmmoPool (Variables|Default|GetPlayerOwner) (Variables|Default|GetAmmoType)))
      (bind _ammotakenfrompool (CallFunction|GetAmmotoReload _ammo))
      (CallFunction|SetAmmoinMag _ammotakenfrompool)
      (Default|OnWeaponFinishedReloading (Variables|Default|GetPlayerOwner) _ammotakenfrompool (Variables|Default|GetAmmoType)))
    (:then_1
      (bind _empty (CallFunction|GetEmptyMag))
      (Default|SetWeaponEmpty (Variables|Default|GetAnimator) _empty)
      (CallFunction|SetAnimation (Utilities|Struct|BreakSTRUCT_BrowningHPAnims (Variables|Default|GetBrowningHPAnims)))
      (Default|SetReloading (Variables|Default|GetAnimator) false))))

(fn OnHolsterEnd
  (|CallParentFunction)
  (bind _output_get (Variables|Default|Set_isHolstering false))
  (Default|SetHolstering (Variables|Default|GetAnimator) _output_get)
  (Default|OnHolsteredCurrentWeapon (Variables|Default|GetPlayerOwner)))

(fn DrawWeapon
  (|CallParentFunction)
  (CallFunction|SetDraw true)
  (Default|SetDisabledWeapon (Variables|Default|GetAnimator) false))

(fn SpawnProjectile
  (|CallParentFunction)
  (bind _returnvalue (Game|SpawnActorfromClass (Variables|Default|GetProjectileClass) (Transformation|GetWorldTransform (Variables|Default|GetMuzzle)) "AlwaysSpawn" "SelectDefaultAtRuntime" self (Variables|Default|GetPlayerOwner)))
  ;[1 1 1] Hardcoded?
  (bind _asbp_hitscan_bullet (Utilities|Casting|CastToBP_HitscanBullet _returnvalue))
  (bind (_xspread _yspread) (Default|GetSpread (Variables|Default|GetWeaponSpreadComponent)))
  (Default|SpawnHitscan _asbp_hitscan_bullet self (Variables|Default|GetMaxDistance) (Variables|Default|GetDamagePerShot) (Variables|Default|GetAmmoType) _xspread _yspread))

(fn ForcedHolstering
  (|CallParentFunction)
  (Default|SetDisabledWeapon (Variables|Default|GetAnimator) true))

(fn StopShooting
  (|CallParentFunction)
  (bind _output_get (Variables|Default|Set_isShooting false))
  (bind _empty (CallFunction|GetEmptyMag))
  (Default|SetShooting (Variables|Default|GetAnimator) _output_get _empty))