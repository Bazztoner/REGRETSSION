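; Player M72 LAW weapon, a disposable rocket launcher built on a parent weapon class.
; Shooting spends magazine ammo, notifies the owner, and spawns a muzzle flash and a rocket initialized with damage and explosion particle.
; Draw, holster, shoot and discard states drive the Animator.
; ShootHandler flags the launcher for discard, so holstering then notifies the owner and destroys it; Reload is empty, though reload callbacks remain.
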(event EventBeginPlay
  (|CallParentFunction) ; This node is disabled and will not be called.\nDrag off pins to build functionality.
)

(event Collision|EventActorBeginOverlap
  (params (OtherActor :type Actor%20Object%20Reference))
  (|CallParentFunction OtherActor) ; This node is disabled and will not be called.\nDrag off pins to build functionality.
)

(event EventTick
  (params (DeltaSeconds :type Float%20%28single-precision%29))
  (|CallParentFunction DeltaSeconds) ; This node is disabled and will not be called.\nDrag off pins to build functionality.
)

(fn ConstructionScript
  (|CallParentFunction))

(fn Shoot
  (|CallParentFunction)
  (bind _ammo (CallFunction|GetAmmoPool (Variables|Default|GetAmmoType)))
  (LocalVariables|SetAmmoPool _ammo)
  (bind _isabletoshoot (CallFunction|CanShoot))
  (if _isabletoshoot
    (Utilities|FlowControl|Sequence
      (:then_0
        (Default|SetShoot (Variables|Default|GetAnimator) true))
      (:then_1
        (Variables|Default|Set_currentAmmoInMag (- (Variables|Default|Get_currentAmmoInMag) (Variables|Default|GetAmmoConsumption))))
      (:then_2
        (Variables|Default|Set_isShooting true))
      (:then_3
        (Default|EvCurrentWeaponShot (Variables|Default|GetPlayerOwner))
        (CallFunction|SpawnProjectile)
        (CallFunction|SpawnMuzzleFlash)))))

(fn Reload
  (params (CurrentAmmoPool :type Integer)))

(fn SetAnimator
  (params (Anim :type ABP%20M72LAW%20Object%20Reference))
  (Variables|Default|SetAnimator Anim))

(fn SetAnimation
  (params (AnimName :type Name))
  (bind _animator (Variables|Default|GetAnimator))
  (bind _animation_montage (Variables|Default|GetAnimation%20Montage))
  (Animation|Montage|MontagePlay _animator _animation_montage 1.0 "MontageLength" 0.0 true)
  (Ability|Animation|MontageJumptoSection _animator AnimName _animation_montage))

(fn InitializeWeapon
  (params (CurrentAmmo :type Integer) (PlayerOwner :type BP%20Player%20Object%20Reference) (DrawWeapon :type Boolean))
  (|CallParentFunction CurrentAmmo PlayerOwner DrawWeapon)
  (Variables|Default|SetLAWAnims (Utilities|Struct|MakeSTRUCT_M72LAWAnims "Draw" "Idle"))
  (if DrawWeapon
    (CallFunction|DrawWeapon)))

(fn SetDraw
  (params (State :type Boolean))
  (|CallParentFunction State)
  (Default|SetDraw (Variables|Default|GetAnimator) State))

(fn SetHolster
  (params (State :type Boolean))
  (if (not (Variables|Default|Get_isHolstering))
    (|CallParentFunction State)
    (Default|SetHolster (Variables|Default|GetAnimator) State)
    (if State
      (if (Variables|Default|Get_isDiscarding)
        (CallFunction|DiscardWeapon)))))

(fn OnReloadEnd
  (Variables|Default|Set_isReloading false)
  (bind _ammo (Default|GetAmmoPool (Variables|Default|GetPlayerOwner) (Variables|Default|GetAmmoType)))
  (bind _ammotakenfrompool (CallFunction|GetAmmotoReload _ammo))
  (CallFunction|SetAmmoinMag _ammotakenfrompool)
  (Default|OnWeaponFinishedReloading (Variables|Default|GetPlayerOwner) _ammotakenfrompool (Variables|Default|GetAmmoType)))

(fn OnHolsterEnd
  (|CallParentFunction)
  (Variables|Default|Set_isHolstering false)
  (Default|OnHolsteredCurrentWeapon (Variables|Default|GetPlayerOwner))
  (Default|SetDisabled (Variables|Default|GetAnimator) true))

(fn ForceReload
  (Variables|Default|Set_isShooting false)
  (Default|ReloadCurrentWeapon (Variables|Default|GetPlayerOwner)))

(fn DrawWeapon
  (|CallParentFunction)
  (CallFunction|SetDraw true)
  (Default|SetDisabled (Variables|Default|GetAnimator) false))

(fn DiscardWeapon
  (bind _self self)
  (Default|OnWeaponDestroyed (Variables|Default|GetPlayerOwner) _self)
  (Actor|DestroyActor _self))

(fn ForcedHolstering
  (if (Variables|Default|Get_isDiscarding)
    (CallFunction|DiscardWeapon)
    (else
      (|CallParentFunction)
      (Default|SetDisabled (Variables|Default|GetAnimator) true))))

(fn ShootHandler
  (Variables|Default|Set_isDiscarding true))

(fn SpawnProjectile
  (|CallParentFunction)
  (bind _returnvalue (Game|SpawnActorfromClass (Variables|Default|GetProjectileClass) (Transformation|GetWorldTransform (Variables|Default|GetMuzzle)) "AlwaysSpawn" "SelectDefaultAtRuntime" self (Variables|Default|GetPlayerOwner)))
  (bind _asbp_lawprojectile (Utilities|Casting|CastToBP_LAWProjectile _returnvalue))
  (Default|InitializeRocket _asbp_lawprojectile self (Variables|Default|GetDamagePerShot) (Variables|Default|GetAmmoType) 0.0 0.0 (Variables|Default|GetExplosionParticle)))

(fn OnReadytoDiscard
  (Default|SetDiscard (Variables|Default|GetAnimator) true))