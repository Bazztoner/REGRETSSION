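; Deagle pistol weapon Blueprint, a child weapon class that handles shooting, reloading, drawing and holstering for its owning player.
; Shooting consumes magazine ammo, starts a cooldown, spawns a hitscan bullet actor with spread from the spread component, or forces a reload when needed.
; Montage sections from a Deagle anims struct, including last-shot and empty-idle variants, and animator flags drive the visuals.
; Reload completion refills the magazine and notifies the owner.
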(event Custom|Ev_ReloadEnd
  (CallFunction|OnReloadEnd))

(event Custom|Ev_ShootCooldownHandler
  (Utilities|ShootCooldownHandler))

(fn ConstructionScript
  (|CallParentFunction))

(fn Shoot
  (bind _deagleanims (Variables|Default|GetDeagleAnims))
  (bind (_shoot _shoot_last) (Utilities|Struct|BreakSTRUCT_DeagleAnims _deagleanims))
  (|CallParentFunction)
  (bind _isabletoshoot (CallFunction|CanShoot))
  (if _isabletoshoot
    (Utilities|FlowControl|Sequence
      (:then_0
        (if (> (Variables|Default|Get_currentAmmoInMag) 1)
          (LocalVariables|Setanim _shoot)
          (else
            (LocalVariables|Setanim _shoot_last))))
      (:then_1
        (CallFunction|SetAnimation (LocalVariables|Getanim))
        (Default|SetShoot (Variables|Default|GetAnimator) true))
      (:then_2
        (Variables|Default|Set_currentAmmoInMag (- (Variables|Default|Get_currentAmmoInMag) (Variables|Default|GetAmmoConsumption)))
        (CallFunction|EvShootCooldownHandler))
      (:then_3
        (Default|EvCurrentWeaponShot (Variables|Default|GetPlayerOwner))
        (CallFunction|SpawnProjectile)
        (CallFunction|SpawnMuzzleFlash)
        (Default|OnShoot (Variables|Default|GetWeaponSpreadComponent))))
    (else
      (bind _ammo (CallFunction|GetAmmoPool (Variables|Default|GetAmmoType)))
      (bind _forcereload (CallFunction|HastoForceReload _ammo))
      (if _forcereload
        (CallFunction|Reload _ammo)))))

(fn Reload
  (params (CurrentAmmoPool :type Integer))
  (bind _reloadavailable (CallFunction|CanReload CurrentAmmoPool))
  (if _reloadavailable
    (Variables|Default|Set_isReloading true)
    (Default|SetReload (Variables|Default|GetAnimator) true)
    (CallFunction|SetAnimation (.Idle (Utilities|Struct|BreakSTRUCT_DeagleAnims (Variables|Default|GetDeagleAnims))))))

(fn SetAnimator
  (params (Anim :type ABP%20Deagle%20Object%20Reference))
  (Variables|Default|SetAnimator Anim))

(fn SetAnimation
  (params (AnimName :type Name))
  (bind _animator (Variables|Default|GetAnimator))
  (bind _animation_montage (Variables|Default|GetAnimation%20Montage))
  (Animation|Montage|MontagePlay _animator _animation_montage 1.0 "MontageLength" 0.0 true)
  (Ability|Animation|MontageJumptoSection _animator AnimName _animation_montage))

(fn InitializeWeapon
  (params (CurrentAmmo :type Integer) (PlayerOwner :type BP%20Player%20Object%20Reference) (DrawWeapon :type Boolean))
  (|CallParentFunction CurrentAmmo PlayerOwner DrawWeapon)
  (Variables|Default|SetDeagleAnims (Utilities|Struct|MakeSTRUCT_DeagleAnims "Draw" "Idle"))
  (if DrawWeapon
    (CallFunction|DrawWeapon)))

(fn SetDraw
  (params (State :type Boolean))
  (bind _deagleanims (Variables|Default|GetDeagleAnims))
  (bind (_draw _idle _shoot _shoot_last _idle_empty) (Utilities|Struct|BreakSTRUCT_DeagleAnims _deagleanims))
  (|CallParentFunction State)
  (Default|SetDraw (Variables|Default|GetAnimator) State)
  (Default|SetDisabled (Variables|Default|GetAnimator) false)
  (bind _empty (CallFunction|GetEmptyMag))
  (if _empty
    (CallFunction|SetAnimation _idle_empty)
    (else
      (CallFunction|SetAnimation _idle))))

(fn SetHolster
  (params (State :type Boolean))
  (if (not (Variables|Default|Get_isHolstering))
    (|CallParentFunction State)
    (Default|SetHolster (Variables|Default|GetAnimator) State)))

(fn OnReloadEnd
  (bind _output_get (Variables|Default|Set_isReloading false))
  (Default|SetReload (Variables|Default|GetAnimator) _output_get)
  (bind _ammo (Default|GetAmmoPool (Variables|Default|GetPlayerOwner) (Variables|Default|GetAmmoType)))
  (bind _ammotakenfrompool (CallFunction|GetAmmotoReload _ammo))
  (CallFunction|SetAmmoinMag _ammotakenfrompool)
  (Default|OnWeaponFinishedReloading (Variables|Default|GetPlayerOwner) _ammotakenfrompool (Variables|Default|GetAmmoType)))

(fn OnHolsterEnd
  (|CallParentFunction)
  (Variables|Default|Set_isHolstering false)
  (Default|SetDisabled (Variables|Default|GetAnimator) true)
  (Default|OnHolsteredCurrentWeapon (Variables|Default|GetPlayerOwner)))

(fn DrawWeapon
  (|CallParentFunction)
  (CallFunction|SetDraw true))

(fn SpawnProjectile
  (|CallParentFunction)
  (bind _returnvalue (Game|SpawnActorfromClass (Variables|Default|GetProjectileClass) (Transformation|GetWorldTransform (Variables|Default|GetMuzzle)) "AlwaysSpawn" "SelectDefaultAtRuntime" self (Variables|Default|GetPlayerOwner)))
  ;[1 1 1] Hardcoded?
  (bind _asbp_hitscan_bullet (Utilities|Casting|CastToBP_HitscanBullet _returnvalue))
  (bind (_xspread _yspread) (Default|GetSpread (Variables|Default|GetWeaponSpreadComponent)))
  (Default|SpawnHitscan _asbp_hitscan_bullet self (Variables|Default|GetMaxDistance) (Variables|Default|GetDamagePerShot) (Variables|Default|GetAmmoType) _xspread _yspread))

(fn StopShooting
  (|CallParentFunction)
  (bind _output_get (Variables|Default|Set_isShooting false))
  (Default|SetShoot (Variables|Default|GetAnimator) _output_get)
  (Default|OnShootEnd (Variables|Default|GetWeaponSpreadComponent)))

(fn ForcedHolstering
  (bind _animator (Variables|Default|GetAnimator))
  (Default|SetDisabled _animator true)
  (|CallParentFunction)
  (Default|SetReload _animator false)
  (Default|SetShoot _animator false)
  (Default|SetDraw _animator false)
  (Default|SetHolster _animator false))