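; Rocket launcher weapon for the player, a child of a base weapon class that handles firing, reloading, drawing and holstering.
; Shooting spends magazine ammo, starts a delayed cooldown, spawns a muzzle flash and an initialized rocket projectile at the muzzle, or reloads when forced.
; Draw, holster, shoot and reload states drive the animator, while the owning player supplies ammo pools and is notified of shots, reloads and holstering.
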(event Custom|Ev_ReloadEnd
  (CallFunction|OnReloadEnd))

(event Custom|Ev_ShootCooldownHandler
  (Utilities|ShootCooldownHandler))

(event EventBeginPlay
  (|CallParentFunction) ; This node is disabled and will not be called.\nDrag off pins to build functionality.
)

(event Collision|EventActorBeginOverlap
  (params (OtherActor :type Actor%20Object%20Reference))
  (|CallParentFunction OtherActor) ; This node is disabled and will not be called.\nDrag off pins to build functionality.
)

(event EventTick
  (params (DeltaSeconds :type Float%20%28single-precision%29))
  (|CallParentFunction DeltaSeconds) ; This node is disabled and will not be called.\nDrag off pins to build functionality.
)

(fn ConstructionScript
  (|CallParentFunction))

(fn Shoot
  (|CallParentFunction)
  (bind _ammo (CallFunction|GetAmmoPool (Variables|Default|GetAmmoType)))
  (LocalVariables|SetAmmoPool _ammo)
  (bind _isabletoshoot (CallFunction|CanShoot))
  (if _isabletoshoot
    (Utilities|FlowControl|Sequence
      (:then_0
        (Default|SetShoot (Variables|Default|GetAnimator) true))
      (:then_1
        (Variables|Default|Set_currentAmmoInMag (- (Variables|Default|Get_currentAmmoInMag) (Variables|Default|GetAmmoConsumption)))
        (CallFunction|EvShootCooldownHandler))
      (:then_2
        (Variables|Default|Set_isShooting true))
      (:then_3
        (Default|EvCurrentWeaponShot (Variables|Default|GetPlayerOwner))
        (CallFunction|SpawnProjectile)
        (CallFunction|SpawnMuzzleFlash)))
    (else
      (bind _forcereload (CallFunction|HastoForceReload (LocalVariables|GetAmmoPool)))
      (if _forcereload
        (CallFunction|Reload (LocalVariables|GetAmmoPool))))))

(fn Reload
  (params (CurrentAmmoPool :type Integer))
  (bind _reloadavailable (CallFunction|CanReload CurrentAmmoPool))
  (if _reloadavailable
    (bind _output_get (Variables|Default|Set_isReloading true))
    (Default|SetReload (Variables|Default|GetAnimator) _output_get)))

(fn SetAnimator
  (params (Anim :type ABP%20Rocket%20Launcher%20Object%20Reference))
  (Variables|Default|SetAnimator Anim))

(fn SetAnimation
  (params (AnimName :type Name))
  (bind _animator (Variables|Default|GetAnimator))
  (bind _animation_montage (Variables|Default|GetAnimation%20Montage))
  (Animation|Montage|MontagePlay _animator _animation_montage 1.0 "MontageLength" 0.0 true)
  (Ability|Animation|MontageJumptoSection _animator AnimName _animation_montage))

(fn InitializeWeapon
  (params (CurrentAmmo :type Integer) (PlayerOwner :type BP%20Player%20Object%20Reference) (DrawWeapon :type Boolean))
  (|CallParentFunction CurrentAmmo PlayerOwner DrawWeapon)
  (Variables|Default|SetRocketLauncherAnims (Utilities|Struct|MakeSTRUCT_RocketLauncherAnims "Draw" "Idle"))
  (if DrawWeapon
    (CallFunction|DrawWeapon)))

(fn SetDraw
  (params (State :type Boolean))
  (|CallParentFunction State)
  (Default|SetDraw (Variables|Default|GetAnimator) State)
  (if (not State)
    (CallFunction|ForceReload)))

(fn SetHolster
  (params (State :type Boolean))
  (if (not (Variables|Default|Get_isHolstering))
    (|CallParentFunction State)
    (Default|SetHolster (Variables|Default|GetAnimator) State)))

(fn OnReloadEnd
  (Variables|Default|Set_isReloading false)
  (bind _ammo (Default|GetAmmoPool (Variables|Default|GetPlayerOwner) (Variables|Default|GetAmmoType)))
  (bind _ammotakenfrompool (CallFunction|GetAmmotoReload _ammo))
  (CallFunction|SetAmmoinMag _ammotakenfrompool)
  (Default|OnWeaponFinishedReloading (Variables|Default|GetPlayerOwner) _ammotakenfrompool (Variables|Default|GetAmmoType))
  (Default|SetReload (Variables|Default|GetAnimator) false))

(fn OnHolsterEnd
  (|CallParentFunction)
  (Variables|Default|Set_isHolstering false)
  (Default|OnHolsteredCurrentWeapon (Variables|Default|GetPlayerOwner))
  (Default|SetDisabled (Variables|Default|GetAnimator) true))

(fn ForceReload
  (bind _output_get (Variables|Default|Set_isShooting false))
  (Default|SetShoot (Variables|Default|GetAnimator) _output_get)
  (Default|ReloadCurrentWeapon (Variables|Default|GetPlayerOwner)))

(fn DrawWeapon
  (|CallParentFunction)
  (CallFunction|SetDraw true)
  (Default|SetDisabled (Variables|Default|GetAnimator) false))

(fn SpawnProjectile
  (|CallParentFunction)
  (bind _returnvalue (Game|SpawnActorfromClass (Variables|Default|GetProjectileClass) (Transformation|GetWorldTransform (Variables|Default|GetMuzzle)) "AlwaysSpawn" "SelectDefaultAtRuntime" self (Variables|Default|GetPlayerOwner)))
  (bind _asbp_rocket_projectile (Utilities|Casting|CastToBP_RocketProjectile _returnvalue))
  (Default|InitializeRocket _asbp_rocket_projectile self (Variables|Default|GetDamagePerShot) (Variables|Default|GetAmmoType) 0.0 0.0 (Variables|Default|GetExplosionParticle)))

(fn ForcedHolstering
  (|CallParentFunction)
  (Default|SetDisabled (Variables|Default|GetAnimator) true))