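; BP_WPNKatana is the player's katana melee weapon, a child weapon class that overrides the shared shoot, draw, holster and ammo functions.
; Shooting, gated by cooldown, drawing and holstering, plays an attack montage section, starts the cooldown delay and notifies the owning player.
; Damage comes from a projectile actor spawned at the muzzle and hard-cast to BP_HitscanMelee for a range-limited hitscan.
; Animator flags mirror weapon states, and reload is empty.
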(event Custom|Ev_ReloadEnd
  (CallFunction|OnReloadEnd))

(event Custom|Ev_ShootCooldownHandler
  (Utilities|ShootCooldownHandler))

(event EventBeginPlay
  (|CallParentFunction) ; This node is disabled and will not be called.\nDrag off pins to build functionality.
)

(event Collision|EventActorBeginOverlap
  (params (OtherActor :type Actor%20Object%20Reference))
  (|CallParentFunction OtherActor) ; This node is disabled and will not be called.\nDrag off pins to build functionality.
)

(event EventTick
  (params (DeltaSeconds :type Float%20%28single-precision%29))
  (|CallParentFunction DeltaSeconds) ; This node is disabled and will not be called.\nDrag off pins to build functionality.
)

(fn ConstructionScript
  (|CallParentFunction))

(fn Shoot
  (|CallParentFunction)
  (bind _isabletoshoot (CallFunction|CanShoot))
  (if _isabletoshoot
    (Utilities|FlowControl|Sequence
      (:then_0
        (CallFunction|SetAnimation (Utilities|Struct|BreakSTRUCT_KatanaAnims (Variables|Default|GetKatanaAnims)))
        (Default|SetShoot (Variables|Default|GetAnimator) true))
      (:then_1
        (CallFunction|EvShootCooldownHandler))
      (:then_2
        (Default|EvCurrentWeaponShot (Variables|Default|GetPlayerOwner))
        (CallFunction|SpawnProjectile)))))

(fn Reload
  (params (CurrentAmmoPool :type Integer)))

(fn SetAnimator
  (params (Anim :type ABP%20Katana%20Object%20Reference))
  (Variables|Default|SetAnimator Anim))

(fn SetAnimation
  (params (AnimName :type Name))
  (bind _animator (Variables|Default|GetAnimator))
  (bind _animation_montage (Variables|Default|GetAnimation%20Montage))
  (Animation|Montage|MontagePlay _animator _animation_montage 1.0 "MontageLength" 0.0 true)
  (Ability|Animation|MontageJumptoSection _animator AnimName _animation_montage))

(fn InitializeWeapon
  (params (CurrentAmmo :type Integer) (PlayerOwner :type BP%20Player%20Object%20Reference) (DrawWeapon :type Boolean))
  (Variables|Default|SetPlayerOwner PlayerOwner)
  (CallFunction|InitializeAmmoinMag)
  (CallFunction|InitializeRPM)
  (Variables|Default|SetKatanaAnims (Utilities|Struct|MakeSTRUCT_KatanaAnims "Draw" "Idle" "Attack" "Holster"))
  (if DrawWeapon
    (CallFunction|DrawWeapon)))

(fn SetDraw
  (params (State :type Boolean))
  (|CallParentFunction State)
  (Default|SetDraw (Variables|Default|GetAnimator) State))

(fn SetHolster
  (params (State :type Boolean))
  (if (not (Variables|Default|Get_isHolstering))
    (|CallParentFunction State)
    (Default|SetHolster (Variables|Default|GetAnimator) State)))

(fn OnReloadEnd)

(fn OnHolsterEnd
  (|CallParentFunction)
  (Variables|Default|Set_isHolstering false)
  (Default|OnHolsteredCurrentWeapon (Variables|Default|GetPlayerOwner))
  (Default|SetDisabled (Variables|Default|GetAnimator) true))

(fn DrawWeapon
  (|CallParentFunction)
  (CallFunction|SetDraw true)
  (Default|SetDisabled (Variables|Default|GetAnimator) false))

(fn CanShoot
  (return (Math|Boolean|ANDBoolean (not (Variables|Default|Get_shootInCooldown)) (not (Variables|Default|Get_isHolstering)) (not (Variables|Default|Get_isDrawing)))))

(fn InitializeAmmoinMag
  (params (CurrentAmmo :type Integer))
  (Variables|Default|Set_currentAmmoInMag (Variables|Default|GetMagSize)))

(fn SpawnProjectile
  (|CallParentFunction)
  (bind _returnvalue (Game|SpawnActorfromClass (Variables|Default|GetProjectileClass) (Transformation|GetWorldTransform (Variables|Default|GetMuzzle)) "AlwaysSpawn" "SelectDefaultAtRuntime" self (Variables|Default|GetPlayerOwner)))
  ;[1 1 1] Hardcoded?
  (bind _asbp_hitscan_melee (Utilities|Casting|CastToBP_HitscanMelee _returnvalue))
  (Default|SpawnHitscan _asbp_hitscan_melee self (Variables|Default|GetMaxDistance) (Variables|Default|GetDamagePerShot) (Variables|Default|GetAmmoType)))

(fn ForcedHolstering
  (bind _animator (Variables|Default|GetAnimator))
  (|CallParentFunction)
  (Default|SetHolster _animator false)
  (Default|SetShoot _animator false)
  (Default|SetDraw _animator false)
  (Default|SetDisabled _animator true))

(fn StopShooting
  (|CallParentFunction)
  (Default|SetShoot (Variables|Default|GetAnimator) false))