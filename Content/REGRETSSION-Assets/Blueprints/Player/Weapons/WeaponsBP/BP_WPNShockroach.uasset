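; Shockroach player weapon, a child weapon Blueprint that fires automatic hitscan beams from its muzzle.
; Each shot spawns a beam actor with damage, range and hit limit, while a cooldown timer re-fires as long as shooting stays active.
; Reload is stubbed out: drawing on initialization and each shot top up the magazine directly from the player's ammo pool.
; Animator flags drive draw, holster and shoot states, with a looping shoot montage jumping to an end section.
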(event Custom|Ev_ReloadEnd
  (CallFunction|OnReloadEnd))

(event Custom|Ev_ShootCooldownHandler
  (Utilities|ShootCooldownHandler))

(fn ConstructionScript
  (|CallParentFunction))

(fn StopShooting
  (bind _output_get (Variables|Default|Set_isShooting false))
  (if (Math|Boolean|NORBoolean (Variables|Default|Get_isDrawing) (Variables|Default|Get_isHolstering))
    (CallFunction|SetShootingMontage _output_get)))

(fn Shoot
  (|CallParentFunction)
  (bind _isabletoshoot (CallFunction|CanShoot))
  (if _isabletoshoot
    (Utilities|FlowControl|Sequence
      (:then_0
        (if (not (Variables|Default|Get_isShooting))
          (CallFunction|SetShootingMontage true)))
      (:then_1
        (CallFunction|EvShootCooldownHandler))
      (:then_2
        (Variables|Default|Set_isShooting true))
      (:then_3
        (Default|EvCurrentWeaponShot (Variables|Default|GetPlayerOwner))
        (CallFunction|ConsumeAmmo)
        (CallFunction|SpawnProjectile)))))

(fn CanShoot
  (bind _isabletoshoot (|CallParentFunction))
  (Utilities|FlowControl|Sequence
    (:then_0
      (if (not _isabletoshoot)
        (Variables|Default|Set_isShooting false)))
    (:then_1
      (return _isabletoshoot))))

(fn Reload
  (params (CurrentAmmoPool :type Integer)))

(fn SetAnimator
  (params (Anim :type ABP%20Shockroach%20Object%20Reference))
  (Variables|Default|SetAnimator Anim))

(fn SetAnimation
  (params (AnimName :type Name))
  (bind _animator (Variables|Default|GetAnimator))
  (bind _animation_montage (Variables|Default|GetAnimation%20Montage))
  (Animation|Montage|MontagePlay _animator _animation_montage 1.0 "MontageLength" 0.0 true)
  (Ability|Animation|MontageJumptoSection _animator AnimName _animation_montage))

(fn InitializeWeapon
  (params (CurrentAmmo :type Integer) (PlayerOwner :type BP%20Player%20Object%20Reference) (DrawWeapon :type Boolean))
  (|CallParentFunction CurrentAmmo PlayerOwner DrawWeapon)
  (Variables|Default|SetShockroachAnims (Utilities|Struct|MakeSTRUCT_ShockroachAnims "Draw" "Idle"))
  (if DrawWeapon
    (CallFunction|DrawWeapon)
    (bind _ammo (Default|GetAmmoPool (Variables|Default|GetPlayerOwner) (Variables|Default|GetAmmoType)))
    (bind _ammotakenfrompool (CallFunction|GetAmmotoReload _ammo))
    (CallFunction|SetAmmoinMag _ammotakenfrompool)
    (Default|OnWeaponFinishedReloading (Variables|Default|GetPlayerOwner) _ammotakenfrompool (Variables|Default|GetAmmoType))))

(fn SetDraw
  (params (State :type Boolean))
  (|CallParentFunction State)
  (Default|SetDraw (Variables|Default|GetAnimator) State))

(fn SetHolster
  (params (State :type Boolean))
  (if (not (Variables|Default|Get_isHolstering))
    (|CallParentFunction State)
    (Default|SetHolster (Variables|Default|GetAnimator) State)))

(fn OnReloadEnd)

(fn OnHolsterEnd
  (bind _animator (Variables|Default|GetAnimator))
  (|CallParentFunction)
  (Variables|Default|Set_isHolstering false)
  (Default|SetHolster _animator false)
  (Default|SetDisabledWeapon _animator true)
  (Default|OnHolsteredCurrentWeapon (Variables|Default|GetPlayerOwner)))

(fn DrawWeapon
  (|CallParentFunction)
  (Default|SetDisabledWeapon (Variables|Default|GetAnimator) false)
  (CallFunction|SetDraw true)
  (Variables|Default|Set_isShooting false))

(fn OnShootEnd)

(fn CheckAutomaticFire
  (if (and (not (Variables|Default|Get_shootInCooldown)) (Variables|Default|Get_isShooting))
    (CallFunction|Shoot)))

(fn ConsumeAmmo
  (if (not (> (Variables|Default|GetAmmoConsumption) (Variables|Default|Get_currentAmmoInMag)))
    (Variables|Default|Set_currentAmmoInMag (- (Variables|Default|Get_currentAmmoInMag) (Variables|Default|GetAmmoConsumption)))
    (bind _ammo (Default|GetAmmoPool (Variables|Default|GetPlayerOwner) (Variables|Default|GetAmmoType)))
    (bind _ammotakenfrompool (CallFunction|GetAmmotoReload _ammo))
    (CallFunction|SetAmmoinMag _ammotakenfrompool)
    (Default|OnWeaponFinishedReloading (Variables|Default|GetPlayerOwner) _ammotakenfrompool (Variables|Default|GetAmmoType))))

(fn SpawnProjectile
  (|CallParentFunction)
  (bind _returnvalue (Game|SpawnActorfromClass (Variables|Default|GetProjectileClass) (Transformation|GetWorldTransform (Variables|Default|GetMuzzle)) "AlwaysSpawn" "SelectDefaultAtRuntime" self (Variables|Default|GetPlayerOwner)))
  (bind _asbp_hitscan_beam (Utilities|Casting|CastToBP_HitscanBeam _returnvalue))
  (Default|SpawnHitscan _asbp_hitscan_beam self (Variables|Default|GetMaxDistance) (Variables|Default|GetDamagePerShot) (Variables|Default|GetAmmoType) (Variables|Default|GetMaxHitsPerBeam)))

(fn SetShootingMontage
  (params (Shooting :type Boolean))
  (Default|SetShoot (Variables|Default|GetAnimator) Shooting)
  (if Shooting
    (Animation|Montage|MontagePlay (Variables|Default|GetAnimator) "/Game/REGRETSSION-Assets/Art/Weapons/Shockroach/Animations/AM_Shockroash_Anim_ShootCycle.AM_Shockroash_Anim_ShootCycle" 1.0 "MontageLength" 0.0 true)
    (else
      (Ability|Animation|MontageJumptoSection (Variables|Default|GetAnimator) (Utilities|Struct|BreakSTRUCT_ShockroachAnims (Variables|Default|GetShockroachAnims)) "/Game/REGRETSSION-Assets/Art/Weapons/Shockroach/Animations/AM_Shockroash_Anim_ShootCycle.AM_Shockroash_Anim_ShootCycle"))))

(fn ForcedHolstering
  (Default|SetDisabledWeapon (Variables|Default|GetAnimator) true)
  (|CallParentFunction))