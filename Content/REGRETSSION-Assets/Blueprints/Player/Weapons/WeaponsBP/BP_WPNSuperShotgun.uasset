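; Super shotgun weapon Blueprint that overrides a parent weapon's shoot, reload, draw and holster logic, passing state to its Animator.
; Firing spends magazine ammo, starts a delay-based cooldown, notifies the owning player and spawns a hitscan shell actor with pellet count and spread via a hardcoded cast.
; Reloads trigger on a failed shot or when draw ends, and reload completion refills the magazine and reports to the player.
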(event Custom|Ev_ReloadEnd
  (CallFunction|OnReloadEnd))

(event Custom|Ev_ShootCooldownHandler
  (Utilities|ShootCooldownHandler))

(event EventBeginPlay
  (|CallParentFunction) ; This node is disabled and will not be called.\nDrag off pins to build functionality.
)

(event EventTick
  (params (DeltaSeconds :type Float%20%28single-precision%29))
  (|CallParentFunction DeltaSeconds) ; This node is disabled and will not be called.\nDrag off pins to build functionality.
)

(fn ConstructionScript
  (|CallParentFunction))

(fn Shoot
  (|CallParentFunction)
  (bind _isabletoshoot (CallFunction|CanShoot))
  (if _isabletoshoot
    (Utilities|FlowControl|Sequence
      (:then_0
        (Default|SetShoot (Variables|Default|GetAnimator) true))
      (:then_1
        (Variables|Default|Set_currentAmmoInMag (- (Variables|Default|Get_currentAmmoInMag) (Variables|Default|GetAmmoConsumption)))
        (CallFunction|EvShootCooldownHandler))
      (:then_2
        (Variables|Default|Set_isShooting true))
      (:then_3
        (Default|EvCurrentWeaponShot (Variables|Default|GetPlayerOwner))
        (CallFunction|SpawnProjectile)
        (CallFunction|SpawnMuzzleFlash)))
    (else
      (bind _ammo (CallFunction|GetAmmoPool (Variables|Default|GetAmmoType)))
      (bind _forcereload (CallFunction|HastoForceReload _ammo))
      (if _forcereload
        (CallFunction|Reload _ammo)))))

(fn Reload
  (params (CurrentAmmoPool :type Integer))
  (bind _reloadavailable (CallFunction|CanReload CurrentAmmoPool))
  (if _reloadavailable
    (bind _output_get (Variables|Default|Set_isReloading true))
    (Default|SetReload (Variables|Default|GetAnimator) _output_get)))

(fn SetAnimator
  (params (Anim :type ABP%20Super%20Shotgun%20Object%20Reference))
  (Variables|Default|SetAnimator Anim))

(fn SetAnimation
  (params (AnimName :type Name))
  (bind _animator (Variables|Default|GetAnimator))
  (bind _animation_montage (Variables|Default|GetAnimation%20Montage))
  (Utilities|FlowControl|Sequence
    (:then_0
      (if (not (Class|AnimInstance|IsAnyMontagePlaying _animator))
        (Animation|Montage|MontagePlay _animator _animation_montage 1.0 "MontageLength" 0.0 true)))
    (:then_1
      (Ability|Animation|MontageJumptoSection _animator AnimName _animation_montage))))

(fn InitializeWeapon
  (params (CurrentAmmo :type Integer) (PlayerOwner :type BP%20Player%20Object%20Reference) (DrawWeapon :type Boolean))
  (|CallParentFunction CurrentAmmo PlayerOwner DrawWeapon)
  (Variables|Default|SetSSGAnims (Utilities|Struct|MakeSTRUCT_SuperShotgunAnims "Draw" "Idle"))
  (if DrawWeapon
    (CallFunction|DrawWeapon)))

(fn SetDraw
  (params (State :type Boolean))
  (|CallParentFunction State)
  (Default|SetDraw (Variables|Default|GetAnimator) State)
  (if (not State)
    (CallFunction|ForceReload)))

(fn SetHolster
  (params (State :type Boolean))
  (if (not (Variables|Default|Get_isHolstering))
    (|CallParentFunction State)
    (Default|SetHolster (Variables|Default|GetAnimator) State)))

(fn OnReloadEnd
  (Variables|Default|Set_isReloading false)
  (bind _ammo (Default|GetAmmoPool (Variables|Default|GetPlayerOwner) (Variables|Default|GetAmmoType)))
  (bind _ammotakenfrompool (CallFunction|GetAmmotoReload _ammo))
  (CallFunction|SetAmmoinMag _ammotakenfrompool)
  (Default|OnWeaponFinishedReloading (Variables|Default|GetPlayerOwner) _ammotakenfrompool (Variables|Default|GetAmmoType))
  (Default|SetReload (Variables|Default|GetAnimator) false))

(fn OnHolsterEnd
  (|CallParentFunction)
  (Variables|Default|Set_isHolstering false)
  (Default|OnHolsteredCurrentWeapon (Variables|Default|GetPlayerOwner))
  (Default|SetDisabled (Variables|Default|GetAnimator) true))

(fn ForceReload
  (bind _output_get (Variables|Default|Set_isShooting false))
  (Default|SetShoot (Variables|Default|GetAnimator) _output_get)
  (Default|ReloadCurrentWeapon (Variables|Default|GetPlayerOwner)))

(fn DrawWeapon
  (|CallParentFunction)
  (CallFunction|SetDraw true)
  (Default|SetDisabled (Variables|Default|GetAnimator) false))

(fn SpawnProjectile
  (|CallParentFunction)
  (bind _returnvalue (Game|SpawnActorfromClass (Variables|Default|GetProjectileClass) (Transformation|GetWorldTransform (Variables|Default|GetMuzzle)) "AlwaysSpawn" "SelectDefaultAtRuntime" self (Variables|Default|GetPlayerOwner)))
  ;[1 1 1] Hardcoded!
  (bind _asbp_hitscan_shell (Utilities|Casting|CastToBP_HitscanShell _returnvalue))
  (Default|SpawnHitscan _asbp_hitscan_shell self (Variables|Default|GetMaxDistance) (Variables|Default|GetDamagePerShot) (Variables|Default|GetAmmoType) (Variables|Default|GetPelletAmount) (Variables|Default|GetVerticalSpread) (Variables|Default|GetHorizontalSpread)))

(fn ForcedHolstering
  (|CallParentFunction)
  (Default|SetDisabled (Variables|Default|GetAnimator) true))