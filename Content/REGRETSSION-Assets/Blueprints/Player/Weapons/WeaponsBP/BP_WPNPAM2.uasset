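; PAM2 automatic firearm: a weapon Blueprint that overrides a parent weapon's shoot, reload, draw and holster behavior, mirroring state to its Animator.
; Shooting spends magazine ammo, spawns a spread-adjusted BP_HitscanBullet with muzzle flash and sound, or forces a reload when needed.
; A cooldown delay re-triggers Shoot while firing is held, producing automatic fire.
; Reload completion refills the magazine from the owning player's ammo pool and notifies the player.
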(event Custom|Ev_ReloadEnd
  (CallFunction|OnReloadEnd))

(event Custom|Ev_ShootCooldownHandler
  (Utilities|ShootCooldownHandler))

(event EventBeginPlay
  (|CallParentFunction) ; This node is disabled and will not be called.\nDrag off pins to build functionality.
)

(event Collision|EventActorBeginOverlap
  (params (OtherActor :type Actor%20Object%20Reference))
  (|CallParentFunction OtherActor) ; This node is disabled and will not be called.\nDrag off pins to build functionality.
)

(event EventTick
  (params (DeltaSeconds :type Float%20%28single-precision%29))
  (|CallParentFunction DeltaSeconds) ; This node is disabled and will not be called.\nDrag off pins to build functionality.
)

(fn ConstructionScript
  (|CallParentFunction))

(fn StopShooting
  (bind _output_get (Variables|Default|Set_isShooting false))
  (Default|SetShoot (Variables|Default|GetAnimator) _output_get)
  (Default|OnShootEnd (Variables|Default|GetWeaponSpreadComponent)))

(fn Shoot
  (|CallParentFunction)
  (bind _isabletoshoot (CallFunction|CanShoot))
  (if _isabletoshoot
    (Utilities|FlowControl|Sequence
      (:then_0
        (CallFunction|SetAnimation (Utilities|Struct|BreakSTRUCT_PAM2Anims (Variables|Default|GetPAM2Anims)))
        (Default|SetShoot (Variables|Default|GetAnimator) true))
      (:then_1
        (Variables|Default|Set_currentAmmoInMag (- (Variables|Default|Get_currentAmmoInMag) (Variables|Default|GetAmmoConsumption)))
        (CallFunction|EvShootCooldownHandler))
      (:then_2
        (Variables|Default|Set_isShooting true))
      (:then_3
        (Default|EvCurrentWeaponShot (Variables|Default|GetPlayerOwner))
        (CallFunction|SpawnProjectile)
        (CallFunction|SpawnMuzzleFlash)
        (Audio|SpawnSoundAttached "/Game/REGRETSSION-Assets/Art/Weapons/PAM2/Sounds/greasegun_shoot_Cue.greasegun_shoot_Cue" (Variables|Default|GetMuzzle) "None" "0, 0, 0" "0, 0, 0" "KeepRelativeOffset" false 1.0 1.0 0.0 0 0)
        (Default|OnShoot (Variables|Default|GetWeaponSpreadComponent))))
    (else
      (bind _ammo (CallFunction|GetAmmoPool (Variables|Default|GetAmmoType)))
      (bind _forcereload (CallFunction|HastoForceReload _ammo))
      (if _forcereload
        (CallFunction|Reload _ammo)))))

(fn CanShoot
  (bind _isabletoshoot (|CallParentFunction))
  (Utilities|FlowControl|Sequence
    (:then_0
      (if (not _isabletoshoot)
        (Variables|Default|Set_isShooting false)))
    (:then_1
      (return _isabletoshoot))))

(fn Reload
  (params (CurrentAmmoPool :type Integer))
  (bind _reloadavailable (CallFunction|CanReload CurrentAmmoPool))
  (if _reloadavailable
    (Variables|Default|Set_isReloading true)
    (bind _empty (CallFunction|GetEmptyMag))
    (Default|SetReload (Variables|Default|GetAnimator) true _empty)))

(fn SetAnimator
  (params (Anim :type ABP%20PAM2%20Object%20Reference))
  (Variables|Default|SetAnimator Anim))

(fn SetAnimation
  (params (AnimName :type Name))
  (bind _animator (Variables|Default|GetAnimator))
  (bind _animation_montage (Variables|Default|GetAnimation%20Montage))
  (Animation|Montage|MontagePlay _animator _animation_montage 1.0 "MontageLength" 0.0 true)
  (Ability|Animation|MontageJumptoSection _animator AnimName _animation_montage))

(fn InitializeWeapon
  (params (CurrentAmmo :type Integer) (PlayerOwner :type BP%20Player%20Object%20Reference) (DrawWeapon :type Boolean))
  (|CallParentFunction CurrentAmmo PlayerOwner DrawWeapon)
  (Variables|Default|SetPAM2Anims (Utilities|Struct|MakeSTRUCT_PAM2Anims "Draw" "Idle"))
  (if DrawWeapon
    (CallFunction|DrawWeapon)))

(fn SetDraw
  (params (State :type Boolean))
  (|CallParentFunction State)
  (Default|SetDraw (Variables|Default|GetAnimator) State))

(fn SetHolster
  (params (State :type Boolean))
  (if (not (Variables|Default|Get_isHolstering))
    (|CallParentFunction State)
    (Default|SetHolster (Variables|Default|GetAnimator) State)))

(fn OnReloadEnd
  (Variables|Default|Set_isReloading false)
  (bind _ammo (Default|GetAmmoPool (Variables|Default|GetPlayerOwner) (Variables|Default|GetAmmoType)))
  (bind _ammotakenfrompool (CallFunction|GetAmmotoReload _ammo))
  (CallFunction|SetAmmoinMag _ammotakenfrompool)
  (Default|OnWeaponFinishedReloading (Variables|Default|GetPlayerOwner) _ammotakenfrompool (Variables|Default|GetAmmoType))
  (Default|SetReload (Variables|Default|GetAnimator) false false))

(fn OnHolsterEnd
  (|CallParentFunction)
  (Variables|Default|Set_isHolstering false)
  (Default|OnHolsteredCurrentWeapon (Variables|Default|GetPlayerOwner))
  (Default|SetDisabled (Variables|Default|GetAnimator) true))

(fn DrawWeapon
  (|CallParentFunction)
  (CallFunction|SetDraw true)
  (Default|SetDisabled (Variables|Default|GetAnimator) false))

(fn CheckAutomaticFire
  (if (and (not (Variables|Default|Get_shootInCooldown)) (Variables|Default|Get_isShooting))
    (CallFunction|Shoot)))

(fn SpawnProjectile
  (|CallParentFunction)
  (bind _returnvalue (Game|SpawnActorfromClass (Variables|Default|GetProjectileClass) (Transformation|GetWorldTransform (Variables|Default|GetMuzzle)) "AlwaysSpawn" "SelectDefaultAtRuntime" self (Variables|Default|GetPlayerOwner)))
  ;[1 1 1] Hardcoded?
  (bind _asbp_hitscan_bullet (Utilities|Casting|CastToBP_HitscanBullet _returnvalue))
  (bind (_xspread _yspread) (Default|GetSpread (Variables|Default|GetWeaponSpreadComponent)))
  (Default|SpawnHitscan _asbp_hitscan_bullet self (Variables|Default|GetMaxDistance) (Variables|Default|GetDamagePerShot) (Variables|Default|GetAmmoType) _xspread _yspread))

(fn ForcedHolstering
  (|CallParentFunction)
  (Default|SetDisabled (Variables|Default|GetAnimator) true))