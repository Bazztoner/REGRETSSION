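; Base weapon Blueprint for the player, holding shared ammo, state and muzzle-flash logic, with shooting, projectile spawning and end-of-action hooks left empty.
; Initialization fills the magazine and derives shot cooldown from RPM.
; State flags for shooting, reloading, drawing and holstering gate CanShoot and CanReload, while reserve ammo comes from the owning player.
; Sway eases the mesh toward its cached rotation when input is idle; computed input offsets are never applied.
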(event EventBeginPlay
  (Variables|Default|SetDefaultTransform (Transformation|GetRelativeTransform (Variables|Default|GetWeaponMesh))))

(event Collision|EventActorBeginOverlap
  (params (OtherActor :type Actor%20Object%20Reference)))

(fn ConstructionScript)

(fn StopShooting)

(fn Shoot)

(fn SpawnProjectile)

(fn SpawnMuzzleFlash
  (bind _muzzle (Variables|Default|GetMuzzle))
  (bind _returnvalue (Transformation|GetWorldTransform _muzzle))
  (Niagara|SpawnSystemAttached (Variables|Default|GetMuzzleFlashParticle) (Variables|Default|GetWeaponMesh) "" (.location _returnvalue) (.rotation _returnvalue) "KeepWorldPosition" true true "AutoRelease" false))

(fn Reload
  (params (CurrentAmmoPool :type Integer))
  (bind _reloadavailable (CallFunction|CanReload CurrentAmmoPool))
  (if _reloadavailable
    (Variables|Default|Set_isReloading true)))

(fn InitializeWeapon
  (params (CurrentAmmo :type Integer) (PlayerOwner :type BP%20Player%20Object%20Reference) (DrawWeapon :type Boolean))
  (Variables|Default|SetPlayerOwner PlayerOwner)
  (CallFunction|InitializeAmmoinMag CurrentAmmo)
  (CallFunction|InitializeRPM))

(fn InitializeAmmoinMag
  (params (CurrentAmmo :type Integer))
  (bind _magsize (Variables|Default|GetMagSize))
  (if (< CurrentAmmo _magsize)
    (Variables|Default|Set_currentAmmoInMag CurrentAmmo)
    (else
      (Variables|Default|Set_currentAmmoInMag _magsize))))

(fn InitializeRPM
  (Variables|Default|Set_shootCD (/ 6e+01 (Variables|Default|GetRPM))))

(fn HastoForceReload
  (params (AmmoPool :type Integer))
  (Utilities|FlowControl|Sequence
    (:then_0
      (LocalVariables|SetAmmo%20Pool AmmoPool))
    (:then_1
      (return (< (Variables|Default|Get_currentAmmoInMag) (Variables|Default|GetAmmoConsumption))))))

(fn CanShoot
  (bind __currentammoinmag (Variables|Default|Get_currentAmmoInMag))
  (bind _ammoconsumption (Variables|Default|GetAmmoConsumption))
  (bind _returnvalue (>= __currentammoinmag _ammoconsumption))
  (if _returnvalue
    (return (Math|Boolean|ANDBoolean _returnvalue (not (Variables|Default|Get_isReloading)) (not (Variables|Default|Get_shootInCooldown)) (not (Variables|Default|Get_isHolstering)) (not (Variables|Default|Get_isDrawing))))
    (else
      (return false))))

(fn CanReload
  (params (AmmoPool :type Integer))
  (Utilities|FlowControl|Sequence
    (:then_0
      (LocalVariables|SetAmmo%20Pool AmmoPool))
    (:then_1
      (return (Math|Boolean|ANDBoolean (>= (LocalVariables|GetAmmo%20Pool) (Variables|Default|GetAmmoConsumption)) (< (Variables|Default|Get_currentAmmoInMag) (Variables|Default|GetMagSize)) (not (Variables|Default|Get_isReloading)) (not (Variables|Default|Get_isHolstering)) (not (Variables|Default|Get_isDrawing)) (not (Variables|Default|Get_isShooting)))))))

(fn GetAmmotoReload
  (params (AmmoPool :type Integer))
  (LocalVariables|SetCurrent%20Ammo AmmoPool)
  (bind _output_get (LocalVariables|SetMissingAmmo (- (Variables|Default|GetMagSize) (Variables|Default|Get_currentAmmoInMag))))
  (if (<= (LocalVariables|GetCurrent%20Ammo) _output_get)
    (return (LocalVariables|GetCurrent%20Ammo))
    (else
      (return _output_get))))

(fn SetAmmoinMag
  (params (AddedAmmo :type Integer))
  (Variables|Default|Set_currentAmmoInMag (Math|Integer|Clamp(Integer) (+ AddedAmmo (Variables|Default|Get_currentAmmoInMag)) 0 (Variables|Default|GetMagSize))))

(fn SetDraw
  (params (State :type Boolean))
  (Variables|Default|Set_isDrawing State))

(fn SetHolster
  (params (State :type Boolean))
  (Variables|Default|Set_isHolstering State))

(fn OnHolsterEnd)

(fn OnReloadEnd)

(fn GetAmmoPool
  (params (Type :type ENUM_AmmoTypes%20Enum :default "NewEnumerator0"))
  (bind _ammo (Default|GetAmmoPool (Variables|Default|GetPlayerOwner) Type))
  (return _ammo))

(fn GetWeaponWheelXY
  (return (Variables|Default|GetWpnWheelXPos) (Variables|Default|GetWpnWheelYPos)))

(fn DrawWeapon
  (Variables|Default|Set_isReloading false)
  (Variables|Default|Set_isHolstering false)
  (Variables|Default|Set_isShooting false))

(fn ForcedHolstering
  (CallFunction|SetActive self false)
  (Variables|Default|Set_isReloading false)
  (Variables|Default|Set_isHolstering false)
  (Variables|Default|Set_isDrawing false)
  (Variables|Default|Set_isShooting false))

(fn AddWeaponSway
  (params (Delta :type Vector%202D%20Structure))
  (bind _swaydata (Variables|Default|GetSwayData))
  (bind _swaytime (Utilities|Struct|BreakSTRUCT_BaseWeaponProcAnimValues _swaydata))
  (if (Class|KismetMathLibrary|IsNearlyZero2D Delta 0.0001)
    (bind (_deltax _deltay) (|GetDeltaRotations)
      (:Out
        (Transformation|AddLocalRotation (Variables|Default|GetWeaponMesh) (Math|Rotator|MakeRotator _deltax 0.0 _deltay) false false)
        (Variables|Default|SetSwayCurrentTime (Math|Float|Clamp(Float) (/ (+ (Variables|Default|GetSwayCurrentTime) (Utilities|Time|GetWorldDeltaSeconds)) _swaytime) 0.0 _swaytime))))
    (else
      (|CheckApplyableDeltaRotation Delta
        (:Out
          (Variables|Default|SetSwayCurrentTime 0.0))))))

(fn GetEmptyMag
  (return (<= (Variables|Default|Get_currentAmmoInMag) 0)))