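; Weapon component that tracks horizontal and vertical bullet spread, which grows with each shot and recovers after firing stops.
; OnShoot cancels any pending recovery timer and adds clamped per-shot spread, while OnShootEnd starts a delay timer that enables decay.
; Tick then lowers both axes at a linear rate scaled from each maximum over SpreadMaxTime.
; GetSpread returns a random offset within the current range on each axis.
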(event Custom|OnShootEnd
  (bind _returnvalue (Utilities|Time|SetTimerbyEvent (delegate Custom|StartSpreadDecrease) (Variables|Default|GetdelayAfterShot)))
  (Variables|Default|SetTimerToDecrease _returnvalue))

(event Custom|StartSpreadDecrease
  (Variables|Default|SetisDecreasingSpread true))

(event Custom|OnShoot
  (Utilities|FlowControl|Sequence
    (:then_0
      (if (Utilities|Time|IsValidTimerHandle (Variables|Default|GetTimerToDecrease))
        (Utilities|Time|ClearandInvalidateTimerbyHandle (Variables|Default|GetTimerToDecrease))))
    (:then_1
      (CallFunction|AddSpread))
    (:then_2
      (Variables|Default|SetisDecreasingSpread false))))

(event EventTick
  (params (DeltaSeconds :type Float%20%28single-precision%29))
  (CallFunction|RemoveSpread DeltaSeconds))

(fn AddSpread
  (Variables|Default|SetcurrentXSpread (Math|Float|Clamp(Float) (+ (Variables|Default|GetcurrentXSpread) (Variables|Default|GetXspreadSumPerShot)) (Variables|Default|GetminXSpread) (Variables|Default|GetmaxXSpread)))
  (Variables|Default|SetcurrentYSpread (Math|Float|Clamp(Float) (+ (Variables|Default|GetcurrentYSpread) (Variables|Default|GetYspreadSumPerShot)) (Variables|Default|GetminYSpread) (Variables|Default|GetmaxYSpread))))

(fn DecreaseSpread
  (params (XDecrease :type Float%20%28single-precision%29) (YDecrease :type Float%20%28single-precision%29))
  (Variables|Default|SetcurrentXSpread (Math|Float|Clamp(Float) (- (Variables|Default|GetcurrentXSpread) XDecrease) (Variables|Default|GetminXSpread) (Variables|Default|GetmaxXSpread)))
  (Variables|Default|SetcurrentYSpread (Math|Float|Clamp(Float) (- (Variables|Default|GetcurrentYSpread) YDecrease) (Variables|Default|GetminYSpread) (Variables|Default|GetmaxYSpread))))

(fn RemoveSpread
  (params (Delta :type Float%20%28single-precision%29))
  (if (Variables|Default|GetisDecreasingSpread)
    (bind (_xdecrease _ydecrease) (CallFunction|GetDecreaseQuota Delta))
    (CallFunction|DecreaseSpread _xdecrease _ydecrease)
    (else
      (return))))

(fn GetSpread
  (bind _currentxspread (Variables|Default|GetcurrentXSpread))
  (bind _currentyspread (Variables|Default|GetcurrentYSpread))
  (return (Math|Random|RandomFloatinRange (* -1 _currentxspread) _currentxspread) (Math|Random|RandomFloatinRange (* -1 _currentyspread) _currentyspread)))

(fn GetDecreaseQuota
  (params (Delta :type Float%20%28single-precision%29))
  (LocalVariables|SetDeltaTime Delta)
  (Utilities|FlowControl|Sequence
    (:then_0
      (bind _result (CallFunction|SimpleThreeRule (Variables|Default|GetspreadMaxTime) (Variables|Default|GetmaxXSpread) (LocalVariables|GetDeltaTime)))
      (LocalVariables|SetDecreaseX _result))
    (:then_1
      (bind _result_2 (CallFunction|SimpleThreeRule (Variables|Default|GetspreadMaxTime) (Variables|Default|GetmaxYSpread) (LocalVariables|GetDeltaTime)))
      (LocalVariables|SetDecreaseY _result_2))
    (:then_2
      (return (LocalVariables|GetDecreaseX) (LocalVariables|GetDecreaseY)))))