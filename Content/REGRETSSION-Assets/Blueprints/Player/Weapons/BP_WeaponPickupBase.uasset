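; Base weapon pickup actor that offers a weapon and ammo to the player on touch.
; When a BP_Player overlaps it, it passes its weapon class, ammo type and ammo amount to the player's CheckPickupWeaponClass.
; It then deactivates itself through SetActive rather than being destroyed, without checking whether the player used the pickup.
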(event EventBeginPlay
  (|CallParentFunction))

(event Collision|EventActorBeginOverlap
  (params (OtherActor :type Actor%20Object%20Reference))
  (bind _asfpsreg (Utilities|Casting|CastToBP_Player OtherActor))
  (Default|CheckPickupWeaponClass _asfpsreg (Variables|Default|GetWeaponPickupClass) (Variables|Default|GetAmmoType) (Variables|Default|GetPickupAmmoAmount))
  (CallFunction|SetActive self false))

(event EventTick
  (params (DeltaSeconds :type Float%20%28single-precision%29))
  (|CallParentFunction DeltaSeconds) ; This node is disabled and will not be called.\nDrag off pins to build functionality.
)

(fn ConstructionScript
  (|CallParentFunction))