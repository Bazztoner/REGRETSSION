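; Desert Eagle player weapon, a child weapon Blueprint that handles shooting, reloading, drawing and holstering.
; Shooting spends magazine ammo and starts a delay-based cooldown, or triggers a forced reload when firing is blocked and one is needed.
; Each action jumps to a named section of one montage, with separate last-shot and empty-idle variants.
; Reload and holster end handlers report back to the owning player, which supplies the ammo pool; holster end also prints a leftover debug string.
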(event Custom|Ev_ReloadEnd
  (CallFunction|OnReloadEnd))

(event Custom|Ev_ShootCooldownHandler
  (Utilities|ShootCooldownHandler))

(event EventBeginPlay
  (|CallParentFunction) ; This node is disabled and will not be called.\nDrag off pins to build functionality.
)

(event Collision|EventActorBeginOverlap
  (params (OtherActor :type Actor%20Object%20Reference))
  (|CallParentFunction OtherActor) ; This node is disabled and will not be called.\nDrag off pins to build functionality.
)

(event EventTick
  (params (DeltaSeconds :type Float%20%28single-precision%29))
  (|CallParentFunction DeltaSeconds) ; This node is disabled and will not be called.\nDrag off pins to build functionality.
)

(fn ConstructionScript
  (|CallParentFunction))

(fn Shoot
  (bind _deagleanims (Variables|Default|GetDeagleAnims))
  (bind (_shoot _shoot_last) (Utilities|Struct|BreakSTRUCT_DeagleAnims _deagleanims))
  (|CallParentFunction)
  (bind _isabletoshoot (CallFunction|CanShoot))
  (if _isabletoshoot
    (Utilities|FlowControl|Sequence
      (:then_0
        (if (> (Variables|Default|Get_currentAmmoInMag) 1)
          (LocalVariables|Setanim _shoot)
          (else
            (LocalVariables|Setanim _shoot_last))))
      (:then_1
        (CallFunction|SetAnimation (LocalVariables|Getanim)))
      (:then_2
        (Variables|Default|Set_currentAmmoInMag (- (Variables|Default|Get_currentAmmoInMag) (Variables|Default|GetAmmoConsumption)))
        (CallFunction|EvShootCooldownHandler)))
    (else
      (bind _ammo (CallFunction|GetAmmoPool (Variables|Default|GetAmmoType)))
      (bind _forcereload (CallFunction|HastoForceReload _ammo))
      (if _forcereload
        (CallFunction|Reload _ammo)))))

(fn Reload
  (params (CurrentAmmoPool :type Integer))
  (bind _reloadavailable (CallFunction|CanReload CurrentAmmoPool))
  (if _reloadavailable
    (Variables|Default|Set_isReloading true)
    (CallFunction|SetAnimation (.Reload (Utilities|Struct|BreakSTRUCT_DeagleAnims (Variables|Default|GetDeagleAnims))))))

(fn SetAnimator
  (params (Anim :type ABP%20Deagle%20Object%20Reference))
  (Variables|Default|SetAnimator Anim))

(fn SetAnimation
  (params (AnimName :type Name))
  (bind _animator (Variables|Default|GetAnimator))
  (bind _animation_montage (Variables|Default|GetAnimation%20Montage))
  (Animation|Montage|MontagePlay _animator _animation_montage 1.0 "MontageLength" 0.0 true)
  (Ability|Animation|MontageJumptoSection _animator AnimName _animation_montage))

(fn InitializeWeapon
  (params (CurrentAmmo :type Integer) (PlayerOwner :type FPS%20Reg%20Object%20Reference))
  (|CallParentFunction CurrentAmmo PlayerOwner)
  (Variables|Default|SetDeagleAnims (Utilities|Struct|MakeSTRUCT_DeagleAnims "Draw" "Idle"))
  (CallFunction|SetDraw true))

(fn SetDraw
  (params (State :type Boolean))
  (bind _deagleanims (Variables|Default|GetDeagleAnims))
  (bind (_draw _idle _shoot _shoot_last _idle_empty) (Utilities|Struct|BreakSTRUCT_DeagleAnims _deagleanims))
  (|CallParentFunction State)
  (if State
    (CallFunction|SetAnimation _draw)
    (elif (!= (Variables|Default|Get_currentAmmoInMag) 0)
      (CallFunction|SetAnimation _idle)
      (else
        (CallFunction|SetAnimation _idle_empty)))))

(fn SetHolster
  (params (State :type Boolean))
  (if (not (Variables|Default|Get_isHolstering))
    (|CallParentFunction State)
    (if State
      (CallFunction|SetAnimation (.Holster (Utilities|Struct|BreakSTRUCT_DeagleAnims (Variables|Default|GetDeagleAnims)))))))

(fn OnReloadEnd
  (Variables|Default|Set_isReloading false)
  (bind _ammo (Default|GetAmmoPool (Variables|Default|GetPlayerOwner) (Variables|Default|GetAmmoType)))
  (bind _ammotakenfrompool (CallFunction|GetAmmotoReload _ammo))
  (CallFunction|SetAmmoinMag _ammotakenfrompool)
  (Default|OnWeaponFinishedReloading (Variables|Default|GetPlayerOwner) _ammotakenfrompool (Variables|Default|GetAmmoType)))

(fn OnHolsterEnd
  (|CallParentFunction)
  (Development|PrintString "Sorete de mierda" true true "(R=1.000000,G=0.221643,B=0.000000,A=1.000000)" 6.0)
  (Default|OnHolsteredCurrentWeapon (Variables|Default|GetPlayerOwner)))