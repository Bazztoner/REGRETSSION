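; Decal manager actor that spawns surface-appropriate decals, including bullet wounds on flesh, either at a world location or attached to a component.
; Both spawn functions take a physical surface and get a random material from the Generic, Concrete, Metal or BulletWounds array through GetDecalBySurface.
; Hard, masonry-like surfaces share the Concrete set, while most others fall back to Generic.
; Spawned decals get a hardcoded zero fade screen size.
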(event EventBeginPlay)

(event Collision|EventActorBeginOverlap
  (params (OtherActor :type Actor%20Object%20Reference)))

(event EventTick
  (params (DeltaSeconds :type Float%20%28single-precision%29)))

(fn ConstructionScript)

(fn SpawnDecalatLocation
  (params (PhysicalSurface :type EPhysicalSurface%20Enum :default "SurfaceType_Default") (DecalSize :type Vector) (Location :type Vector) (Rotation :type Rotator) (LifeSpan :type Float%20%28double-precision%29))
  (bind _decalselected (CallFunction|GetDecalbySurface PhysicalSurface))
  (bind _returnvalue (Rendering|Decal|SpawnDecalatLocation _decalselected DecalSize Location Rotation LifeSpan))
  (Utilities|IsValid _returnvalue
    (:Is%20Valid
      ;[1 0 0.6704] HARDCODED!!!
      (Rendering|Components|Decal|SetFadeScreenSize _returnvalue 0.0))))

(fn SpawnDecalAttached
  (params (PhysicalSurface :type EPhysicalSurface%20Enum :default "SurfaceType_Default") (DecalSize :type Vector) (AttachTo :type Scene%20Component%20Object%20Reference) (Location :type Vector) (Rotation :type Rotator) (LifeSpan :type Float%20%28double-precision%29))
  (bind _decalselected (CallFunction|GetDecalbySurface PhysicalSurface))
  (bind _returnvalue (Class|GameplayStatics|SpawnDecalAttached _decalselected DecalSize AttachTo "None" Location Rotation "KeepRelativeOffset" LifeSpan))
  (Utilities|IsValid _returnvalue
    (:Is%20Valid
      ;[1 0 0.6704] HARDCODED!!!
      (Rendering|Components|Decal|SetFadeScreenSize _returnvalue 0.0))))

(fn GetDecalbySurface
  (params (PhysicSurface :type EPhysicalSurface%20Enum :default "SurfaceType_Default"))
  (switch Utilities|FlowControl|Switch|SwitchonEPhysicalSurface PhysicSurface
    (:SurfaceType_Default
      _)
    (:SurfaceType1
      _)
    (:SurfaceType2
      (return (.OutItem (Utilities|Array|Random (Variables|Default|GetConcrete)))))
    (:SurfaceType3
      _)
    (:SurfaceType6
      _)
    (:SurfaceType7
      (return (.OutItem (Utilities|Array|Random (Variables|Default|GetMetal)))))
    (:SurfaceType8
      _)
    (:SurfaceType10
      _)
    (:SurfaceType11
      (return (.OutItem (Utilities|Array|Random (Variables|Default|GetConcrete)))))
    (:SurfaceType12
      _)
    (:SurfaceType13
      _)
    (:SurfaceType14
      (return (.OutItem (Utilities|Array|Random (Variables|Default|GetConcrete)))))
    (:SurfaceType15
      (return (.OutItem (Utilities|Array|Random (Variables|Default|GetConcrete)))))
    (:SurfaceType16
      _)
    (:SurfaceType17
      _)
    (:SurfaceType18
      _)
    (:SurfaceType19
      _)
    (:SurfaceType20
      (return (.OutItem (Utilities|Array|Random (Variables|Default|GetConcrete)))))
    (:SurfaceType21
      _)
    (:SurfaceType23
      (return (.OutItem (Utilities|Array|Random (Variables|Default|GetBulletWounds)))))
    (:SurfaceType24
      _))
  (return (.OutItem (Utilities|Array|Random (Variables|Default|GetGeneric)))))