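; REG_GameInstance is the game instance that owns and provides access to a ParticleManager actor.
; On Init it spawns the manager at the world origin and caches the reference.
; GetParticleManager returns the cached actor, or spawns and caches a replacement when the reference is no longer valid.
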(event EventInit
  (bind _returnvalue (Game|SpawnActorfromClass "/Game/REGRETSSION-Assets/Blueprints/Managers/ParticleManager.ParticleManager_C" (Math|Transform|MakeTransform "0, 0, 0") "Undefined" 0 0))
  (Variables|Default|SetParticleManager _returnvalue))

(fn GetParticleManager
  (Utilities|IsValid (Variables|Default|GetParticleManager)
    (:Is%20Valid
      (return (Variables|Default|GetParticleManager)))
    (:Is%20Not%20Valid
      (bind _returnvalue (Game|SpawnActorfromClass "/Game/REGRETSSION-Assets/Blueprints/Managers/ParticleManager.ParticleManager_C" (Math|Transform|MakeTransform "0, 0, 0") "Undefined" 0 0))
      (bind _output_get (Variables|Default|SetParticleManager _returnvalue))
      (return _output_get))))