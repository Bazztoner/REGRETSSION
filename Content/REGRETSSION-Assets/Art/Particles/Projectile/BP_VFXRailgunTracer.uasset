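; Railgun tracer VFX actor that exists for a limited lifetime in the world.
; On BeginPlay it rotates its X axis to point from its location toward TargetPosition.
; Tick accumulates elapsed time in CurrentLifeTime and destroys the actor once it reaches LifeTime.
; The graph contains no movement or hit logic, and the construction script is empty.
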(event EventBeginPlay
  (Transformation|SetActorRotation (Math|Conversions|RotationFromXVector (Math|Vector|Normalize (- (Variables|Default|GetTargetPosition) (Transformation|GetActorLocation))))))

(event EventTick
  (params (DeltaSeconds :type Float%20%28single-precision%29))
  (bind _output_get (Variables|Default|Set_currentLifeTime (+ DeltaSeconds (Variables|Default|Get_currentLifeTime))))
  (if (>= _output_get (Variables|Default|GetLifeTime))
    (Actor|DestroyActor)))

(fn ConstructionScript)