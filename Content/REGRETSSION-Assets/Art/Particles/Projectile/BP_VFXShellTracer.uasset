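; BP_VFXShellTracer is a projectile VFX actor, apparently a tracer for fired shells.
; On BeginPlay it waits a tick, then copies TracerSpeed into the ProjectileMovement component's max and initial speeds.
; Tick accumulates lifetime and destroys the actor once LifeTime expires or it comes within one unit of TargetPosition.
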(event EventBeginPlay
  (bind _projectilemovement (Variables|Default|GetProjectileMovement))
  (Utilities|FlowControl|DelayUntilNextTick)
  (bind _output_get (Variables|/Script/Engine.ProjectileMovementComponent|SetMaxSpeed _projectilemovement (Variables|Default|GetTracerSpeed)))
  (Variables|/Script/Engine.ProjectileMovementComponent|SetInitialSpeed _projectilemovement _output_get))

(event EventTick
  (params (DeltaSeconds :type Float%20%28single-precision%29))
  (bind _output_get (Variables|Default|Set_currentLifeTime (+ DeltaSeconds (Variables|Default|Get_currentLifeTime))))
  (if (or (>= _output_get (Variables|Default|GetLifeTime)) (<= (Math|Vector|Distance(Vector) (Transformation|GetActorLocation) (Variables|Default|GetTargetPosition)) 1.0))
    (Actor|DestroyActor)))

(fn ConstructionScript)