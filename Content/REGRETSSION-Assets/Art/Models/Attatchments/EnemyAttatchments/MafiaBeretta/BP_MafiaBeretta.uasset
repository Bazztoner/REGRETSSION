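; BP_MafiaBeretta is an enemy Beretta pistol attachment that supplies muzzle data for shooting and can be dropped.
; A Muzzle component provides the shot origin and transform, with its right vector serving as the firing direction.
; DropWeapon detaches the root from its parent, then switches the static mesh to physics-only collision and simulated physics.
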(fn ConstructionScript)

(fn GetShootingDirection
  (bind _muzzle (Variables|Default|GetMuzzle))
  (return (Transformation|GetWorldLocation _muzzle) (Math|Vector|GetRightVector _muzzle)))

(fn GetMuzzleTransform
  (return (Transformation|GetWorldTransform (Variables|Default|GetMuzzle))))

(fn DropWeapon
  (bind _staticmesh (Variables|Default|GetStaticMesh))
  (Transformation|DetachFromComponent (Variables|Default|GetDefaultSceneRoot) "KeepRelative" "KeepRelative" "KeepRelative" true)
  (Collision|SetCollisionEnabled _staticmesh "PhysicsOnly")
  (Physics|SetSimulatePhysics _staticmesh true))