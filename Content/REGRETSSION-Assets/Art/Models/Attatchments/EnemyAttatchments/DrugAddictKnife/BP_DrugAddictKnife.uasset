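; BP_DrugAddictKnife is the melee knife attachment for the Drug Addict enemy, dealing the owner's AttackDamage to the player on overlap.
; InitializeWeapon stores the owner, and SetHitboxState toggles both the damage flag and the hitbox collision, which starts disabled.
; A successful hit immediately disables the hitbox, so each activation damages only once.
; DropWeapon detaches the mesh and root and turns on physics simulation.
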(event EventBeginPlay
  (CallFunction|SetHitboxState false))

(event Collision|EventActorBeginOverlap
  (params (OtherActor :type Actor%20Object%20Reference))
  (bind _drugaddictowner (Variables|Default|GetDrugAddictOwner))
  (bind _asfpsreg (Utilities|Casting|CastToBP_Player OtherActor))
  (if (Variables|Default|GetCanApplyDamage)
    (Game|Damage|ApplyDamage _asfpsreg (Math|Conversions|ToFloat(Integer) (Variables|/Game/REGRETSSION-Assets/Art/Models/Characters/Enemies/DrugAddict/Blueprints/BP_DrugAddict.BP_DrugAddict_C|GetAttackDamage _drugaddictowner)) (Game|GetInstigatorController _drugaddictowner) _drugaddictowner)
    (CallFunction|SetHitboxState false)))

(fn ConstructionScript)

(fn SetHitboxState
  (params (Enabled :type Boolean))
  (bind _hitbox (Variables|Default|GetHitbox))
  (bind _output_get (Variables|Default|SetCanApplyDamage Enabled))
  (if _output_get
    (Collision|SetCollisionEnabled _hitbox "QueryAndPhysics")
    (else
      (Collision|SetCollisionEnabled _hitbox "NoCollision"))))

(fn InitializeWeapon
  (params (Owner :type BP%20Drug%20Addict%20Object%20Reference))
  (Variables|Default|SetDrugAddictOwner Owner)
  (CallFunction|SetHitboxState false))

(fn DropWeapon
  (bind _staticmesh (Variables|Default|GetStaticMesh))
  (Transformation|DetachFromComponent _staticmesh "KeepRelative" "KeepRelative" "KeepRelative" true)
  (Collision|SetCollisionEnabled _staticmesh "PhysicsOnly")
  (Physics|SetSimulatePhysics _staticmesh true))