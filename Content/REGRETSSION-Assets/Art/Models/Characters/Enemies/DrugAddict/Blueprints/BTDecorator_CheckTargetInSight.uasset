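; Behavior tree decorator for the DrugAddict enemy that tracks whether its target is in line of sight.
; On execution start it caches the AI controller and pawn.
; Each tick it tests line of sight to the controller's CurrentTarget, storing the result on the controller and in the TargetInSight blackboard key.
; While visible, it copies the blackboard Target's location into LastKnownPosition; it defines no condition check of its own.
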(event EventReceiveTickAI
  (params (OwnerController :type AI%20Controller%20Object%20Reference) (ControlledPawn :type Pawn%20Object%20Reference) (DeltaSeconds :type Float%20%28single-precision%29))
  (bind _returnvalue (Utilities|Name|MakeLiteralName "Target"))
  (bind _controller (Variables|Default|GetController))
  (bind _controller_2 (Variables|Default|GetController))
  (bind _returnvalue_2 (AI|GetBlackboard _controller))
  (bind _returnvalue_3 (AI|Components|Blackboard|GetValueasObject _returnvalue_2 _returnvalue))
  (bind _output_get (Variables|/Game/REGRETSSION-Assets/Art/Models/Characters/Enemies/DrugAddict/Blueprints/AIC_DrugAddict.AIC_DrugAddict_C|SetTargetInSight _controller_2 (Controller|LineOfSightTo _controller_2 (Variables|/Game/REGRETSSION-Assets/Art/Models/Characters/Enemies/DrugAddict/Blueprints/AIC_DrugAddict.AIC_DrugAddict_C|GetCurrentTarget _controller_2) "0, 0, 0" false)))
  (AI|Components|Blackboard|SetValueasBool (AI|GetBlackboard _controller_2) (Utilities|Name|MakeLiteralName "TargetInSight") _output_get)
  (if _output_get
    (Utilities|IsValid _returnvalue_3
      (:Is%20Valid
        (bind _asactor (Utilities|Casting|CastToActor _returnvalue_3))
        (AI|Components|Blackboard|SetValueasVector _returnvalue_2 (Utilities|Name|MakeLiteralName "LastKnownPosition") (.location (Transformation|GetActorTransform _asactor)))))))

(event EventReceiveExecutionStartAI
  (params (OwnerController :type AI%20Controller%20Object%20Reference) (ControlledPawn :type Pawn%20Object%20Reference))
  (bind _asaic_drug_addict (Utilities|Casting|CastToAIC_DrugAddict OwnerController))
  (Variables|Default|SetController _asaic_drug_addict)
  (bind _asbp_drug_addict (Utilities|Casting|CastToBP_DrugAddict ControlledPawn))
  (Variables|Default|SetDrugAddict _asbp_drug_addict))