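; Drug addict enemy character that manages health, movement states, attacks, jumps, flinching and death.
; On spawn it initializes AIC_DrugAddict, then relays flinch and death to that controller and animation changes to an Animator reference.
; Damage triggers either a chance-based flinch, which cancels attacks and starts a cooldown, or death with a randomized animation direction and disabled capsule collision.
; Attacks lock movement until they end; the polling MovementChecker is never run.
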(event Custom|FlinchHandler
  (Utilities|FlinchCooldownHandler))

(event EventBeginPlay
  (CallFunction|InitializeEnemy))

(event Collision|EventActorBeginOverlap
  (params (OtherActor :type Actor%20Object%20Reference)))

(event EventTick
  (params (DeltaSeconds :type Float%20%28single-precision%29)))

(event Game|Damage|EventAnyDamage
  (params (Damage :type Float%20%28single-precision%29) (DamageType :type Damage%20Type%20Object%20Reference) (InstigatedBy :type Controller%20Object%20Reference) (DamageCauser :type Actor%20Object%20Reference))
  (CallFunction|TakeDamage Damage))

(fn ConstructionScript)

(fn SetAnimator
  (params (Animator :type ABP%20Drug%20Addict%20Object%20Reference))
  (Variables|Default|SetAnimator Animator))

(fn OnAttackEnd
  (Variables|Default|SetisAttacking false)
  (Pawn|Components|CharacterMovement|SetMovementMode (Variables|Character|GetCharacterMovement) "MOVE_Walking" 0))

(fn OnFlinchEnd
  (bind _output_get (Variables|Default|SetisFlinching false))
  (Default|SetFlinch (Variables|Default|GetAIController) _output_get))

(fn OnJumpEnd
  (Variables|Default|SetisJumping true)
  (Character|StopJumping))

(fn OnDeathEnd)

(fn StartAttack
  (Default|StartAttack (Variables|Default|GetAnimator))
  (Variables|Default|SetisAttacking true)
  (Pawn|Components|CharacterMovement|DisableMovement (Variables|Character|GetCharacterMovement)))

(fn StartFlinch
  (bind _output_get (Variables|Default|SetisFlinching true))
  (Default|SetFlinch (Variables|Default|GetAIController) _output_get)
  (CallFunction|OnAttackEnd)
  (Variables|Default|SetflinchInCooldown true)
  (Default|StartFlinch (Variables|Default|GetAnimator))
  (CallFunction|FlinchHandler))

(fn StartJump
  (Variables|Default|SetisJumping true)
  (Character|Jump)
  (Default|StartJump (Variables|Default|GetAnimator)))

(fn StartDeath
  (params (ShotAngle :type Float%20%28single-precision%29))
  (bind _returnvalue (Math|Random|RandomInteger 3))
  ;[1 1 1] TO DO CALCULATE SHOOT ANGLE
  (Utilities|FlowControl|Sequence
    (:then_0
      (Variables|Default|SetcurrentSpeed 0.0))
    (:then_1
      (Variables|Default|SetisAttacking false)
      (Variables|Default|SetisFlinching false)
      (CallFunction|OnJumpEnd))
    (:then_2
      (Variables|Default|SetisDying true)
      (Default|OnDeath (Variables|Default|GetAIController)))
    (:then_3
      (Default|OnDeath (Variables|Default|GetAnimator) (== _returnvalue 1) (== _returnvalue 2))
      (Collision|SetCollisionEnabled (Variables|Collision|GetCapsuleComponent) "NoCollision")
      (Physics|SetEnableGravity (Variables|Collision|GetCapsuleComponent) false))))

(fn CanFlinch
  (return (not (Math|Boolean|ANDBoolean (Variables|Default|GetflinchInCooldown) (Variables|Default|GetisJumping) (Variables|Default|GetisDying)))))

(fn CheckFlinchChance
  (bind _canflinch (CallFunction|CanFlinch))
  (if _canflinch
    (if (<= (Math|Random|RandomIntegerinRange 1 100) (Variables|Default|GetFlinchChance))
      (CallFunction|StartFlinch))))

(fn TakeDamage
  (params (Dmg :type Float%20%28single-precision%29))
  (bind _output_get (Variables|Default|Set_currentHP (- (Variables|Default|Get_currentHP) Dmg)))
  (if (<= _output_get 0.0)
    (CallFunction|StartDeath 0.0)
    (else
      (CallFunction|CheckFlinchChance))))

(fn InitializeEnemy
  (Variables|Default|Set_currentHP (Math|Conversions|ToFloat(Integer) (Variables|Default|GetMaxHP)))
  (Variables|/Script/Engine.CharacterMovementComponent|SetMaxWalkSpeed (Variables|Character|GetCharacterMovement) (Variables|Default|GetWalkSpeed))
  (Variables|Default|SetSpawnedPosition (Transformation|GetWorldLocation (Variables|Collision|GetCapsuleComponent)))
  (bind _asaic_drug_addict (Utilities|Casting|CastToAIC_DrugAddict (AI|GetAIController self)))
  (bind _output_get (Variables|Default|SetAIController _asaic_drug_addict))
  (Default|InitializeAI _output_get))

(fn SetMovementState
  (params (State :type ENUM_DrugAddictStates%20Enum :default "NewEnumerator0"))
  (bind _animator (Variables|Default|GetAnimator))
  (Utilities|FlowControl|Sequence
    (:then_0
      (switch Utilities|FlowControl|Switch|SwitchonENUM_DrugAddictStates State
        (:NewEnumerator0
          (LocalVariables|Setspeed 0.0)
          (Default|SetSpeed _animator))
        (:NewEnumerator1
          (LocalVariables|Setspeed (Variables|Default|GetWalkSpeed))
          (Default|SetSpeed _animator 1))
        (:NewEnumerator2
          (LocalVariables|Setspeed (Variables|Default|GetRunSpeed))
          (Default|SetSpeed _animator 2))))
    (:then_1
      (CallFunction|SetMovementSpeed (LocalVariables|Getspeed)))
    (:then_2
      (Variables|Default|Set_currentMovementState State))))

(fn SetMovementSpeed
  (params (Speed :type Float%20%28single-precision%29))
  (Variables|/Script/Engine.CharacterMovementComponent|SetMaxWalkSpeed (Variables|Character|GetCharacterMovement) Speed))