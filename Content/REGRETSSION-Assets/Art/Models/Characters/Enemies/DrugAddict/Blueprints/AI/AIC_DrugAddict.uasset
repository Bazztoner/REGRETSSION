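; AI controller for the DrugAddict enemy that runs its behavior tree and targets the player.
; Perception updates write sight and last known position to the Blackboard, with the first sighting notifying the pawn.
; Damage from the player also reveals their position; helpers set flinch and death states, with death unpossessing the pawn.
; A looping line-of-sight polling macro is defined but not called in this controller.
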(event OnTargetPerceptionUpdated(AIPerception)
  (params (Actor :type Actor%20Object%20Reference) (Stimulus :type AI%20Stimulus%20Structure))
  (bind _bsuccessfullysensed (Utilities|Struct|BreakAIStimulus Stimulus))
  (bind _currenttarget (Variables|Default|GetCurrentTarget))
  (if (== Actor _currenttarget)
    (CallFunction|SetBlackboardValues _bsuccessfullysensed (Transformation|GetActorLocation _currenttarget))
    (if _bsuccessfullysensed
      (AI|Components|Blackboard|SetValueasBool (AI|GetBlackboard 0) (Utilities|Name|MakeLiteralName "targetLost") false)
      (Utilities|FlowControl|DoOnce false
        (:Completed
          (Default|OnTargetFound (Variables|Default|GetPawnOwner)))))))

(event Custom|InitializeAI
  (Utilities|FlowControl|Sequence
    (:then_0
      (bind _asbp_drug_addict (Utilities|Casting|CastToBP_DrugAddict (Pawn|GetControlledPawn)))
      (Variables|Default|SetPawnOwner _asbp_drug_addict))
    (:then_1
      (bind _returnvalue (Actor|GetActorOfClass "/Game/REGRETSSION-Assets/Blueprints/Player/BP_Player.BP_Player_C"))
      (bind _output_get (Variables|Default|SetPlayerActor _returnvalue))
      (Variables|Default|SetCurrentTarget _output_get))
    (:then_2
      (AI|RunBehaviorTree "/Game/REGRETSSION-Assets/Art/Models/Characters/Enemies/DrugAddict/Blueprints/AI/BT_DrugAddict.BT_DrugAddict"))
    (:then_3
      (AI|Components|Blackboard|SetValueasObject (AI|GetBlackboard 0) (Utilities|Name|MakeLiteralName "Target") (Variables|Default|GetCurrentTarget))
      (AI|Components|Blackboard|SetValueasBool (AI|GetBlackboard 0) (Utilities|Name|MakeLiteralName "targetLost") true))))

(event Custom|OnDeath
  (AI|Components|Blackboard|SetValueasBool (AI|GetBlackboard 0) (Utilities|Name|MakeLiteralName "isDead") true)
  (Pawn|UnPossess))

(fn ConstructionScript)

(fn CheckPlayerinSight
  (bind _output_get (Variables|Default|SetTargetInSight (Controller|LineOfSightTo (Variables|Default|GetCurrentTarget) "0, 0, 0" false)))
  (if _output_get
    (AI|Components|Blackboard|SetValueasBool (AI|GetBlackboard 0) (Utilities|Name|MakeLiteralName "targetLost") false)))

(fn SetBlackboardValues
  (params (In%20Sight :type Boolean) (Last%20Known%20Pos :type Vector))
  (AI|Components|Blackboard|SetValueasBool (AI|GetBlackboard 0) (Utilities|Name|MakeLiteralName "TargetInSight") In%20Sight)
  (if In%20Sight
    (AI|Components|Blackboard|SetValueasVector (AI|GetBlackboard 0) (Utilities|Name|MakeLiteralName "LastKnownPosition") Last%20Known%20Pos)
    (AI|Components|Blackboard|SetValueasBool (AI|GetBlackboard 0) (Utilities|Name|MakeLiteralName "targetLost") false)))

(fn SetFlinch
  (params (Flinching :type Boolean))
  (AI|Components|Blackboard|SetValueasBool (AI|GetBlackboard 0) (Utilities|Name|MakeLiteralName "isFlinching") Flinching))

(fn OnTakeDamage
  (params (Instigator :type Actor%20Object%20Reference))
  (bind _asbp_player (Utilities|Casting|CastToBP_Player Instigator))
  (CallFunction|SetBlackboardValues true (Transformation|GetActorLocation _asbp_player))
  (AI|Components|Blackboard|SetValueasBool (AI|GetBlackboard 0) (Utilities|Name|MakeLiteralName "targetLost") true))