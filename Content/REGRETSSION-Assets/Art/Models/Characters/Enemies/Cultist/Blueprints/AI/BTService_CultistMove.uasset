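; Behavior tree service that keeps the Cultist enemy's movement state in step with its current condition.
; On activation it caches the controlled BP_Cultist and its AIC_Cultist controller.
; Each tick it calls SetMovementState on the pawn by priority: flinching first, then target lost on the controller, then berserker or non-berserker.
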(event EventReceiveActivationAI
  (params (OwnerController :type AI%20Controller%20Object%20Reference) (ControlledPawn :type Pawn%20Object%20Reference))
  (Utilities|FlowControl|Sequence
    (:then_0
      (bind _asbp_cultist (Utilities|Casting|CastToBP_Cultist ControlledPawn))
      (Variables|Default|SetCultistPawn _asbp_cultist))
    (:then_1
      (bind _asaic_cultist (Utilities|Casting|CastToAIC_Cultist OwnerController))
      (Variables|Default|SetAIController _asaic_cultist))))

(event EventReceiveTickAI
  (params (OwnerController :type AI%20Controller%20Object%20Reference) (ControlledPawn :type Pawn%20Object%20Reference) (DeltaSeconds :type Float%20%28single-precision%29))
  (if (Variables|/Game/REGRETSSION-Assets/Art/Models/Characters/Enemies/Cultist/Blueprints/BP_Cultist.BP_Cultist_C|GetisFlinching (Variables|Default|GetCultistPawn))
    (Default|SetMovementState (Variables|Default|GetCultistPawn) "NewEnumerator0")
    (elif (Variables|/Game/REGRETSSION-Assets/Art/Models/Characters/Enemies/Cultist/Blueprints/AI/AIC_Cultist.AIC_Cultist_C|GetTargetLost (Variables|Default|GetAIController))
      (Default|SetMovementState (Variables|Default|GetCultistPawn) "NewEnumerator1")
      (elif (Variables|/Game/REGRETSSION-Assets/Art/Models/Characters/Enemies/Cultist/Blueprints/BP_Cultist.BP_Cultist_C|GetisBerserker (Variables|Default|GetCultistPawn))
        (Default|SetMovementState (Variables|Default|GetCultistPawn) "NewEnumerator3")
        (else
          (Default|SetMovementState (Variables|Default|GetCultistPawn) "NewEnumerator2"))))))