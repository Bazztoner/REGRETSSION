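; AI controller for the Cultist enemy that runs BT_Cultist and targets the player.
; InitializeAI caches the pawn, binds to player death and seeds the blackboard.
; Perception updates and player damage feed sight, last known position and target-lost keys, with first sighting notifying the pawn once.
; Setters mirror flinch, berserk and dagger-throw states to the blackboard; player death clears the target, and its own death unpossesses.
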(event OnTargetPerceptionUpdated(AIPerception)
  (params (Actor :type Actor%20Object%20Reference) (Stimulus :type AI%20Stimulus%20Structure))
  (bind _currenttarget (Variables|Default|GetCurrentTarget))
  (if (== Actor _currenttarget)
    (bind _output_get (Variables|Default|SetTargetInSight (.bSuccessfullySensed (Utilities|Struct|BreakAIStimulus Stimulus))))
    (CallFunction|SetBlackboardValues _output_get (Transformation|GetActorLocation _currenttarget))
    (if _output_get
      (AI|Components|Blackboard|SetValueasBool (AI|GetBlackboard 0) (Utilities|Name|MakeLiteralName "TargetLost") false)
      (CallFunction|SetTargetLost false)
      (Utilities|FlowControl|DoOnce false
        (:Completed
          (Default|OnTargetFound (Variables|Default|GetPawnOwner))
          (AI|Components|Blackboard|SetValueasBool (AI|GetBlackboard 0) (Utilities|Name|MakeLiteralName "PlayerFirstSight") true))))))

(event Custom|InitializeAI
  (Utilities|FlowControl|Sequence
    (:then_0
      (bind _asbp_cultist (Utilities|Casting|CastToBP_Cultist (Pawn|GetControlledPawn)))
      (Variables|Default|SetPawnOwner _asbp_cultist))
    (:then_1
      (bind _returnvalue (Actor|GetActorOfClass "/Game/REGRETSSION-Assets/Blueprints/Player/BP_Player.BP_Player_C"))
      (bind _output_get (Variables|Default|SetPlayerActor _returnvalue))
      (Variables|Default|SetCurrentTarget _output_get)
      (EventDispatchers|BindEventtoOnPlayerDeath _output_get (delegate Custom|OnPlayerDeath)))
    (:then_2
      (AI|RunBehaviorTree "/Game/REGRETSSION-Assets/Art/Models/Characters/Enemies/Cultist/Blueprints/AI/BT_Cultist.BT_Cultist"))
    (:then_3
      (AI|Components|Blackboard|SetValueasObject (AI|GetBlackboard 0) (Utilities|Name|MakeLiteralName "Target") (Variables|Default|GetCurrentTarget))
      (AI|Components|Blackboard|SetValueasBool (AI|GetBlackboard 0) (Utilities|Name|MakeLiteralName "targetLost") true))))

(event Custom|OnDeath
  (AI|Components|Blackboard|SetValueasBool (AI|GetBlackboard 0) (Utilities|Name|MakeLiteralName "IsDead") true)
  (Pawn|UnPossess))

(event Custom|OnPlayerDeath
  (AI|Components|Blackboard|SetValueasObject (AI|GetBlackboard 0) (Utilities|Name|MakeLiteralName "Target") 0)
  (CallFunction|SetTargetLost true))

(fn ConstructionScript)

(fn SetBlackboardValues
  (params (In%20Sight :type Boolean) (Last%20Known%20Pos :type Vector))
  (AI|Components|Blackboard|SetValueasBool (AI|GetBlackboard 0) (Utilities|Name|MakeLiteralName "TargetInSight") In%20Sight)
  (if In%20Sight
    (AI|Components|Blackboard|SetValueasVector (AI|GetBlackboard 0) (Utilities|Name|MakeLiteralName "LastKnownPosition") Last%20Known%20Pos)
    (CallFunction|SetTargetLost false)))

(fn OnTakeDamage
  (params (Instigator :type Actor%20Object%20Reference))
  (bind _asbp_player (Utilities|Casting|CastToBP_Player Instigator))
  (CallFunction|SetBlackboardValues true (Transformation|GetActorLocation _asbp_player)))

(fn SetDaggerThrowAttackinCooldown
  (params (InCooldown :type Boolean))
  (bind _output_get (Variables|Default|SetDaggerThrowInCooldown InCooldown))
  (AI|Components|Blackboard|SetValueasBool (Variables|Default|GetBlackboard) (Utilities|Name|MakeLiteralName "DaggerThrowInCooldown") _output_get))

(fn SetFlinch
  (params (State :type Boolean))
  (bind _output_get (Variables|Default|SetisFlinching State))
  (AI|Components|Blackboard|SetValueasBool (Variables|Default|GetBlackboard) (Utilities|Name|MakeLiteralName "IsFlinching") _output_get))

(fn SetBerserkAttack
  (params (IsBerserk :type Boolean))
  (bind _output_get (Variables|Default|SetisBerserkAttack IsBerserk))
  (AI|Components|Blackboard|SetValueasBool (Variables|Default|GetBlackboard) (Utilities|Name|MakeLiteralName "IsBerserk") _output_get))

(fn InitializePlayerTarget
  (bind _returnvalue (Actor|GetActorOfClass "/Game/REGRETSSION-Assets/Blueprints/Player/BP_Player.BP_Player_C"))
  (bind _output_get (Variables|Default|SetPlayerActor _returnvalue))
  (Variables|Default|SetCurrentTarget _output_get))

(fn SetTargetLost
  (params (Lost :type Boolean))
  (bind _output_get (Variables|Default|SetTargetLost Lost))
  (AI|Components|Blackboard|SetValueasBool (Variables|Default|GetBlackboard) (Utilities|Name|MakeLiteralName "TargetLost") _output_get))

(fn SetDaggerThrowAttack
  (params (ThrowingDagger :type Boolean))
  (bind _output_get (Variables|Default|SetIsThrowingDagger ThrowingDagger))
  (AI|Components|Blackboard|SetValueasBool (Variables|Default|GetBlackboard) (Utilities|Name|MakeLiteralName "IsThrowingDagger") _output_get))