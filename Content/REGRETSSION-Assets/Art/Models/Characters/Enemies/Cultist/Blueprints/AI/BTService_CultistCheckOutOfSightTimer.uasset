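; Behavior tree service for the Cultist enemy AI that decides when it has lost its target.
; On activation it caches the controlled Cultist pawn and AI controller and reads the controller's out-of-sight timeout.
; Each tick it resets a timer while the target is in sight, otherwise accumulates delta time and flags the target as lost on the controller once the timeout is reached.
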(event EventReceiveActivationAI
  (params (OwnerController :type AI%20Controller%20Object%20Reference) (ControlledPawn :type Pawn%20Object%20Reference))
  (Utilities|FlowControl|Sequence
    (:then_0
      (bind _asbp_cultist (Utilities|Casting|CastToBP_Cultist ControlledPawn))
      (Variables|Default|SetCultistPawn _asbp_cultist))
    (:then_1
      (bind _asaic_cultist (Utilities|Casting|CastToAIC_Cultist OwnerController))
      (bind _output_get (Variables|Default|SetAIController _asaic_cultist))
      (Variables|Default|SetOutOfSightTimeout (Variables|/Game/REGRETSSION-Assets/Art/Models/Characters/Enemies/Cultist/Blueprints/AI/AIC_Cultist.AIC_Cultist_C|GetOutOfSightTimeout _output_get)))))

(event EventReceiveTickAI
  (params (OwnerController :type AI%20Controller%20Object%20Reference) (ControlledPawn :type Pawn%20Object%20Reference) (DeltaSeconds :type Float%20%28single-precision%29))
  (if (Variables|/Game/REGRETSSION-Assets/Art/Models/Characters/Enemies/Cultist/Blueprints/AI/AIC_Cultist.AIC_Cultist_C|GetTargetInSight (Variables|Default|GetAIController))
    (Variables|Default|Set_currentOutOfSightTimer 0.0)
    (else
      (bind _output_get (Variables|Default|Set_currentOutOfSightTimer (+ DeltaSeconds (Variables|Default|Get_currentOutOfSightTimer))))
      (if (>= _output_get (Variables|Default|GetOutOfSightTimeout))
        (Default|SetTargetLost (Variables|Default|GetAIController) true)))))