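; Cultist enemy character with two attacks: a timed berserk dagger rush and a dagger thrown at the player.
; Damage either kills it, dropping both daggers, or triggers random flinch and berserk rolls, with a FlipFlop alternating which gets priority.
; State flags gate each action, while delay-based handlers run cooldowns and tick berserk duration.
; It drives its animator, movement speed and AIC_Cultist controller, passing flinch, throw and death states.
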(event Custom|FlinchHandler
  (Utilities|FlinchCooldownHandler))

(event Custom|OnBerserkAttack
  (Utilities|BerserkAttackHandler))

(event Custom|OnBerserkAttackEnd
  (Utilities|BerserkAttackCooldownHandler))

(event Custom|OnDaggerThrowEnd
  (Utilities|DaggerThrowCooldownHandler))

(event EventBeginPlay
  (CallFunction|InitializeEnemy))

(event Game|Damage|EventPointDamage
  (params (Damage :type Float%20%28single-precision%29) (DamageType :type Damage%20Type%20Object%20Reference) (HitLocation :type Vector :default "0, 0, 0") (HitNormal :type Vector :default "0, 0, 0") (HitComponent :type Primitive%20Component%20Object%20Reference) (BoneName :type Name :default "None") (ShotFromDirection :type Vector :default "0, 0, 0") (InstigatedBy :type Controller%20Object%20Reference) (DamageCauser :type Actor%20Object%20Reference) (HitInfo :type Hit%20Result%20Structure%20%28by%20ref%29))
  (CallFunction|TakeDamagePoint Damage HitLocation HitNormal BoneName))

(event Game|Damage|EventRadialDamage
  (params (DamageReceived :type Float%20%28single-precision%29) (DamageType :type Damage%20Type%20Object%20Reference) (Origin :type Vector :default "0, 0, 0") (HitInfo :type Hit%20Result%20Structure%20%28by%20ref%29) (InstigatedBy :type Controller%20Object%20Reference) (DamageCauser :type Actor%20Object%20Reference))
  (CallFunction|TakeDamageGeneric DamageReceived))

(fn ConstructionScript)

(fn SetAnimator
  (params (Animator :type ABP%20Cultist%20Object%20Reference))
  (Variables|Default|SetAnimator Animator))

(fn OnAttackEnd
  (Variables|Default|SetisAttacking false)
  (Pawn|Components|CharacterMovement|SetMovementMode (Variables|Character|GetCharacterMovement) "MOVE_Walking" 0)
  (CallFunction|SetWeaponHitboxState false))

(fn OnFlinchEnd
  (bind _output_get (Variables|Default|SetisFlinching false))
  ;[1 1 1] AIC set flinch
  (Default|SetFlinch (Variables|Default|GetAIController) _output_get)
  (CallFunction|FlinchHandler))

(fn OnJumpEnd
  (Variables|Default|SetisJumping true)
  (Character|StopJumping))

(fn OnDeathEnd)

(fn StartAttack
  (params (Melee :type Boolean))
  (Variables|Default|SetisAttacking true)
  (Default|StartAttack (Variables|Default|GetAnimator) Melee)
  (if Melee
    (CallFunction|StartBerserkAttack)
    (else
      (CallFunction|StartDaggerThrowAttack))))

(fn StartBerserkAttack
  (bind _output_get (Variables|Default|SetberserkAttackInCooldown true))
  (Variables|Default|SetisBerserker _output_get)
  (Default|StartAttack (Variables|Default|GetAnimator) true)
  (CallFunction|PlaySound (Utilities|Struct|BreakSTRUCT_CultistSound (Variables|Default|GetSoundList)) true true)
  (CallFunction|OnBerserkAttack)
  (CallFunction|SetMovementState "NewEnumerator3"))

(fn StartDaggerThrowAttack
  (bind _aicontroller (Variables|Default|GetAIController))
  (Default|StartAttack (Variables|Default|GetAnimator) false)
  (Variables|Default|SetdaggerThrowInCooldown true)
  (Pawn|Components|CharacterMovement|DisableMovement (Variables|Character|GetCharacterMovement))
  (Default|SetDaggerThrowAttackinCooldown _aicontroller true)
  (Default|SetDaggerThrowAttack _aicontroller true))

(fn StartFlinch
  (bind _output_get (Variables|Default|SetisFlinching true))
  (Default|SetFlinch (Variables|Default|GetAIController) _output_get)
  (CallFunction|OnAttackEnd)
  (Variables|Default|SetflinchInCooldown true)
  (Default|StartFlinch (Variables|Default|GetAnimator))
  (CallFunction|FlinchHandler)
  (CallFunction|SetMovementState "NewEnumerator0"))

(fn StartJump
  (Variables|Default|SetisJumping true)
  (Character|Jump)
  (Default|StartJump (Variables|Default|GetAnimator)))

(fn CanFlinch
  (return (not (Math|Boolean|ORBoolean (Variables|Default|GetflinchInCooldown) (Variables|Default|GetisJumping) (Variables|Default|GetisDying) (Variables|Default|GetisAttacking)))))

(fn CheckFlinchChance
  (bind _canflinch (CallFunction|CanFlinch))
  (if _canflinch
    (if (<= (Math|Random|RandomIntegerinRange 1 100) (Variables|Default|GetFlinchChance))
      (CallFunction|StartFlinch))))

(fn TakeDamage
  (params (Dmg :type Float%20%28double-precision%29))
  (bind _output_get (Variables|Default|Set_currentHP (- (Variables|Default|Get_currentHP) Dmg)))
  (if (not (<= _output_get 0.0))
    (CallFunction|CheckonHitBehaviour)))

(fn SetMovementState
  (params (State :type ENUM_CultistStates%20Enum :default "NewEnumerator0"))
  (bind _animator (Variables|Default|GetAnimator))
  (Utilities|FlowControl|Sequence
    (:then_0
      (switch Utilities|FlowControl|Switch|SwitchonENUM_CultistStates State
        (:NewEnumerator0
          (LocalVariables|Setspeed 0.0)
          (Default|SetSpeed _animator))
        (:NewEnumerator1
          (LocalVariables|Setspeed (Variables|Default|GetWalkSpeed))
          (Default|SetSpeed _animator 1))
        (:NewEnumerator2
          (LocalVariables|Setspeed (Variables|Default|GetRunSpeed))
          (Default|SetSpeed _animator 2))
        (:NewEnumerator3
          (LocalVariables|Setspeed (Variables|Default|GetBerserkSpeed))
          (Default|SetSpeed _animator))))
    (:then_1
      (CallFunction|SetMovementSpeed (LocalVariables|Getspeed)))
    (:then_2
      (Variables|Default|Set_currentMovementState State))))

(fn SetMovementSpeed
  (params (Speed :type Float%20%28double-precision%29))
  (Variables|/Script/Engine.CharacterMovementComponent|SetMaxWalkSpeed (Variables|Character|GetCharacterMovement) Speed))

(fn SetWeaponHitboxState
  (params (Enabled :type Boolean))
  (Default|SetHitboxState (Variables|Default|GetWeaponBerserkDagger) Enabled))

(fn CheckonHitBehaviour
  (Utilities|FlowControl|FlipFlop
    (:A
      ;[0.6832 0.95 1] V1 Flinch more priority
      (CallFunction|CheckFlinchChance)
      (if (not (Variables|Default|GetisFlinching))
        (CallFunction|CheckBerserkAttackChance)))
    (:B
      ;[1 0.8521 0.5492] V2 Berserk More Priority
      (CallFunction|CheckBerserkAttackChance)
      (if (not (Variables|Default|GetisAttacking))
        (CallFunction|CheckFlinchChance)))))

(fn CheckBerserkAttackChance
  (bind _berserkattackavailable (CallFunction|CanAttackBerserk))
  (if _berserkattackavailable
    (if (<= (Math|Random|RandomIntegerinRange 1 100) (Variables|Default|GetBerserkAttackChance))
      (CallFunction|StartAttack true))))

(fn CanAttackBerserk
  (return (not (Math|Boolean|ORBoolean (Variables|Default|GetberserkAttackInCooldown) (Variables|Default|GetisJumping) (Variables|Default|GetisDying) (Variables|Default|GetisAttacking) (Variables|Default|GetisFlinching)))))

(fn CanAttackThrowDagger
  (return (not (Math|Boolean|ORBoolean (Variables|Default|GetisAttacking) (Variables|Default|GetisBerserker) (Variables|Default|GetisFlinching) (Variables|Default|GetisDying) (Variables|Default|GetdaggerThrowInCooldown)))))

(fn CheckDaggerAttackChance
  (bind _canthrowdagger (CallFunction|CanAttackThrowDagger))
  (if _canthrowdagger
    (if (<= (Math|Random|RandomIntegerinRange 1 100) (Variables|Default|GetDaggerThrowChance))
      (CallFunction|StartAttack false))))

(fn CheckBerserkAttackContinued
  (bind _output_get (Variables|Default|Set_currentBerserkDuration (+ (Variables|Default|Get_currentBerserkDuration) 0.1)))
  (if (< _output_get (Variables|Default|GetbersekAttackDuration))
    (CallFunction|OnBerserkAttack)
    (else
      (CallFunction|OnBerserkAttackEnd)
      (Variables|Default|SetisBerserker false)
      (Default|OnAttackEnd (Variables|Default|GetAnimator)))))

(fn SpawnDaggerProjectile
  (bind _self self)
  (bind _returnvalue (Game|SpawnActorfromClass (Variables|Default|GetDaggerProjectileClass) (Math|Transform|MakeTransform (.location (Transformation|GetWorldTransform (Variables|Default|GetThrowingDaggerSpawn))) (Math|Conversions|RotationFromXVector (Math|Vector|Normalize (- (Transformation|GetWorldLocation (Variables|/Script/Engine.Character|GetCapsuleComponent (Variables|Default|GetPlayer))) (Transformation|GetWorldLocation (Variables|Default|GetThrowingDaggerSpawn))))) "1.000000,1.000000,1.000000") "AdjustIfPossibleButAlwaysSpawn" "SelectDefaultAtRuntime" _self _self))
  (if (Utilities|IsValid _returnvalue)
    (Default|InitializeProjectile _returnvalue (Math|Conversions|ToFloat(Integer) (Variables|Default|GetDaggerThrowDamage)) "NewEnumerator6")))

(fn OnAttackDaggerThrowEnd
  (CallFunction|OnDaggerThrowEnd)
  (CallFunction|SetMovementState "NewEnumerator2")
  (Default|SetDaggerThrowAttack (Variables|Default|GetAIController) false))

(fn ForcedFlinchEnd
  (Default|OnFlinchEnd (Variables|Default|GetAnimator)))

(fn PlaySound
  (params (Sound :type Sound%20Base%20Object%20Reference) (CancelPreviousSound :type Boolean) (Cancellable :type Boolean))
  (|CallParentFunction Sound CancelPreviousSound Cancellable))

(fn OnTargetFound
  (|CallParentFunction)
  (if (not (Variables|Default|GetisDying))
    (CallFunction|PlaySound (Utilities|Struct|BreakSTRUCT_CultistSound (Variables|Default|GetSoundList)) false true)))

(fn StartDeath
  (params (ImpactPoint :type Vector :default "0, 0, 0") (KillingDamage :type Float%20%28double-precision%29))
  (bind _soundlist (Variables|Default|GetSoundList))
  (bind (_death _gibbing) (Utilities|Struct|BreakSTRUCT_CultistSound _soundlist))
  (|CallParentFunction ImpactPoint KillingDamage)
  (Utilities|FlowControl|Sequence
    (:then_0
      (Variables|Default|SetcurrentSpeed 0.0))
    (:then_1
      (Variables|Default|SetisAttacking false)
      (Variables|Default|SetisFlinching false)
      (CallFunction|OnJumpEnd))
    (:then_2
      (Variables|Default|SetisDying true)
      (Default|OnDeath (Variables|Default|GetAIController))
      (CallFunction|OnAttackEnd))
    (:then_3
      (Default|StartDeath (Variables|Default|GetAnimator))
      (Collision|SetCollisionEnabled (Variables|Default|GetCapsuleComponent) "NoCollision")
      (Physics|SetEnableGravity (Variables|Default|GetCapsuleComponent) false)
      (Utilities|FlowControl|Sequence
        (:then_0
          (switch Utilities|FlowControl|Switch|SwitchonENUM_EnemyDeathStates (Variables|Default|GetDeathType)
            (:NewEnumerator0
              (LocalVariables|SetSoundToPlay _death))
            (:NewEnumerator1
              (LocalVariables|SetSoundToPlay _gibbing :!label _label))
            (:NewEnumerator2
              (goto _label))))
        (:then_1
          (CallFunction|PlaySound (LocalVariables|GetSoundToPlay) true false)
          (CallFunction|DropWeapon))))))

(fn InitializeEnemy
  (|CallParentFunction)
  (Variables|/Script/Engine.CharacterMovementComponent|SetMaxWalkSpeed (Variables|Character|GetCharacterMovement) (Variables|Default|GetWalkSpeed))
  (bind _asbp_cultist_dagger (Utilities|Casting|CastToBP_CultistDagger (Variables|/Script/Engine.ChildActorComponent|GetChildActor (Variables|Default|GetBerserkDagger))))
  (bind _output_get (Variables|Default|SetWeaponBerserkDagger _asbp_cultist_dagger))
  (Default|InitializeWeapon _output_get self)
  (bind _asaic_cultist (Utilities|Casting|CastToAIC_Cultist (AI|GetAIController self)))
  (bind _output_get_2 (Variables|Default|SetAIController _asaic_cultist))
  (Default|InitializeAI _output_get_2))

(fn TakeDamageGeneric
  (params (Dmg :type Float%20%28double-precision%29))
  (|CallParentFunction Dmg)
  (if (<= (Variables|Default|Get_currentHP) 0.0)
    (CallFunction|StartDeath "0, 0, 0" Dmg)
    (else
      (CallFunction|CheckonHitBehaviour))))

(fn TakeDamagePoint
  (params (Dmg :type Float%20%28double-precision%29) (HitLoc :type Vector :default "0, 0, 0") (HitNormal :type Vector :default "0, 0, 0") (HitBone :type Name :default "None"))
  (|CallParentFunction Dmg HitLoc HitNormal HitBone)
  (if (<= (Variables|Default|Get_currentHP) 0.0)
    (CallFunction|StartDeath HitLoc Dmg)
    (else
      (CallFunction|CheckonHitBehaviour))))

(fn DropWeapon
  (bind _throwingdagger (Variables|Default|GetThrowingDagger))
  (Utilities|FlowControl|Sequence
    (:then_0
      (bind _asbp_cultist_dagger (Utilities|Casting|CastToBP_CultistDagger (Variables|/Script/Engine.ChildActorComponent|GetChildActor (Variables|Default|GetBerserkDagger))))
      (Default|DropWeapon _asbp_cultist_dagger))
    (:then_1
      (Transformation|DetachFromComponent _throwingdagger "KeepRelative" "KeepRelative" "KeepRelative" true)
      (Collision|SetCollisionEnabled _throwingdagger "PhysicsOnly")
      (Physics|SetSimulatePhysics _throwingdagger true))))