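; AI controller for Mafia enemies that hunts the player, running either the standard or sniper behavior tree based on the pawn's variant.
; Perception updates, player-inflicted damage and a repeating sight check write visibility and last known position to the blackboard.
; The first sighting notifies the pawn once, and player death clears the target.
; It also mirrors attack cooldown and roll state to the blackboard, and unpossesses on its own death.
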(event OnTargetPerceptionUpdated(AIPerception)
  (params (Actor :type Actor%20Object%20Reference) (Stimulus :type AI%20Stimulus%20Structure))
  (bind _bsuccessfullysensed (Utilities|Struct|BreakAIStimulus Stimulus))
  (bind _currenttarget (Variables|Default|GetCurrentTarget))
  (if (== Actor _currenttarget)
    (CallFunction|SetBlackboardValues _bsuccessfullysensed (Transformation|GetActorLocation _currenttarget))
    (if _bsuccessfullysensed
      (AI|Components|Blackboard|SetValueasBool (AI|GetBlackboard 0) (Utilities|Name|MakeLiteralName "targetLost") false)
      (Utilities|FlowControl|DoOnce false
        (:Completed
          (Default|OnTargetFound (Variables|Default|GetPawnOwner)))))))

(event Custom|InitializeAI
  (Utilities|FlowControl|Sequence
    (:then_0
      (bind _asbp_mafia (Utilities|Casting|CastToBP_Mafia (Pawn|GetControlledPawn)))
      (bind _output_get (Variables|Default|SetPawnOwner _asbp_mafia))
      (Variables|Default|SetsniperVariant (Variables|/Game/REGRETSSION-Assets/Art/Models/Characters/Enemies/Mafia/Blueprints/BP_Mafia.BP_Mafia_C|GetsniperVariant _output_get)))
    (:then_1
      (bind _returnvalue (Actor|GetActorOfClass "/Game/REGRETSSION-Assets/Blueprints/Player/BP_Player.BP_Player_C"))
      (bind _output_get_2 (Variables|Default|SetPlayerActor _returnvalue))
      (Variables|Default|SetCurrentTarget _output_get_2)
      (EventDispatchers|BindEventtoOnPlayerDeath _output_get_2 (delegate Custom|OnPlayerDeath)))
    (:then_2
      (if (Variables|Default|GetsniperVariant)
        (AI|RunBehaviorTree "/Game/REGRETSSION-Assets/Art/Models/Characters/Enemies/Mafia/Blueprints/AI/BT_MafiaSniper.BT_MafiaSniper")
        (else
          (AI|RunBehaviorTree "/Game/REGRETSSION-Assets/Art/Models/Characters/Enemies/Mafia/Blueprints/AI/BT_Mafia.BT_Mafia"))))
    (:then_3
      (AI|Components|Blackboard|SetValueasObject (AI|GetBlackboard 0) (Utilities|Name|MakeLiteralName "Target") (Variables|Default|GetCurrentTarget))
      (AI|Components|Blackboard|SetValueasBool (AI|GetBlackboard 0) (Utilities|Name|MakeLiteralName "targetLost") true))))

(event Custom|OnDeath
  (AI|Components|Blackboard|SetValueasBool (AI|GetBlackboard 0) (Utilities|Name|MakeLiteralName "isDead") true)
  (Pawn|UnPossess))

(event Custom|OnPlayerDeath
  (AI|Components|Blackboard|SetValueasObject (AI|GetBlackboard 0) (Utilities|Name|MakeLiteralName "Target") 0)
  (AI|Components|Blackboard|SetValueasBool (AI|GetBlackboard 0) (Utilities|Name|MakeLiteralName "targetLost") true))

(fn ConstructionScript)

(fn SetBlackboardValues
  (params (In%20Sight :type Boolean) (Last%20Known%20Pos :type Vector))
  (AI|Components|Blackboard|SetValueasBool (AI|GetBlackboard 0) (Utilities|Name|MakeLiteralName "TargetInSight") In%20Sight)
  (if In%20Sight
    (AI|Components|Blackboard|SetValueasVector (AI|GetBlackboard 0) (Utilities|Name|MakeLiteralName "LastKnownPosition") Last%20Known%20Pos)
    (AI|Components|Blackboard|SetValueasBool (AI|GetBlackboard 0) (Utilities|Name|MakeLiteralName "targetLost") false)))

(fn OnTakeDamage
  (params (Instigator :type Actor%20Object%20Reference))
  (bind _asbp_player (Utilities|Casting|CastToBP_Player Instigator))
  (CallFunction|SetBlackboardValues true (Transformation|GetActorLocation _asbp_player))
  (AI|Components|Blackboard|SetValueasBool (AI|GetBlackboard 0) (Utilities|Name|MakeLiteralName "targetLost") false))

(fn SetAttackinCooldown
  (params (InCooldown :type Boolean))
  (bind _output_get (Variables|Default|SetAttackInCooldown InCooldown))
  (AI|Components|Blackboard|SetValueasBool (Variables|Default|GetBlackboard) (Utilities|Name|MakeLiteralName "AttackInCooldown") _output_get))

(fn SetRoll
  (params (State :type Boolean))
  (bind _output_get (Variables|Default|SetisRolling State))
  (AI|Components|Blackboard|SetValueasBool (Variables|Default|GetBlackboard) (Utilities|Name|MakeLiteralName "isRolling") _output_get))