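; AI controller for Mafia enemies that runs their behavior tree and targets the player (FPSReg).
; Initialization caches the pawn and player, then seeds the Blackboard.
; Perception updates and damage from the player write sight and last known position, with first detection notifying the pawn; death and flinch also set Blackboard flags.
; A PeriodicPlayerInSight macro offers looping line-of-sight checks on a retriggerable delay, but no graph here calls it.
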(event OnTargetPerceptionUpdated(AIPerception)
  (params (Actor :type Actor%20Object%20Reference) (Stimulus :type AI%20Stimulus%20Structure))
  (bind _bsuccessfullysensed (Utilities|Struct|BreakAIStimulus Stimulus))
  (bind _currenttarget (Variables|Default|GetCurrentTarget))
  (if (== Actor _currenttarget)
    (CallFunction|SetBlackboardValues _bsuccessfullysensed (Transformation|GetActorLocation _currenttarget))
    (if _bsuccessfullysensed
      (AI|Components|Blackboard|SetValueasBool (AI|GetBlackboard 0) (Utilities|Name|MakeLiteralName "targetLost") false)
      (Utilities|FlowControl|DoOnce false
        (:Completed
          (Default|OnTargetFound (Variables|Default|GetPawnOwner)))))))

(event Custom|InitializeAI
  (Utilities|FlowControl|Sequence
    (:then_0
      (bind _asbp_mafia (Utilities|Casting|CastToBP_Mafia (Pawn|GetControlledPawn)))
      (Variables|Default|SetPawnOwner _asbp_mafia))
    (:then_1
      (bind _returnvalue (Actor|GetActorOfClass "/Game/REGRETSSION-Assets/Blueprints/Player/FPSReg.FPSReg_C"))
      (bind _output_get (Variables|Default|SetPlayerActor _returnvalue))
      (Variables|Default|SetCurrentTarget _output_get))
    (:then_2
      (AI|RunBehaviorTree "/Game/REGRETSSION-Assets/Art/Models/Characters/Enemies/Mafia/Blueprints/BT_Mafia.BT_Mafia"))
    (:then_3
      (AI|Components|Blackboard|SetValueasObject (AI|GetBlackboard 0) (Utilities|Name|MakeLiteralName "Target") (Variables|Default|GetCurrentTarget))
      (AI|Components|Blackboard|SetValueasBool (AI|GetBlackboard 0) (Utilities|Name|MakeLiteralName "targetLost") true))))

(event Custom|OnDeath
  (AI|Components|Blackboard|SetValueasBool (AI|GetBlackboard 0) (Utilities|Name|MakeLiteralName "isDead") true))

(fn ConstructionScript)

(fn CheckPlayerinSight
  (Variables|Default|SetTargetInSight (Controller|LineOfSightTo (Variables|Default|GetCurrentTarget) "0, 0, 0" false)))

(fn SetBlackboardValues
  (params (In%20Sight :type Boolean) (Last%20Known%20Pos :type Vector))
  (AI|Components|Blackboard|SetValueasBool (AI|GetBlackboard 0) (Utilities|Name|MakeLiteralName "TargetInSight") In%20Sight)
  (if In%20Sight
    (AI|Components|Blackboard|SetValueasVector (AI|GetBlackboard 0) (Utilities|Name|MakeLiteralName "LastKnownPosition") Last%20Known%20Pos)))

(fn SetFlinch
  (params (Flinching :type Boolean))
  (AI|Components|Blackboard|SetValueasBool (AI|GetBlackboard 0) (Utilities|Name|MakeLiteralName "isFlinching") Flinching))

(fn OnTakeDamage
  (params (Instigator :type Actor%20Object%20Reference))
  (bind _asfpsreg (Utilities|Casting|CastToFPSReg Instigator))
  (CallFunction|SetBlackboardValues true (Transformation|GetActorLocation _asfpsreg)))