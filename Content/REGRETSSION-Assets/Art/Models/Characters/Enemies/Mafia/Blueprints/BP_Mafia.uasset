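; Mafia gunman enemy character that shoots at the player with a Beretta child actor and may dodge-roll when damaged.
; It extends a parent enemy, linking the AIC_Mafia controller and an animator through attack, roll and movement states with cooldowns.
; OnAim stores the player's camera position, and OnShoot fires a hitscan bullet from the muzzle toward it.
; Death notifies AI and animator, disables collision, picks death or gib audio, and drops the weapon.
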(event Custom|AttackCooldownStart
  (Utilities|AttackCooldownHandler))

(event Custom|RollCooldownStart
  (Utilities|RollCooldownHandler))

(event EventBeginPlay
  (CallFunction|InitializeEnemy))

(event Collision|EventActorBeginOverlap
  (params (OtherActor :type Actor%20Object%20Reference)))

(event EventTick
  (params (DeltaSeconds :type Float%20%28single-precision%29)))

(event Game|Damage|EventPointDamage
  (params (Damage :type Float%20%28single-precision%29) (DamageType :type Damage%20Type%20Object%20Reference) (HitLocation :type Vector :default "0, 0, 0") (HitNormal :type Vector :default "0, 0, 0") (HitComponent :type Primitive%20Component%20Object%20Reference) (BoneName :type Name :default "None") (ShotFromDirection :type Vector :default "0, 0, 0") (InstigatedBy :type Controller%20Object%20Reference) (DamageCauser :type Actor%20Object%20Reference) (HitInfo :type Hit%20Result%20Structure%20%28by%20ref%29))
  (CallFunction|TakeDamagePoint Damage HitLocation HitNormal BoneName))

(event Game|Damage|EventRadialDamage
  (params (DamageReceived :type Float%20%28single-precision%29) (DamageType :type Damage%20Type%20Object%20Reference) (Origin :type Vector :default "0, 0, 0") (HitInfo :type Hit%20Result%20Structure%20%28by%20ref%29) (InstigatedBy :type Controller%20Object%20Reference) (DamageCauser :type Actor%20Object%20Reference))
  (CallFunction|TakeDamageGeneric DamageReceived))

(fn ConstructionScript)

(fn SetAnimator
  (params (Animator :type ABP%20Mafia%20Object%20Reference))
  (Variables|Default|SetAnimator Animator))

(fn OnAttackEnd
  (params (ForcedEnd :type Boolean))
  (Variables|Default|SetisAttacking false)
  (Pawn|Components|CharacterMovement|SetMovementMode (Variables|Character|GetCharacterMovement) "MOVE_Walking" 0)
  (if ForcedEnd
    (CallFunction|AttackCooldownStart)))

(fn OnJumpEnd)

(fn OnRollEnd
  (bind _output_get (Variables|Default|SetisRolling false))
  (Default|SetRoll (Variables|Default|GetAIController) _output_get)
  (CallFunction|RollCooldownStart)
  (CallFunction|ForceGroundedRotation))

(fn OnDeathEnd)

(fn OnShoot
  (CallFunction|SpawnProjectile)
  (CallFunction|PlaySound (Utilities|Struct|BreakSTRUCT_MafiaSound (Variables|Default|GetSound%20List)) false false))

(fn OnAim
  (Variables|Default|SetPlayerPos (Transformation|GetWorldLocation (Variables|/Game/REGRETSSION-Assets/Blueprints/Player/BP_Player.BP_Player_C|GetFirstPersonCamera (Variables|Default|GetPlayer)))))

(fn StartAttack
  (if (not (Math|Boolean|ANDBoolean (Variables|Default|GetisAttacking) (Variables|Default|Get_attackInCooldown) (Variables|Default|GetisRolling)))
    (Default|StartAttack (Variables|Default|GetAnimator))
    (Variables|Default|SetisAttacking true)
    (Pawn|Components|CharacterMovement|DisableMovement (Variables|Character|GetCharacterMovement))))

(fn StartJump)

(fn StartRoll
  (Variables|Default|SetisRolling true)
  (CallFunction|OnAttackEnd true)
  (Default|StartRoll (Variables|Default|GetAnimator) (Math|Random|RandomInteger 4))
  (Default|SetRoll (Variables|Default|GetAIController) true))

(fn CanRoll
  (return (not (Math|Boolean|ORBoolean (Variables|Default|GetisRolling) (Variables|Default|GetisAttacking) (Variables|Default|GetisDying) (Variables|Default|Get_rollInCooldown)))))

(fn CheckRollChance
  (bind _can_roll (CallFunction|CanRoll))
  (if _can_roll
    (if (<= (Math|Random|RandomIntegerinRange 1 100) (Variables|Default|GetRollChance))
      (CallFunction|StartRoll))))

(fn SetMovementState
  (params (State :type ENUM_MafiaStates%20Enum :default "NewEnumerator0"))
  (bind _animator (Variables|Default|GetAnimator))
  (Utilities|FlowControl|Sequence
    (:then_0
      (switch Utilities|FlowControl|Switch|SwitchonENUM_MafiaStates State
        (:NewEnumerator0
          (LocalVariables|Setspeed 0.0)
          (Default|SetSpeed _animator))
        (:NewEnumerator1
          (LocalVariables|Setspeed (Variables|Default|GetWalkSpeed))
          (Default|SetSpeed _animator 1))
        (:NewEnumerator2
          (LocalVariables|Setspeed (Variables|Default|GetRunSpeed))
          (Default|SetSpeed _animator 2))))
    (:then_1
      (CallFunction|SetMovementSpeed (LocalVariables|Getspeed)))
    (:then_2
      (Variables|Default|Set_currentMovementState State))))

(fn SetMovementSpeed
  (params (Speed :type Float%20%28double-precision%29))
  (Variables|/Script/Engine.CharacterMovementComponent|SetMaxWalkSpeed (Variables|Character|GetCharacterMovement) Speed))

(fn SpawnProjectile
  (bind _transform (Default|GetMuzzleTransform (Variables|Default|GetWeapon)))
  (bind _returnvalue (Game|SpawnActorfromClass "/Game/REGRETSSION-Assets/Blueprints/Actors/Enemy/EnemyProjectiles/BP_EnemyHitscanBullet.BP_EnemyHitscanBullet_C" _transform "Undefined" "OverrideRootScale" 0 0))
  (bind _pos (Default|GetShootingDirection (Variables|Default|GetWeapon)))
  (Default|SpawnHitscan _returnvalue 5e+03 (Math|Conversions|ToFloat(Integer) (Variables|Default|GetAttackDamage)) "NewEnumerator0" _pos (Math|Vector|Normalize (- (Variables|Default|GetPlayerPos) _pos))))

(fn ForceGroundedRotation
  (Transformation|SetWorldRotation (Variables|Default|GetCapsuleComponent) (Math|Rotator|MakeRotator 0.0 0.0 (.yaw (Transformation|GetWorldRotation (Variables|Default|GetCapsuleComponent)))) false false))

(fn ForcedRollEnd
  (Default|OnRollEnd (Variables|Default|GetAnimator)))

(fn InitializeEnemy
  (|CallParentFunction)
  (Variables|/Script/Engine.CharacterMovementComponent|SetMaxWalkSpeed (Variables|Character|GetCharacterMovement) (Variables|Default|GetWalkSpeed))
  (bind _asaic_mafia (Utilities|Casting|CastToAIC_Mafia (AI|GetAIController self)))
  (bind _output_get (Variables|Default|SetAIController _asaic_mafia))
  (Default|InitializeAI _output_get)
  (bind _asbp_mafia_beretta (Utilities|Casting|CastToBP_MafiaBeretta (Variables|/Script/Engine.ChildActorComponent|GetChildActor (Variables|Default|GetBeretta))))
  (Variables|Default|SetWeapon _asbp_mafia_beretta))

(fn StartDeath
  (params (ImpactPoint :type Vector :default "0, 0, 0") (KillingDamage :type Float%20%28double-precision%29))
  (bind _sound_list (Variables|Default|GetSound%20List))
  (bind (_death _gibbing) (Utilities|Struct|BreakSTRUCT_MafiaSound _sound_list))
  (|CallParentFunction ImpactPoint KillingDamage)
  (Utilities|FlowControl|Sequence
    (:then_0
      (Variables|Default|SetcurrentSpeed 0.0))
    (:then_1
      (Variables|Default|SetisAttacking false)
      (Variables|Default|SetisRolling false)
      (CallFunction|OnJumpEnd))
    (:then_2
      (Variables|Default|SetisDying true)
      (Default|OnDeath (Variables|Default|GetAIController))
      (CallFunction|OnAttackEnd true))
    (:then_3
      (Default|OnDeath (Variables|Default|GetAnimator))
      (Collision|SetCollisionEnabled (Variables|Default|GetCapsuleComponent) "NoCollision")
      (Physics|SetEnableGravity (Variables|Default|GetCapsuleComponent) false)
      (Utilities|FlowControl|Sequence
        (:then_0
          (switch Utilities|FlowControl|Switch|SwitchonENUM_EnemyDeathStates (Variables|Default|GetDeathType)
            (:NewEnumerator0
              (LocalVariables|SetSoundToPlay _death))
            (:NewEnumerator1
              (LocalVariables|SetSoundToPlay _gibbing :!label _label))
            (:NewEnumerator2
              (goto _label))))
        (:then_1
          (CallFunction|PlaySound (LocalVariables|GetSoundToPlay) true false)
          (CallFunction|ForceGroundedRotation)
          (CallFunction|DropWeapon))))))

(fn PlaySound
  (params (Sound :type Sound%20Base%20Object%20Reference) (CancelPreviousSound :type Boolean) (Cancellable :type Boolean))
  (|CallParentFunction Sound CancelPreviousSound Cancellable))

(fn TakeDamageGeneric
  (params (Dmg :type Float%20%28double-precision%29))
  (|CallParentFunction Dmg)
  (if (<= (Variables|Default|Get_currentHP) 0.0)
    (CallFunction|StartDeath "0, 0, 0" Dmg)
    (else
      (CallFunction|CheckRollChance))))

(fn TakeDamagePoint
  (params (Dmg :type Float%20%28double-precision%29) (HitLoc :type Vector :default "0, 0, 0") (HitNormal :type Vector :default "0, 0, 0") (HitBone :type Name :default "None"))
  (|CallParentFunction Dmg HitLoc HitNormal HitBone)
  (if (<= (Variables|Default|Get_currentHP) 0.0)
    (CallFunction|StartDeath HitLoc Dmg)
    (else
      (CallFunction|CheckRollChance))))

(fn OnTargetFound
  (|CallParentFunction)
  (if (not (Variables|Default|GetisDying))
    (CallFunction|PlaySound (Utilities|Struct|BreakSTRUCT_MafiaSound (Variables|Default|GetSound%20List)) false true)))

(fn DropWeapon
  (bind _asbp_mafia_beretta (Utilities|Casting|CastToBP_MafiaBeretta (Variables|/Script/Engine.ChildActorComponent|GetChildActor (Variables|Default|GetBeretta))))
  (Default|DropWeapon _asbp_mafia_beretta))