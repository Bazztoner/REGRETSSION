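; Behavior tree service for Mafia enemies that supplies a random nearby destination and updates the pawn's movement state.
; On activation it caches the controlled pawn, picks a random navigable point within a searchable radius around it and writes that to the RandomClosePoint blackboard key.
; Each service tick switches the cached pawn between two movement states depending on whether it is rolling.
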(event EventReceiveActivationAI
  (params (OwnerController :type AI%20Controller%20Object%20Reference) (ControlledPawn :type Pawn%20Object%20Reference))
  (bind _output_get (Variables|Default|SetMyPawn ControlledPawn))
  (bind _randomlocation (Class|NavigationSystemV1|GetRandomLocationinNavigableRadius (Transformation|GetActorLocation _output_get) (Variables|Default|GetSearchableRadius) 0 0))
  (AI|Components|Blackboard|SetValueasVector (AI|GetBlackboard OwnerController) (Utilities|Name|MakeLiteralName "RandomClosePoint") _randomlocation))

(event EventReceiveTickAI
  (params (OwnerController :type AI%20Controller%20Object%20Reference) (ControlledPawn :type Pawn%20Object%20Reference) (DeltaSeconds :type Float%20%28single-precision%29))
  (bind _mypawn (Variables|Default|GetMyPawn))
  (if (Variables|/Game/REGRETSSION-Assets/Art/Models/Characters/Enemies/Mafia/Blueprints/BP_Mafia.BP_Mafia_C|GetisRolling (Variables|Default|GetMyPawn))
    (Default|SetMovementState _mypawn "NewEnumerator0")
    (else
      (Default|SetMovementState _mypawn "NewEnumerator1"))))